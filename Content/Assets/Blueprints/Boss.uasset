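; Boss actor with health and three attack or ability events: raising the dead, throwing two axes, and repairing pillars.
; Abilities pulse state bools around delays, firing necro effects or spawning axe and pillar energy actors tracked in arrays.
; A timeline fades emissive intensity on a dynamic material created in the construction script.
; Damage applies only while CanBeHurt, and zero health calls Progress on the BossFightController.
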(event Custom|TurnOffEmissive
  (Rendering|Material|SetScalarParameterValue (Variables|Default|GetEmmisiveMaterial) "Emissive Intensity" 0.0 :!class /Script/Engine.MaterialInstanceDynamic))

(event Custom|ChangeEmissive
  (params (CustomValue :type Float%20%28single-precision%29) (PlayRate :type Float%20%28single-precision%29))
  (bind _emissive (Variables|Default|GetEmissive))
  (bind _returnvalue (Rendering|Material|GetScalarParameterValue (Variables|Default|GetEmmisiveMaterial) "Emissive Intensity" :!class /Script/Engine.MaterialInstanceDynamic))
  (Variables|Default|SetCurrentEmissiveValue _returnvalue)
  (if (> CustomValue 0.0)
    (Variables|Default|SetTargetValue CustomValue)
    (else
      (Variables|Default|SetTargetValue (Variables|Default|GetDefaultEmissiveValue))))
  (if (> PlayRate 0.0)
    (Components|Timeline|SetPlayRate _emissive PlayRate)
    (bind _value (Timeline|Emissive PlayFromStart)
      (:Update
        (Rendering|Material|SetScalarParameterValue (Variables|Default|GetEmmisiveMaterial) "Emissive Intensity" (Math|Float|Lerp (Variables|Default|GetCurrentEmissiveValue) (Variables|Default|GetTargetValue) _value) :!class /Script/Engine.MaterialInstanceDynamic)))
    (else
      (Components|Timeline|SetPlayRate _emissive 1.0)
      (Timeline|Emissive PlayFromStart))))

(event Custom|AxeThrowAttack
  (bind _axesize (Variables|Default|GetAxeSize))
  (bind _axespawnright (Variables|Default|GetAxeSpawnRight))
  (bind _axespawnleft (Variables|Default|GetAxeSpawnLeft))
  (bind _axesize_2 (Variables|Default|GetAxeSize))
  (bind _returnvalue (Transformation|GetWorldTransform _axespawnright))
  (bind _returnvalue_2 (Transformation|GetWorldTransform _axespawnleft))
  (Variables|Default|SetAxeThrow true)
  (bind _returnvalue_3 (Game|SpawnActorfromClass "/Game/Assets/Blueprints/Axe.Axe_C" (Math|Transform|MakeTransform (.location _returnvalue_2) (.rotation _returnvalue_2) (Math|Vector|MakeVector _axesize _axesize _axesize)) "AlwaysSpawn" 0 0))
  (Utilities|Array|Add (Variables|Default|GetAxeRefs) _returnvalue_3)
  (bind _returnvalue_4 (Game|SpawnActorfromClass "/Game/Assets/Blueprints/Axe.Axe_C" (Math|Transform|MakeTransform (.location _returnvalue) (.rotation _returnvalue) (Math|Vector|MakeVector _axesize_2 _axesize_2 _axesize_2)) "AlwaysSpawn" 0 0))
  (Utilities|Array|Add (Variables|Default|GetAxeRefs) _returnvalue_4)
  (Utilities|FlowControl|Delay 0.5)
  (Variables|Default|SetAxeThrow false))

(event Custom|RepairThePillar
  (params (SpawnInfo :type Transform) (Index :type Integer))
  (Variables|Default|SetRepairPillar true)
  (Utilities|FlowControl|Delay 0.5)
  (Variables|Default|SetRepairPillar false)
  (Utilities|FlowControl|Delay 3.0)
  (bind _returnvalue (Game|SpawnActorfromClass "/Game/Assets/Blueprints/PillarEnergy.PillarEnergy_C" (Math|Transform|MakeTransform (.location SpawnInfo) (.rotation SpawnInfo) "1,1,1") "AlwaysSpawn" 0 0))
  (Utilities|Array|SetArrayElem (Variables|Default|GetPillarHoldRefs) Index _returnvalue))

(event Custom|RaiseThyDead
  (Components|Activation|Activate (Variables|Default|GetNecro_charge) false)
  (Variables|Default|SetRaiseTheDead true)
  (Utilities|FlowControl|Delay 5.0)
  (Components|Activation|Activate (Variables|Default|GetNecro_wave) false)
  (Variables|Default|SetRaiseTheDead false))

(event EventBeginPlay
  (bind _returnvalue (Rendering|Material|GetScalarParameterValue (Variables|Default|GetEmmisiveMaterial) "Emissive Intensity" :!class /Script/Engine.MaterialInstanceDynamic))
  (Variables|Default|SetDefaultEmissiveValue _returnvalue)
  (CallFunction|TurnOffEmissive))

(event Collision|EventActorBeginOverlap
  (params (OtherActor :type Actor%20Object%20Reference)))

(event EventTick
  (params (DeltaSeconds :type Float%20%28single-precision%29)))

(event EventTakeDamage
  (params (DamageAmount :type Float%20%28single-precision%29) (Constant :type Boolean) (Effect :type Effects%20Enum :default "NewEnumerator4") (EffectTime :type Float%20%28single-precision%29) (Hit_Location :type Vector :default "0, 0, 0"))
  (if (Variables|Default|GetcanBeHurt)
    (bind _output_get (Variables|Default|SetHealth (- (Variables|Default|GetHealth) DamageAmount)))
    (if (<= _output_get 0.0)
      (bind _outactors (Actor|GetAllActorsOfClass "/Game/Assets/Blueprints/Boss_Fight/BossFightController.BossFightController_C"))
      (Utilities|IsValid (Utilities|Array|Get(acopy) _outactors)
        (:Is%20Valid
          (Default|Progress (Utilities|Array|Get(acopy) _outactors)))))))

(fn ConstructionScript
  (bind _skeletalmesh (Variables|Components|GetSkeletalMesh))
  (bind _skeletalmesh_2 (Variables|Components|GetSkeletalMesh))
  (Transformation|AttachComponentToComponent (Variables|Components|GetRight_Hand_spawn) _skeletalmesh_2 "R_Middle_01_Jnt" "SnapToTarget" "KeepRelative" "KeepRelative" true)
  (Transformation|AttachComponentToComponent (Variables|Components|GetLeft_Hand_spawn) _skeletalmesh_2 "L_Middle_01_Jnt" "SnapToTarget" "KeepRelative" "KeepRelative" true)
  (bind _returnvalue (Rendering|Material|CreateDynamicMaterialInstance _skeletalmesh 0 (Rendering|Material|GetMaterial _skeletalmesh 0) :!class /Script/Engine.PrimitiveComponent))
  (Variables|Default|SetEmmisiveMaterial _returnvalue))

(fn DestroyPillarEnergys
  (bind _pillarholdrefs (Variables|Default|GetPillarHoldRefs))
  (bind _output (Utilities|Array|Get(acopy) _pillarholdrefs))
  (bind _output_2 (Utilities|Array|Get(acopy) _pillarholdrefs 3))
  (Utilities|IsValid _output
    (:Is%20Valid
      (Actor|DestroyActor _output)
      (Utilities|Array|SetArrayElem _pillarholdrefs 0 0))
    (:Is%20Not%20Valid
      _))
  (Utilities|IsValid _output_2
    (:Is%20Valid
      (Actor|DestroyActor _output_2)
      (Utilities|Array|SetArrayElem _pillarholdrefs 3 0))))