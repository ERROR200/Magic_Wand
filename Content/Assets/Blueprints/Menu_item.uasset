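; Menu item actor that acts as an in-world button, triggered by taking damage.
; Depending on its type, it fades the PersonalMCPawn's screen and loads a level, quits the game, or switches category.
; Category switching sets Active on listed menu items and option buttons, then updates each.
; Updates play a shutter sound and apply Active to mesh visibility and collision behind a briefly locked DoOnce; construction applies the same state.
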(event Custom|update_element
  (bind _mesh (Variables|Default|Getmesh))
  (bind _active (Variables|Default|Getactive))
  (Audio|PlaySound2D "/Engine/VREditor/Sounds/UI/Camera_Shutter.Camera_Shutter")
  (Utilities|FlowControl|DoOnce false :!label _label
    (:Completed
      (Rendering|SetVisibility _mesh _active false)
      (Collision|SetCollisionEnabled _mesh (select _active "QueryAndPhysics" "NoCollision"))
      (Utilities|FlowControl|Delay 0.1)
      (goto _label Reset))))

(event EventBeginPlay)

(event Collision|EventActorBeginOverlap
  (params (OtherActor :type Actor%20Object%20Reference)))

(event EventTick
  (params (DeltaSeconds :type Float%20%28single-precision%29)))

(event EventTakeDamage
  (params (DamageAmount :type Float%20%28single-precision%29) (Constant :type Boolean) (Effect :type Effects%20Enum :default "NewEnumerator4") (EffectTime :type Float%20%28single-precision%29) (Hit_Location :type Vector :default "0, 0, 0"))
  (bind _aspersonal_mcpawn (Utilities|Casting|CastToPersonalMCPawn (Game|Player|GetPlayerPawn 0)))
  (switch Utilities|FlowControl|Switch|Switchonmenu_item_type (Variables|Default|Getmenu%20item%20type)
    (:NewEnumerator0
      (Default|ScreenFade _aspersonal_mcpawn)
      (Utilities|FlowControl|Delay 3.0)
      (Game|OpenLevel(byName) (Variables|Default|Getlevel_Name)))
    (:NewEnumerator3
      (Game|QuitGame 0 "Quit"))
    (:NewEnumerator4
      (for _array_element (Variables|Default|GetCatagory_Activate_list)
        (bind _asmenu_item (Utilities|Casting|CastToMenu_item _array_element)
          (:then
            (Variables|Menu_item_C|Setactive _asmenu_item true)
            (CallFunction|UpdateElement _asmenu_item))
          (:CastFailed
            (bind _asmenu_item_option_button (Utilities|Casting|CastToMenu_item_option_button _array_element)
              (:then
                (Variables|/Game/Assets/Blueprints/Menu_item_option_button.Menu_item_option_button_C|Setactive _asmenu_item_option_button true)
                (Default|UpdateElement _asmenu_item_option_button))
              (:CastFailed
                (bind _asmenu_item_option_button_2 (Utilities|Casting|CastToMenu_item_option_button _array_element))
                (Variables|/Game/Assets/Blueprints/Menu_item_option_button.Menu_item_option_button_C|Setactive _asmenu_item_option_button_2 true)
                (Default|UpdateElement _asmenu_item_option_button_2))))))
      (for _array_element_2 (Variables|Default|GetCatagory_Deactivate_list)
        (bind _asmenu_item_2 (Utilities|Casting|CastToMenu_item _array_element_2)
          (:then
            (Variables|Menu_item_C|Setactive _asmenu_item_2 false)
            (CallFunction|UpdateElement _asmenu_item_2))
          (:CastFailed
            (bind _asmenu_item_option_button_3 (Utilities|Casting|CastToMenu_item_option_button _array_element_2)
              (:then
                (Variables|/Game/Assets/Blueprints/Menu_item_option_button.Menu_item_option_button_C|Setactive _asmenu_item_option_button_3 false)
                (Default|UpdateElement _asmenu_item_option_button_3))
              (:CastFailed
                (bind _asmenu_item_option_button_4 (Utilities|Casting|CastToMenu_item_option_button _array_element_2))
                (Variables|/Game/Assets/Blueprints/Menu_item_option_button.Menu_item_option_button_C|Setactive _asmenu_item_option_button_4 false)
                (Default|UpdateElement _asmenu_item_option_button_4)))))))))

(fn ConstructionScript
  (bind _active (Variables|Default|Getactive))
  (Rendering|SetVisibility (Variables|Default|Getmesh) _active false)
  (Collision|SetCollisionEnabled (Variables|Default|Getmesh) (select _active "QueryAndPhysics" "NoCollision")))