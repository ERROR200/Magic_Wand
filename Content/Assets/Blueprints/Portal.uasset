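; Portal actor that teleports the player within the current level or opens another level by name.
; Tick orients its components along the camera-to-cube line, while activate_portal moves the screen into place and plays particles and an opening timeline.
; PortalActivated or taking damage, unless overridden, triggers a once-guarded post-process fade and light flash before travel.
; Same-level travel repositions pawn and spring arm, drops the screen away, then reverses the fade to re-arm.
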(event Custom|Portal_Next_Location
  (params (Portal_point :type Vector) (LevelName :type String))
  (Transformation|SetWorldLocation (Variables|Default|GetPortal_Point) Portal_point false false)
  (Variables|Default|SetNextLevel LevelName))

(event Custom|PortalActivated
  (bind _returnvalue (Game|Player|GetPlayerPawn 0))
  (bind _pointlight (Variables|Default|GetPointLight))
  (bind _next_position (Variables|Default|GetNext_position))
  (bind _nextlevel (Variables|Default|GetNextLevel))
  (if (not (Variables|Default|GetoverrideTeleportingStop))
    (Utilities|FlowControl|DoOnce false :!label _label
      (:Completed
        (bind (_direction _newtrack_1) (Timeline|pp PlayFromStart)
          (:Update
            (Variables|/Script/Engine.PostProcessComponent|SetBlendWeight (Variables|Default|GetPostProcess) _newtrack_1))
          (:Finished
            (if (Utilities|Enum|Equal(Enum) _direction "Forward")
              (Rendering|Components|Light|SetIntensity _pointlight 1e+07)
              (Utilities|FlowControl|Delay 1.0)
              (if (Utilities|Enum|Equal(Enum) (Variables|Default|GetCurrentLevel) _nextlevel)
                (bind _aspersonal_mcpawn (Utilities|Casting|CastToPersonalMCPawn _returnvalue))
                (Transformation|SetActorLocationAndRotation _returnvalue (.location _next_position) (.rotation _next_position))
                (Transformation|SetRelativeRotation (Variables|/Game/Assets/Blueprints/PersonalMCPawn.PersonalMCPawn_C|GetSpringArm _aspersonal_mcpawn) (.rotation _next_position) false false)
                (Transformation|AddLocalRotation (Variables|/Game/Assets/Blueprints/PersonalMCPawn.PersonalMCPawn_C|GetSpringArm _aspersonal_mcpawn) "180.000000, 0, 0" false false)
                (Transformation|AddRelativeLocation (Variables|Default|Getportal_screen_point) "0, 0,-2000.000000" false false)
                (Timeline|pp Reverse)
                (else
                  (Game|OpenLevel(byName) (Utilities|String|StringToName _nextlevel))))
              (else
                (Rendering|Components|Light|SetIntensity _pointlight 0.0)
                (goto _label Reset)))))))))

(event Custom|activate_portal
  (params (Portal%20Location :type Vector))
  (Transformation|SetWorldLocation (Variables|Default|Getportal_screen_point) Portal%20Location false false)
  (Components|Activation|Activate (Variables|Default|GetParticleSystem) true)
  (bind _newtrack_0 (Timeline|Portal_open PlayFromStart)
    (:Update
      (Transformation|SetRelativeScale3D (Variables|Default|Getportal_screen_point) (Math|Conversions|ToVector(Float) _newtrack_0)))))

(event EventBeginPlay
  (bind _returnvalue (Game|GetCurrentLevelName true))
  (Variables|Default|SetCurrentLevel _returnvalue))

(event Collision|EventActorBeginOverlap
  (params (OtherActor :type Actor%20Object%20Reference)))

(event EventTick
  (params (DeltaSeconds :type Float%20%28single-precision%29))
  (bind _returnvalue (Game|GetPlayerCameraManager 0))
  (bind _cube (Variables|Default|GetCube))
  (bind _returnvalue_2 (Camera|GetCameraLocation _returnvalue))
  (bind _returnvalue_3 (Transformation|GetWorldLocation _cube))
  (Transformation|SetWorldRotation (Variables|Default|Getportal_direction) (Math|Rotator|FindLookatRotation _returnvalue_2 _returnvalue_3) false false)
  (Transformation|SetWorldRotation (Variables|Default|Getportal_screen_point) (Math|Rotator|FindLookatRotation _returnvalue_3 _returnvalue_2) false false)
  (if (Variables|Default|Getdemo%20mode)
    (Utilities|FlowControl|Delay 1.0)
    (bind _newtrack_0 (Timeline|Portal_open Play)
      (:Update
        (Transformation|SetRelativeScale3D (Variables|Default|Getportal_screen_point) (Math|Conversions|ToVector(Float) _newtrack_0))))))

(event EventTakeDamage
  (params (DamageAmount :type Float%20%28single-precision%29) (Constant :type Boolean) (Effect :type Effects%20Enum :default "NewEnumerator4") (EffectTime :type Float%20%28single-precision%29) (Hit_Location :type Vector :default "0, 0, 0"))
  (bind _returnvalue (Game|Player|GetPlayerPawn 0))
  (bind _pointlight (Variables|Default|GetPointLight))
  (bind _next_position (Variables|Default|GetNext_position))
  (bind _nextlevel (Variables|Default|GetNextLevel))
  (if (not (Variables|Default|GetoverrideTeleportingStop))
    (Utilities|FlowControl|DoOnce false :!label _label
      (:Completed
        (bind (_direction _newtrack_1) (Timeline|pp PlayFromStart)
          (:Update
            (Variables|/Script/Engine.PostProcessComponent|SetBlendWeight (Variables|Default|GetPostProcess) _newtrack_1))
          (:Finished
            (if (Utilities|Enum|Equal(Enum) _direction "Forward")
              (Rendering|Components|Light|SetIntensity _pointlight 1e+07)
              (Utilities|FlowControl|Delay 1.0)
              (if (Utilities|Enum|Equal(Enum) (Variables|Default|GetCurrentLevel) _nextlevel)
                (bind _aspersonal_mcpawn (Utilities|Casting|CastToPersonalMCPawn _returnvalue))
                (Transformation|SetActorLocationAndRotation _returnvalue (.location _next_position) (.rotation _next_position))
                (Transformation|SetRelativeRotation (Variables|/Game/Assets/Blueprints/PersonalMCPawn.PersonalMCPawn_C|GetSpringArm _aspersonal_mcpawn) (.rotation _next_position) false false)
                (Transformation|AddLocalRotation (Variables|/Game/Assets/Blueprints/PersonalMCPawn.PersonalMCPawn_C|GetSpringArm _aspersonal_mcpawn) "180.000000, 0, 0" false false)
                (Transformation|AddRelativeLocation (Variables|Default|Getportal_screen_point) "0, 0,-2000.000000" false false)
                (Timeline|pp Reverse)
                (else
                  (Game|OpenLevel(byName) (Utilities|String|StringToName _nextlevel))))
              (else
                (Rendering|Components|Light|SetIntensity _pointlight 0.0)
                (goto _label Reset)))))))))

(fn ConstructionScript)