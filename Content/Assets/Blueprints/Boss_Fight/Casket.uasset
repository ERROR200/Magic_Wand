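; Casket is a boss-fight prop whose green emissive glow turns on in response to overlaps from components tagged LightSwitch.
; The construction script creates a dynamic material instance on the static mesh, and BeginPlay sets it to green at zero intensity.
; A Box overlap feeds a FlipFlop with only the B output wired, so the glow switches on at the second tagged overlap and is never switched off.
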(event OnComponentBeginOverlap(Box)
  (params (OverlappedComponent :type Primitive%20Component%20Object%20Reference) (OtherActor :type Actor%20Object%20Reference) (OtherComp :type Primitive%20Component%20Object%20Reference) (OtherBodyIndex :type Integer) (bFromSweep :type Boolean) (SweepResult :type Hit%20Result%20Structure%20%28by%20ref%29))
  (if (Components|ComponentHasTag OtherComp "LightSwitch")
    (Utilities|FlowControl|FlipFlop
      (:B
        (Rendering|Material|SetScalarParameterValue (Variables|Default|GetEmissive) "Emissive Intensity" 1.0 :!class /Script/Engine.MaterialInstanceDynamic)))))

(event EventBeginPlay
  (bind _emissive (Variables|Default|GetEmissive))
  (Rendering|Material|SetScalarParameterValue _emissive "Emissive Intensity" 0.0 :!class /Script/Engine.MaterialInstanceDynamic)
  (Rendering|Material|SetVectorParameterValue _emissive "Emissive Colour" "(R=0.068478,G=1.000000,B=0.000000,A=1.000000)" :!class /Script/Engine.MaterialInstanceDynamic))

(event Collision|EventActorBeginOverlap
  (params (OtherActor :type Actor%20Object%20Reference)))

(event EventTick
  (params (DeltaSeconds :type Float%20%28single-precision%29)))

(fn ConstructionScript
  (bind _staticmeshcomponent (Variables|Debug|GetStaticMeshComponent))
  (bind _returnvalue (Rendering|Material|CreateDynamicMaterialInstance _staticmeshcomponent 0 (Rendering|Material|GetMaterial _staticmeshcomponent 0) :!class /Script/Engine.PrimitiveComponent))
  (Variables|Default|SetEmissive _returnvalue))