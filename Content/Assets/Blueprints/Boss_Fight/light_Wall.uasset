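; Boss fight wall light actor that switches between Fire and Necro styles, each pairing an effect component with its own point light.
; The construction script sets auto-activation and light visibility from LightStyle.
; At runtime, BeginPlay, the changelightstyle event and a Tick check against OldStyle share one routine that turns everything off, then enables the selected pair.
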(event Custom|change%20light%20style
  (params (light_style :type light_style%20Enum :default "NewEnumerator0"))
  (bind _fire (Variables|Default|GetFire))
  (bind _pointlight1 (Variables|Default|GetPointLight1))
  (Variables|Default|Setold_style light_style)
  (Variables|Default|Setlight_style light_style)
  (Rendering|SetVisibility _pointlight1 false false)
  (Components|Activation|Deactivate _fire)
  (switch Utilities|FlowControl|Switch|Switchonlight_style (Variables|Default|Getlight_style)
    (:NewEnumerator1
      (Components|Activation|SetActive _fire true false)
      (Rendering|SetVisibility (Variables|Default|GetPointLight) true false))
    (:NewEnumerator2
      (Components|Activation|SetActive (Variables|Default|GetNecro) true false)
      (Rendering|SetVisibility _pointlight1 true false))))

(event EventBeginPlay
  (bind _fire (Variables|Default|GetFire))
  (bind _pointlight1 (Variables|Default|GetPointLight1))
  (Rendering|SetVisibility _pointlight1 false false)
  (Components|Activation|Deactivate _fire)
  (switch Utilities|FlowControl|Switch|Switchonlight_style (Variables|Default|Getlight_style)
    (:NewEnumerator1
      (Components|Activation|SetActive _fire true false)
      (Rendering|SetVisibility (Variables|Default|GetPointLight) true false))
    (:NewEnumerator2
      (Components|Activation|SetActive (Variables|Default|GetNecro) true false)
      (Rendering|SetVisibility _pointlight1 true false))))

(event Collision|EventActorBeginOverlap
  (params (OtherActor :type Actor%20Object%20Reference)))

(event EventTick
  (params (DeltaSeconds :type Float%20%28single-precision%29))
  (bind _fire (Variables|Default|GetFire))
  (bind _pointlight1 (Variables|Default|GetPointLight1))
  (if (not (Utilities|Enum|Equal(Enum) (Variables|Default|Getlight_style) (Variables|Default|Getold_style)))
    (Variables|Default|Setold_style (Variables|Default|Getlight_style))
    (Rendering|SetVisibility _pointlight1 false false)
    (Components|Activation|Deactivate _fire)
    (switch Utilities|FlowControl|Switch|Switchonlight_style (Variables|Default|Getlight_style)
      (:NewEnumerator1
        (Components|Activation|SetActive _fire true false)
        (Rendering|SetVisibility (Variables|Default|GetPointLight) true false))
      (:NewEnumerator2
        (Components|Activation|SetActive (Variables|Default|GetNecro) true false)
        (Rendering|SetVisibility _pointlight1 true false)))))

(fn ConstructionScript
  (bind _pointlight1 (Variables|Default|GetPointLight1))
  (bind _fire (Variables|Default|GetFire))
  (Components|Activation|SetAutoActivate _fire false)
  (Rendering|SetVisibility _pointlight1 false false)
  (switch Utilities|FlowControl|Switch|Switchonlight_style (Variables|Default|Getlight_style)
    (:NewEnumerator1
      (Components|Activation|SetAutoActivate _fire true)
      (Rendering|SetVisibility (Variables|Default|GetPointLight) true false))
    (:NewEnumerator2
      (Components|Activation|SetAutoActivate (Variables|Default|GetNecro) true)
      (Rendering|SetVisibility _pointlight1 true false))))