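; BossFightController runs the boss fight as a staged state machine: intro audio, a main loop, then shield drop and final stand stages that are mostly stubs.
; Tick fires BattleTick on an Advance flag to start each step, otherwise polls Checking for cleared enemies or expired timers.
; The main loop cycles timer-driven random WaveGenerator waves, gargoyle activation and a placeholder pillar magic phase.
; BeginPlay caches actor references and sweeps a timeline-driven trigger box alongside a timed light toggle.
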(event Custom|BattleTick
  (bind _audio_intro (Variables|Default|GetAudio_Intro))
  (bind _skullref (Variables|Default|GetSkullRef))
  (bind _wavegeneratorref (Variables|Default|GetWaveGeneratorRef))
  (bind _audio (Variables|/Game/Assets/Blueprints/LevelManager.LevelManager_C|GetAudio _skullref))
  (switch Utilities|FlowControl|Switch|SwitchonBossLevelTracking (Variables|Default|GetProgressionTracking)
    (:NewEnumerator0
      (Utilities|IsValid _skullref
        (:Is%20Valid
          (Audio|Components|Audio|SetSound _audio _audio_intro)
          (Audio|Components|Audio|Play _audio 0.0)
          (Utilities|Time|SetTimerbyFunctionName 0 "Progress" (Variables|/Script/Engine.SoundBase|GetDuration _audio_intro)))
        (:Is%20Not%20Valid
          (Development|PrintString "No level manager/skull reference"))))
    (:NewEnumerator1)
    (:NewEnumerator2
      (switch Utilities|FlowControl|Switch|SwitchonBF_MainLoop (Variables|Default|GetMainLoop)
        (:NewEnumerator0
          (if (>= (Math|Random|RandomFloatinRangefromStream 0.0 1.0 (Variables|Default|GetRandom)) 0.2)
            (CallFunction|DetermineWaveData :!label _label)
            (CallFunction|SetSpawnData)
            (Utilities|Time|SetTimerbyFunctionName 0 "CanSpawnNextWave" 1.0 true)
            (else
              (Utilities|IsValid _wavegeneratorref
                (:Is%20Valid
                  (Default|SetCustomRound _wavegeneratorref)
                  (goto _label))
                (:Is%20Not%20Valid
                  (Development|PrintString "No wave generator"))))))
        (:NewEnumerator1
          (Utilities|IsValid _wavegeneratorref
            (:Is%20Valid
              (Variables|/Game/Assets/Blueprints/WaveGenerator.WaveGenerator_C|SetisPremadeRound _wavegeneratorref false)
              (CallFunction|GargoyleToggleOn/Off true))))
        (:NewEnumerator3
          (CallFunction|SpawnHoldingEnergy))))
    (:NewEnumerator3
      (Variables|Default|SetTimer 2e+01))))

(event Custom|Checking
  (switch Utilities|FlowControl|Switch|SwitchonBossLevelTracking (Variables|Default|GetProgressionTracking)
    (:NewEnumerator2
      (switch Utilities|FlowControl|Switch|SwitchonBF_MainLoop (Variables|Default|GetMainLoop)
        (:NewEnumerator0
          (bind _return (CallFunction|CheckforNoEnemies))
          (if _return
            (Variables|Default|SetisChecking false :!label _label)))
        (:NewEnumerator1
          (bind _return_2 (CallFunction|ReduceTimer))
          (if _return_2
            (CallFunction|DisableGargoyles 0 false)
            (Variables|Default|SetTimer 2e+01)
            (goto _label)))
        (:NewEnumerator3
          (bind _return_3 (CallFunction|ReduceTimer))
          (if _return_3
            (CallFunction|Progress)
            (Variables|Default|SetMainLoop "NewEnumerator0")
            (goto _label)))))
    (:NewEnumerator3
      (bind _return_4 (CallFunction|ReduceTimer))
      (if _return_4
        _))
    (:NewEnumerator4
      (goto _label))))

(event Custom|Sweep
  (params (LightsOff :type Boolean))
  (if LightsOff
    (Components|Timeline|SetPlayRate (Variables|Default|GetSweepBox) 5.0)
    (bind _newtrack_0 (Timeline|SweepBox PlayFromStart)
      (:Update
        (Transformation|SetWorldLocation (Variables|Default|GetTriggerBox) (Math|Vector|Lerp(Vector) (Transformation|GetWorldLocation (Variables|Default|GetStartSwepLoc)) (Transformation|GetWorldLocation (Variables|Default|GetEndSwepLoc)) _newtrack_0) false false)))
    (else
      (Components|Timeline|SetPlayRate (Variables|Default|GetSweepBox) 5.0)
      (Timeline|SweepBox ReverseFromEnd))))

(event Custom|SetupSkull&Boss
  (bind _skullref (Variables|Default|GetSkullRef))
  (bind _audio (Variables|/Game/Assets/Blueprints/LevelManager.LevelManager_C|GetAudio _skullref))
  (Transformation|SetActorTransform (Variables|Default|GetSkullRef) (Transformation|GetWorldTransform (Variables|Default|GetCageLocation)))
  (Rendering|SetActorHiddenInGame (Variables|Default|GetBossRef) false)
  (Utilities|IsValid _skullref
    (:Is%20Valid
      (Audio|Components|Audio|SetSound _audio (Variables|Default|GetSkull_DraggedAway))
      (Audio|Components|Audio|Play _audio 0.0)
      (Utilities|FlowControl|Delay 2.0))))

(event EventBeginPlay
  (bind _outactors (Actor|GetAllActorsOfClass "/Game/Assets/Blueprints/Gargoyle.Gargoyle_C"))
  (Variables|Default|SetGargoyleRefs _outactors)
  (bind _outactors_2 (Actor|GetAllActorsOfClass "/Game/Assets/Blueprints/WaveGenerator.WaveGenerator_C"))
  (Variables|Default|SetWaveGeneratorRef (Utilities|Array|Get(acopy) _outactors_2))
  (bind _outactors_3 (Actor|GetAllActorsOfClass "/Game/Assets/Blueprints/LevelManager.LevelManager_C"))
  (Variables|Default|SetSkullRef (Utilities|Array|Get(acopy) _outactors_3))
  (Utilities|FlowControl|Delay 2.0)
  (Default|CallActivateLights true)
  (CallFunction|Sweep true)
  (Utilities|FlowControl|Delay 1e+01)
  (Default|CallActivateLights false)
  (CallFunction|Sweep false))

(event Collision|EventActorBeginOverlap
  (params (OtherActor :type Actor%20Object%20Reference)))

(event EventTick
  (params (DeltaSeconds :type Float%20%28single-precision%29))
  (if (Variables|Default|GetAdvance)
    (Variables|Default|SetAdvance false)
    (CallFunction|BattleTick)
    (elif (Variables|Default|GetisChecking)
      (CallFunction|Checking))))

(fn ConstructionScript)

(fn Progress
  (Variables|Default|SetAdvance true)
  (if (or (and (Utilities|Enum|Equal(Enum) (Variables|Default|GetProgressionTracking) "NewEnumerator2") (>= (Variables|Default|GetRoundIndex) 4)) (Utilities|Enum|NotEqual(Enum) (Variables|Default|GetProgressionTracking) "NewEnumerator2"))
    (Variables|Default|SetProgressionTracking (Utilities|Enum|ByteToEnumBossLevelTracking (+ (Variables|Default|GetProgressionTracking) 1)))
    (else
      (Math|Integer|IncrementInt (Variables|Default|GetRoundIndex)))))

(fn DetermineWaveData
  (bind _random (Variables|Default|GetRandom))
  (Variables|Default|SetNumberOfWaves (Math|Random|RandomIntegerinRangefromStream 4 7 _random))
  (Variables|Default|SetTimeBetweenWaves (Math|Random|RandomFloatinRangefromStream 1.0 2.0 _random)))

(fn SetSpawnData
  (bind _random (Variables|Default|GetRandom))
  (bind _returnvalue (Math|Random|RandomFloatinRangefromStream 0.1 1.0 _random))
  (Default|SpawnEnemy (Variables|Default|GetWaveGeneratorRef) (Math|Random|RandomIntegerinRangefromStream 6 8 _random) (<= _returnvalue 0.5) _returnvalue (Math|Random|RandomFloatinRangefromStream 2.0 3.0 _random)))

(fn GargoyleToggleOn/Off
  (params (TurnOn :type Boolean))
  (for _array_element (Variables|Default|GetGargoyleRefs)
    (Utilities|IsValid _array_element
      (:Is%20Valid
        (if TurnOn
          (Variables|/Game/Assets/Blueprints/Gargoyle.Gargoyle_C|SetisActive _array_element true)
          (else
            (Default|Deactivate _array_element)))))))

(fn CheckforNoEnemies
  (bind _outactors (Actor|GetAllActorsOfClass "/Game/Assets/Blueprints/AIBasicEnemy.AIBasicEnemy_C"))
  (if (== (- (Utilities|Array|LastIndex _outactors) (Utilities|Array|LastIndex (Variables|Default|GetGargoyleRefs))) 0)
    (Variables|Default|SetMainLoop "NewEnumerator1")
    (Variables|Default|SetAdvance true)
    (return true)
    (else
      (return false))))

(fn ReduceTimer
  (bind _output_get (Variables|Default|SetTimer (- (Variables|Default|GetTimer) (Utilities|Time|GetWorldDeltaSeconds))))
  (return (<= _output_get 0.0)))

(fn CanSpawnNextWave
  (bind _wavegeneratorref (Variables|Default|GetWaveGeneratorRef))
  (if (> (Variables|Default|GetNumberOfWaves) 0)
    (Utilities|IsValid _wavegeneratorref
      (:Is%20Valid
        (if (not (Variables|/Game/Assets/Blueprints/WaveGenerator.WaveGenerator_C|GetSpawningActive _wavegeneratorref))
          (Utilities|Time|SetTimerbyFunctionName 0 "SetSpawnData" (Variables|Default|GetTimeBetweenWaves))
          (Math|Integer|DecrementInt (Variables|Default|GetNumberOfWaves)))))
    (else
      (Utilities|Time|ClearTimerbyFunctionName 0 "CanSpawnNextWave")
      (Variables|Default|SetisChecking true))))

(fn DisableGargoyles
  (params (GargoyleRef :type Gargoyle%20Object%20Reference) (DoesProgress :type Boolean))
  (Utilities|IsValid GargoyleRef
    (:Is%20Valid
      (Utilities|Array|RemoveItem (Variables|Default|GetGargoyleRefs) GargoyleRef))
    (:Is%20Not%20Valid
      _))
  (CallFunction|GargoyleToggleOn/Off false)
  (if DoesProgress
    (Variables|Default|SetMainLoop "NewEnumerator3")
    (else
      (Variables|Default|SetMainLoop "NewEnumerator0")))
  (Variables|Default|SetAdvance true))

(fn SpawnHoldingEnergy
  (Variables|Default|SetisChecking true)
  (Variables|Default|SetTimer 3.0))