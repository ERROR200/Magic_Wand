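; Level manager actor: a wizard-skull orb that moves between level points and runs the round and portal progression.
; Damage starts a round, enabling the current spawner and any skull targets, or, once ready, opens the portal to the next point and records player progression.
; Added energy brightens its dynamic emissive material and completes target rounds at the required count.
; LoadLevelDirectly clears enemies, reloads gargoyles and jumps to a given level.
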(event Custom|WavesComplete
  (Math|Integer|IncrementInt (Variables|Default|GetCurrentSpawnEmmiter)
    (:%20%20
      (if (< (Variables|Default|GetCurrentSpawnEmmiter) (Utilities|Array|Length (Variables|Default|GetSpawnerHolder)))
        ;[1 1 1] Set_complete
        (Variables|Default|SetLevelState "NewEnumerator0")
        (Variables|Default|SetPortal_ready true)
        (else
          ;[1 1 1] endgame
          (Variables|Default|SetLevelState "NewEnumerator2")
          (Development|PrintString "LEVEL BEATEN!" true true "(R=0.959213,G=1.000000,B=0.000000,A=1.000000)" 2e+01))))))

(event Custom|LoadLevelDirectly
  (params (LevelValue :type Integer))
  (bind _level_manager_points (Variables|Default|GetLevel_Manager_Points))
  (bind _spawnerholder (Variables|Default|GetSpawnerHolder))
  ;[1 1 1] Force load given level
  (bind _outactors (Actor|GetAllActorsOfClass "/Game/Assets/Blueprints/AIBasicEnemy.AIBasicEnemy_C"))
  (for _array_element _outactors
    (Utilities|Casting|CastToGargoyle _array_element
      (:CastFailed
        (Default|ForceKillforLevelLoad _array_element))))
  (for _index (range (- (Utilities|Array|Length _spawnerholder) 1) 0)
    (Utilities|IsValid (Utilities|Array|Get(acopy) _spawnerholder _index)
      (:Is%20Valid
        (Default|ReloadGargoyles (Utilities|Array|Get(acopy) _spawnerholder _index)))))
  (bind _outactors_2 (Actor|GetAllActorsOfClass "/Game/Assets/Blueprints/Portal.Portal_C"))
  (Default|ActivatePortal (Utilities|Array|Get(acopy) _outactors_2) (Transformation|GetWorldLocation (Variables|/Game/Assets/Blueprints/LevelManagerPoint.LevelManagerPoint_C|Getportal_point (Utilities|Array|Get(acopy) _level_manager_points (Variables|Default|GetLevel_point)))))
  (bind _output_get (Variables|Default|SetCurrentSpawnEmmiter LevelValue))
  (bind _output_get_2 (Variables|Default|SetLevel_point _output_get))
  (if (== _output_get_2 5)
    (Default|PortalNextLocation (Utilities|Array|Get(acopy) _outactors_2) (Transformation|GetWorldLocation (Variables|/Game/Assets/Blueprints/LevelManagerPoint.LevelManagerPoint_C|Getportal_point (Utilities|Array|Get(acopy) _level_manager_points (Variables|Default|GetLevel_point)))) "Crypt_level")
    (else
      (Default|PortalNextLocation (Utilities|Array|Get(acopy) _outactors_2) (Transformation|GetWorldLocation (Variables|/Game/Assets/Blueprints/LevelManagerPoint.LevelManagerPoint_C|Getportal_point (Utilities|Array|Get(acopy) _level_manager_points (Variables|Default|GetLevel_point)))) "Progression_Level")))
  (Variables|/Game/Assets/Blueprints/Portal.Portal_C|SetNext_position (Utilities|Array|Get(acopy) _outactors_2) (Transformation|GetWorldTransform (Variables|/Game/Assets/Blueprints/LevelManagerPoint.LevelManagerPoint_C|Getplayer_point (Utilities|Array|Get(acopy) _level_manager_points (Variables|Default|GetLevel_point)))))
  (Variables|Default|SetPortal_ready false)
  (Default|TakeDamage (Utilities|Array|Get(acopy) _outactors_2) 0.0 false "NewEnumerator4" 0.0 "0, 0, 0")
  (CallFunction|ForceLoadLevel))

(event Custom|energy_added
  (Math|Float|IncrementFloat (Variables|Default|GetSet_points)
    (:%20%20
      (CallFunction|LightPulse)
      (Rendering|Material|SetScalarParameterValue (Variables|Default|GetEmissiveMaterial) "Emissive Intensity" (Math|Float|MapRangeClamped (Variables|Default|GetSet_points) 0.0 (Variables|Default|Getrequired_points) 0.1 1.0) :!class /Script/Engine.MaterialInstanceDynamic)
      (if (>= (Variables|Default|GetSet_points) (Variables|Default|Getrequired_points))
        (Variables|Default|SetSet_points 0.0)
        (CallFunction|LightPulse)
        (if (Variables|/Game/Assets/Blueprints/LevelManagerPoint.LevelManagerPoint_C|GetTarget_round (Utilities|Array|Get(acopy) (Variables|Default|GetLevel_Manager_Points) (Variables|Default|GetLevel_point)))
          (CallFunction|WavesComplete))))))

(event Custom|ForceLoadLevel
  (bind _level_manager_points (Variables|Default|GetLevel_Manager_Points))
  (bind _level_point (Variables|Default|GetLevel_point))
  (bind _output (Utilities|Array|Get(acopy) _level_manager_points _level_point))
  ;[1 1 1] Reset
  (CallFunction|ResetSphere)
  (Transformation|SetActorTransform (Transformation|GetWorldTransform (Variables|/Game/Assets/Blueprints/LevelManagerPoint.LevelManagerPoint_C|GetOrb_point _output)))
  (Variables|Default|Setrequired_points (Math|Conversions|ToFloat(Integer) (Variables|/Game/Assets/Blueprints/LevelManagerPoint.LevelManagerPoint_C|GetRequired%20points _output))))

(event Custom|ResetSphere
  (Rendering|Material|SetScalarParameterValue (Variables|Default|GetEmissiveMaterial) "Emissive Intensity" 0.0 :!class /Script/Engine.MaterialInstanceDynamic))

(event Custom|lightPulse)

(event EventBeginPlay
  (bind _level_manager_points (Variables|Default|GetLevel_Manager_Points))
  (bind _level_point (Variables|Default|GetLevel_point))
  (bind _output (Utilities|Array|Get(acopy) _level_manager_points _level_point))
  (bind _outactors (Actor|GetAllActorsOfClass "/Game/Assets/Blueprints/Portal.Portal_C"))
  (bind _outactors_2 (Actor|GetAllActorsOfClass "/Game/Assets/Blueprints/PersonalMCPawn.PersonalMCPawn_C"))
  ;[1 1 1] Reset
  (CallFunction|ResetSphere)
  (Transformation|SetActorTransform (Transformation|GetWorldTransform (Variables|/Game/Assets/Blueprints/LevelManagerPoint.LevelManagerPoint_C|GetOrb_point _output)))
  (Variables|Default|Setrequired_points (Math|Conversions|ToFloat(Integer) (Variables|/Game/Assets/Blueprints/LevelManagerPoint.LevelManagerPoint_C|GetRequired%20points _output))))

(event Collision|EventActorBeginOverlap
  (params (OtherActor :type Actor%20Object%20Reference)))

(event EventTakeDamage
  (params (DamageAmount :type Float%20%28single-precision%29) (Constant :type Boolean) (Effect :type Effects%20Enum :default "NewEnumerator4") (EffectTime :type Float%20%28single-precision%29) (Hit_Location :type Vector :default "0, 0, 0"))
  (bind _level_manager_points (Variables|Default|GetLevel_Manager_Points))
  (bind _level_point (Variables|Default|GetLevel_point))
  (bind _level_point_2 (Variables|Default|GetLevel_point))
  (bind _output (Utilities|Array|Get(acopy) _level_manager_points _level_point))
  (if (Variables|Default|GetPortal_ready)
    (if (== _level_point_2 4)
      (CallFunction|TurnPortalon (Utilities|Array|Get(acopy) (stale EventBeginPlay _outactors)) "Crypt_level")
      (else
        (bind _returnvalue (Game|GetCurrentLevelName true))
        (CallFunction|TurnPortalon (Utilities|Array|Get(acopy) (stale EventBeginPlay _outactors)) _returnvalue)))
    (Default|Progression (Utilities|Array|Get(acopy) (stale EventBeginPlay _outactors_2)) _level_point_2)
    (bind _result (Math|Integer|IncrementInt _level_point_2)
      (:%20%20
        (if (<= _result (- (Utilities|Array|Length (Variables|Default|GetLevel_Manager_Points)) 1))
          ;[1 1 1] Reset
          (CallFunction|ResetSphere)
          (Transformation|SetActorTransform (Transformation|GetWorldTransform (Variables|/Game/Assets/Blueprints/LevelManagerPoint.LevelManagerPoint_C|GetOrb_point _output)))
          (Variables|Default|Setrequired_points (Math|Conversions|ToFloat(Integer) (Variables|/Game/Assets/Blueprints/LevelManagerPoint.LevelManagerPoint_C|GetRequired%20points _output))))))
    (elif (Utilities|Enum|Equal(Enum) (Variables|Default|GetLevelState) "NewEnumerator0")
      (CallFunction|StartRound))))

(event EventTick
  (params (DeltaSeconds :type Float%20%28single-precision%29)))

(fn ConstructionScript
  (bind _wizardskull_rigged (Variables|Default|GetWizardSkull_Rigged))
  (bind _returnvalue (Rendering|Material|CreateDynamicMaterialInstance _wizardskull_rigged 0 (Rendering|Material|GetMaterial _wizardskull_rigged 0) :!class /Script/Engine.PrimitiveComponent))
  (Variables|Default|SetEmissiveMaterial _returnvalue))

(fn StartRound
  (bind _spawnerholder (Variables|Default|GetSpawnerHolder))
  (bind _currentspawnemmiter (Variables|Default|GetCurrentSpawnEmmiter))
  (bind _output (Utilities|Array|Get(acopy) _spawnerholder _currentspawnemmiter))
  (Utilities|IsValid _output
    (:Is%20Valid
      (Variables|/Game/Assets/Blueprints/SpawnController.SpawnController_C|SetEnableSpawning _output true))
    (:Is%20Not%20Valid
      _))
  (Variables|Default|SetLevelState "NewEnumerator1")
  (CallFunction|LightPulse)
  (if (Variables|/Game/Assets/Blueprints/LevelManagerPoint.LevelManagerPoint_C|GetTarget_round (Utilities|Array|Get(acopy) (Variables|Default|GetLevel_Manager_Points) (Variables|Default|GetLevel_point)))
    (bind _outactors (Actor|GetAllActorsOfClass "/Game/Assets/Blueprints/Skull_target.Skull_target_C"))
    (for _array_element _outactors
      (Default|ActivateSkulls _array_element))))

(fn TurnPortalon
  (params (Portal :type Portal%20Object%20Reference) (LevelName :type String))
  (bind _level_manager_points (Variables|Default|GetLevel_Manager_Points))
  (bind _level_point (Variables|Default|GetLevel_point))
  (bind _returnvalue (+ _level_point 1))
  (bind _output (Utilities|Array|Get(acopy) _level_manager_points _returnvalue))
  (Default|ActivatePortal Portal (Transformation|GetWorldLocation (Variables|/Game/Assets/Blueprints/LevelManagerPoint.LevelManagerPoint_C|Getportal_point (Utilities|Array|Get(acopy) _level_manager_points _level_point))))
  (Default|PortalNextLocation Portal (Transformation|GetWorldLocation (Variables|/Game/Assets/Blueprints/LevelManagerPoint.LevelManagerPoint_C|Getportal_point _output)) LevelName)
  (Variables|/Game/Assets/Blueprints/Portal.Portal_C|SetNext_position Portal (Transformation|GetWorldTransform (Variables|/Game/Assets/Blueprints/LevelManagerPoint.LevelManagerPoint_C|Getplayer_point _output)))
  (Variables|Default|SetPortal_ready false))