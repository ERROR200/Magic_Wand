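; Wave spawner actor that runs endless self-timed waves of skeletons and gargoyles, with support for random premade rounds.
; Looping timers spawn weighted random types from a random stream at randomly chosen active spawn points, configured through construction-script toggles.
; After each wave, rates shift from normal skeletons toward tougher types until max difficulty shortens spawn intervals.
; Gargoyles reuse placed gargoyles' transforms, falling back to normal skeletons when all are occupied.
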(event Custom|SpawnEnemy
  (params (AmountToSpawn :type Integer) (RandomSpawnLoc :type Boolean) (SpawnRate :type Float%20%28single-precision%29) (ChangeSpawnEvery :type Float%20%28single-precision%29))
  (Variables|Default|SetSpawningActive true)
  (if (Variables|Default|GetisPremadeRound)
    (Variables|Default|SetSpawnTally_Goal (Variables|Default|GetEnemySpawnedTally))
    (else
      (Variables|Default|SetSpawnTally_Goal AmountToSpawn)))
  (bind _output_get (Variables|Default|SetSpawnOnRandom RandomSpawnLoc))
  (if _output_get
    (Utilities|Time|SetTimerbyFunctionName 0 "SetSpawnLocation" SpawnRate true)
    (else
      (CallFunction|SetSpawnLocation)
      (Utilities|Time|SetTimerbyFunctionName 0 "ContinueToSpawn" SpawnRate true)
      (Utilities|Time|SetTimerbyFunctionName 0 "SetSpawnLocation" ChangeSpawnEvery true))))

(event Custom|SelfSetup
  (bind _mintime (Variables|Default|GetminTime))
  (bind _random (Variables|Default|GetRandom))
  (bind _maxtime (Variables|Default|GetMaxTime))
  (bind _returnvalue (Math|Random|RandomFloatinRangefromStream _mintime _maxtime _random))
  (if (Variables|Default|GetisSelfRunning)
    (CallFunction|SpawnEnemy (Math|Random|RandomIntegerinRangefromStream 6 8 _random) (<= _returnvalue (+ (Variables|Default|GetminTime) 0.5)) _returnvalue (Math|Random|RandomFloatinRangefromStream 2.0 3.0 _random))
    (Variables|Default|SetAfterWaveDelay (Math|Random|RandomFloatinRangefromStream 1.0 2.5 (Variables|Default|GetRandom)))))

(event Custom|SetSpawnLocation
  (bind _spawnlocation (CallFunction|DetermineSpawnLocation))
  (Variables|Default|SetSpawnLoc _spawnlocation)
  (if (Variables|Default|GetSpawnOnRandom)
    (bind (_spawntype _spawncount) (CallFunction|GetSpawnType))
    (if (== _spawncount (Variables|Default|GetEnemySpawnedTally))
      (Math|Integer|IncrementInt (Variables|Default|GetCustomTallyIndex)
        (:%20%20
          _)))
    (Utilities|Casting|CastToGargoyleClass _spawntype
      (:then
        (CallFunction|SpawnGargoyle))
      (:CastFailed
        (Game|SpawnActorfromClass _spawntype (Variables|Default|GetSpawnLoc) "AlwaysSpawn" 0 0)))
    (bind _result (Math|Integer|IncrementInt (Variables|Default|GetSpawnTally))
      (:%20%20
        (if (== _result (Variables|Default|GetSpawnTally_Goal))
          (Utilities|Time|ClearTimerbyFunctionName 0 "SetSpawnLocation")
          (Utilities|Time|ClearTimerbyFunctionName 0 "ContinueToSpawn")
          (Variables|Default|SetSpawningActive false)
          (Variables|Default|SetSpawnTally 0)
          (if (Variables|Default|GetisSelfRunning)
            (Math|Integer|IncrementInt (Variables|Default|GetWaveTally)
              (:%20%20
                (CallFunction|AdjustRates)
                (Utilities|FlowControl|Delay (Variables|Default|GetAfterWaveDelay))
                (CallFunction|SelfSetup)))))))))

(event Custom|StopSpawningOverride
  (Variables|Default|SetisSelfRunning false)
  (Utilities|Time|ClearTimerbyFunctionName 0 "SetSpawnLocation")
  (Utilities|Time|ClearTimerbyFunctionName 0 "ContinueToSpawn"))

(event Custom|ContinueToSpawn
  (bind (_spawntype _spawncount) (CallFunction|GetSpawnType))
  (if (== _spawncount (Variables|Default|GetEnemySpawnedTally))
    (Math|Integer|IncrementInt (Variables|Default|GetCustomTallyIndex)
      (:%20%20
        _)))
  (Utilities|Casting|CastToGargoyleClass _spawntype
    (:then
      (CallFunction|SpawnGargoyle))
    (:CastFailed
      (Game|SpawnActorfromClass _spawntype (Variables|Default|GetSpawnLoc) "AlwaysSpawn" 0 0)))
  (bind _result (Math|Integer|IncrementInt (Variables|Default|GetSpawnTally))
    (:%20%20
      (if (== _result (Variables|Default|GetSpawnTally_Goal))
        (Utilities|Time|ClearTimerbyFunctionName 0 "SetSpawnLocation")
        (Utilities|Time|ClearTimerbyFunctionName 0 "ContinueToSpawn")
        (Variables|Default|SetSpawningActive false)
        (Variables|Default|SetSpawnTally 0)
        (if (Variables|Default|GetisSelfRunning)
          (Math|Integer|IncrementInt (Variables|Default|GetWaveTally)
            (:%20%20
              (CallFunction|AdjustRates)
              (Utilities|FlowControl|Delay (Variables|Default|GetAfterWaveDelay))
              (CallFunction|SelfSetup))))))))

(event Custom|SetCustomRound
  (Variables|Default|SetisPremadeRound true)
  (Variables|Default|SetCustomWaveIndex (Math|Random|RandomIntegerinRangefromStream 0 (- (Utilities|Array|Length (Variables|Default|GetPreMadeWaves)) 1) (Variables|Default|GetRandom)))
  (CallFunction|TallyEnemies))

(event EventBeginPlay
  (Class|KismetMathLibrary|SeedRandomStream (Variables|Default|GetRandom))
  (bind _astracking_game_instance (Utilities|Casting|CastToTracking_GameInstance (Game|GetGameInstance)))
  (Utilities|FlowControl|Sequence
    (:then_0
      (Variables|Default|SetShieldRate 15))
    (:then_1
      (Utilities|Map|Add (Variables|Default|GetSpawnRates) "/Game/Assets/Blueprints/Skeleton_Normal.Skeleton_Normal_C" (Variables|Default|GetNormalRate))
      (Utilities|Map|Add (Variables|Default|GetSpawnRates) "/Game/Assets/Blueprints/Skeleton_Speedy.Skeleton_Speedy_C" (Variables|Default|GetSpeedyRate))
      (Utilities|Map|Add (Variables|Default|GetSpawnRates) "/Game/Assets/Blueprints/Skeleton_Strong.Skeleton_Strong_C" (Variables|Default|GetShieldRate)))
    (:then_2
      (Utilities|Map|Add (Variables|Default|GetSpawnRates) "/Game/Assets/Blueprints/Gargoyle.Gargoyle_C" (Variables|Default|GetGargoyleRate))
      (Variables|Default|SetisSelfRunning true)
      (CallFunction|GetGargoyleSpawns)
      (Utilities|FlowControl|Delay (Variables|Default|GetStartingDelay))
      (CallFunction|SelfSetup))))

(event Collision|EventActorBeginOverlap
  (params (OtherActor :type Actor%20Object%20Reference)))

(event EventTick
  (params (DeltaSeconds :type Float%20%28single-precision%29)))

(fn ConstructionScript
  (Variables|Default|SetSpawnRefs (Utilities|Array|MakeArray (Variables|Default|GetSpawnLocation1) (Variables|Default|GetSpawnLocation2) (Variables|Default|GetSpawnLocation3) (Variables|Default|GetSpawnLocation4) (Variables|Default|GetSpawnLocation5) (Variables|Default|GetSpawnLocation6) (Variables|Default|GetSpawnLocation7) (Variables|Default|GetSpawnLocation8) (Variables|Default|GetSpawnLocation9) (Variables|Default|GetSpawnLocation10)))
  (if (Variables|Default|GetRemoveSpawn)
    (if (> (Variables|Hidden|GetActiveSpawns) 1)
      (Math|Integer|DecrementInt (Variables|Hidden|GetActiveSpawns)
        (:%20%20
          _)))
    (Variables|Default|SetRemoveSpawn false)
    (elif (Variables|Default|GetAddSpawn)
      (if (< (Variables|Hidden|GetActiveSpawns) 10)
        (Math|Integer|IncrementInt (Variables|Hidden|GetActiveSpawns)
          (:%20%20
            _)))
      (Variables|Default|SetAddSpawn false)))
  (for _index (range 0 (- (Variables|Hidden|GetActiveSpawns) 1))
    (Rendering|SetVisibility (Utilities|Array|Get(acopy) (Variables|Default|GetSpawnRefs) _index) true false)))

(fn GetSpawnType
  (bind _customtallyindex (Variables|Default|GetCustomTallyIndex))
  (bind _premadewaves (Variables|Default|GetPreMadeWaves))
  (bind _customwaveindex (Variables|Default|GetCustomWaveIndex))
  (bind _random (Variables|Default|GetRandom))
  (bind _returnvalue (Math|Random|RandomIntegerinRangefromStream 0 100 _random))
  (bind _output (Utilities|Array|Get(acopy) _premadewaves _customwaveindex))
  (bind _enemytype (Utilities|Struct|BreakWaveEnemies _output))
  (bind _output_2 (Utilities|Array|Get(acopy) _enemytype _customtallyindex))
  (bind (_enemytype_2 _numberofenemies) (Utilities|Struct|BreakNumOfEnemies _output_2))
  (if (not (Variables|Default|GetisPremadeRound))
    (bind _values (Utilities|Map|Values (Variables|Default|GetSpawnRates)))
    (if (<= _returnvalue (Utilities|Array|Get(acopy) _values))
      (return "/Game/Assets/Blueprints/Skeleton_Normal.Skeleton_Normal_C" -1)
      (elif (<= _returnvalue (+ (Utilities|Array|Get(acopy) _values) (Utilities|Array|Get(acopy) _values 1)))
        (return "/Game/Assets/Blueprints/Skeleton_Speedy.Skeleton_Speedy_C" -1)
        (elif (<= _returnvalue (+ (+ (Utilities|Array|Get(acopy) _values) (Utilities|Array|Get(acopy) _values 1)) (Utilities|Array|Get(acopy) _values 2)))
          (bind _shieldtype (CallFunction|GetShieldSpawn))
          (return _shieldtype -1)
          (else
            (return "/Game/Assets/Blueprints/Gargoyle.Gargoyle_C" -1)))))
    (else
      (return _enemytype_2 _numberofenemies))))

(fn CheckSpawnRates
  (bind _values (Utilities|Map|Values (Variables|Default|GetSpawnRates)))
  (if (!= (+ (Utilities|Array|Get(acopy) _values) (Utilities|Array|Get(acopy) _values 1) (Utilities|Array|Get(acopy) _values 2)) 100)
    (Utilities|Map|Add (Variables|Default|GetSpawnRates) "/Game/Assets/Blueprints/Skeleton_Normal.Skeleton_Normal_C" (+ (Utilities|Array|Get(acopy) _values) (- 100 (+ (Utilities|Array|Get(acopy) _values) (Utilities|Array|Get(acopy) _values 1) (Utilities|Array|Get(acopy) _values 2)))))))

(fn ChangeSpawnChance
  (params (NormalSpawnRate :type Integer) (SpeedySpawnRate :type Integer) (ShieldSpawnRate :type Integer))
  (Utilities|Map|Add (Variables|Default|GetSpawnRates) "/Game/Assets/Blueprints/Skeleton_Normal.Skeleton_Normal_C" NormalSpawnRate)
  (Utilities|Map|Add (Variables|Default|GetSpawnRates) "/Game/Assets/Blueprints/Skeleton_Speedy.Skeleton_Speedy_C" SpeedySpawnRate)
  (Utilities|Map|Add (Variables|Default|GetSpawnRates) "/Game/Assets/Blueprints/Skeleton_Strong.Skeleton_Strong_C" ShieldSpawnRate)
  (CallFunction|CheckSpawnRates))

(fn GetShieldSpawn
  (bind _random (Variables|Default|GetRandom))
  (bind _returnvalue (Math|Random|RandomIntegerinRangefromStream 0 100 _random))
  (if (<= _returnvalue 33)
    ;[1 1 1] Wood
    (return "/Game/Assets/Blueprints/Skeleton_Strong.Skeleton_Strong_C")
    (elif (<= _returnvalue 66)
      ;[1 1 1] Ice
      (return "/Game/Assets/Blueprints/Skeleton_Strong_ice.Skeleton_Strong_ice_C")
      (else
        ;[1 1 1] Stone
        (return "/Game/Assets/Blueprints/Skeleton_Strong_Stone.Skeleton_Strong_Stone_C")))))

(fn DetermineSpawnLocation
  (return (Transformation|GetWorldTransform (Utilities|Array|Get(acopy) (Variables|Default|GetSpawnRefs) (Math|Random|RandomIntegerinRangefromStream 0 (- (Variables|Hidden|GetActiveSpawns) 1) (Variables|Default|GetRandom))))))

(fn TallyEnemies
  (for _array_element (Utilities|Struct|BreakWaveEnemies (Utilities|Array|Get(acopy) (Variables|Default|GetPreMadeWaves) (Variables|Default|GetCustomWaveIndex)))
    (if (> (.NumberOfEnemies (Utilities|Struct|BreakNumOfEnemies _array_element)) 1)
      (Variables|Default|SetEnemySpawnedTally (+ (.NumberOfEnemies (Utilities|Struct|BreakNumOfEnemies _array_element)) (Variables|Default|GetEnemySpawnedTally)))
      (else
        (Math|Integer|IncrementInt (Variables|Default|GetEnemySpawnedTally))))))

(fn AdjustRates
  (if (not (Variables|Default|GetmaxDifficultly))
    (Utilities|FlowControl|Sequence
      (:then_0
        (CallFunction|ChangeRateValue (Variables|Default|GetSpeedyMaxRate) (Variables|Default|GetSpeedyRate) 1))
      (:then_1
        (CallFunction|ChangeRateValue (Variables|Default|GetShieldMaxRate) (Variables|Default|GetShieldRate) 1))
      (:then_2
        (CallFunction|ChangeRateValue (Variables|Default|GetGargoyleMaxRate) (Variables|Default|GetGargoyleRate) 0))
      (:then_3
        (if (<= (Variables|Default|GetNormalRate) (Variables|Default|GetNormalMinRate))
          (Variables|Default|SetNormalRate (Variables|Default|GetNormalMinRate))))
      (:then_4
        (Utilities|Map|Add (Variables|Default|GetSpawnRates) "/Game/Assets/Blueprints/Skeleton_Normal.Skeleton_Normal_C" (Variables|Default|GetNormalRate))
        (Utilities|Map|Add (Variables|Default|GetSpawnRates) "/Game/Assets/Blueprints/Skeleton_Speedy.Skeleton_Speedy_C" (Variables|Default|GetSpeedyRate))
        (Utilities|Map|Add (Variables|Default|GetSpawnRates) "/Game/Assets/Blueprints/Skeleton_Strong.Skeleton_Strong_C" (Variables|Default|GetShieldRate))
        (Utilities|Map|Add (Variables|Default|GetSpawnRates) "/Game/Assets/Blueprints/Gargoyle.Gargoyle_C" (Variables|Default|GetGargoyleRate))
        (if (and (== (Variables|Default|GetSpeedyRate) (Variables|Default|GetSpeedyMaxRate)) (== (Variables|Default|GetShieldRate) (Variables|Default|GetShieldMaxRate)))
          (Variables|Default|SetmaxDifficultly true)
          (Variables|Default|SetGargoyleRate (Variables|Default|GetGargoyleMaxRate))
          (Variables|Default|SetNormalRate (Variables|Default|GetNormalMinRate))
          (Variables|Default|SetminTime 0.7)
          (Variables|Default|SetMaxTime 1.5)
          (elif (== (Variables|Default|GetWaveTally) 20)
            (Variables|Default|SetMaxTime 2.4)))))))

(fn ChangeRateValue
  (params (MaxRate :type Integer) (Rate :type Integer%20%28by%20ref%29) (MinValue :type Integer))
  (if (!= MaxRate Rate)
    (LocalVariables|SetRandomNumber (Math|Random|RandomIntegerinRangefromStream MinValue 2 (Variables|Default|GetRandom)))
    (|SetBy-RefVar Rate (+ Rate (LocalVariables|GetRandomNumber)))
    (if (> Rate MaxRate)
      (Variables|Default|SetNormalRate (- (Variables|Default|GetNormalRate) (- (LocalVariables|GetRandomNumber) (- Rate (Variables|Default|GetSpeedyMaxRate)))))
      (|SetBy-RefVar Rate MaxRate)
      (else
        (Variables|Default|SetNormalRate (- (Variables|Default|GetNormalRate) (LocalVariables|GetRandomNumber)))))))

(fn SpawnGargoyle
  (bind _transforms (LocalVariables|GetTransforms))
  (bind _return (CallFunction|CheckforGargoyles (Variables|Default|GetBox)))
  (if _return
    (Utilities|Array|Add (LocalVariables|GetTransforms) (Transformation|GetWorldTransform (Variables|Default|GetGargoyleSpawn1))))
  (bind _return_2 (CallFunction|CheckforGargoyles (Variables|Default|GetBox1)))
  (if _return_2
    (Utilities|Array|Add (LocalVariables|GetTransforms) (Transformation|GetWorldTransform (Variables|Default|GetGargoyleSpawn2))))
  (bind _return_3 (CallFunction|CheckforGargoyles (Variables|Default|GetBox2)))
  (if _return_3
    (Utilities|Array|Add (LocalVariables|GetTransforms) (Transformation|GetWorldTransform (Variables|Default|GetGargoyleSpawn3))))
  (if (> (Utilities|Array|Length _transforms) 0)
    (Game|SpawnActorfromClass "/Game/Assets/Blueprints/Gargoyle.Gargoyle_C" (Utilities|Array|Get(acopy) (LocalVariables|GetTransforms) (Math|Random|RandomIntegerinRangefromStream 0 (Utilities|Array|LastIndex _transforms) (Variables|Default|GetRandom))) "AlwaysSpawn" 0 true 0)
    (else
      (Game|SpawnActorfromClass "/Game/Assets/Blueprints/Skeleton_Normal.Skeleton_Normal_C" (Variables|Default|GetSpawnLoc) "AlwaysSpawn" 0 0))))

(fn GetGargoyleSpawns
  (bind _outactors (Actor|GetAllActorsOfClass "/Game/Assets/Blueprints/Gargoyle.Gargoyle_C"))
  (Utilities|FlowControl|Sequence
    (:then_0
      (Utilities|IsValid (Utilities|Array|Get(acopy) _outactors)
        (:Is%20Valid
          (Transformation|SetWorldTransform (Variables|Default|GetGargoyleSpawn1) (Transformation|GetActorTransform (Utilities|Array|Get(acopy) _outactors)) false false))))
    (:then_1
      (Utilities|IsValid (Utilities|Array|Get(acopy) _outactors 1)
        (:Is%20Valid
          (Transformation|SetWorldTransform (Variables|Default|GetGargoyleSpawn2) (Transformation|GetActorTransform (Utilities|Array|Get(acopy) _outactors 1)) false false))))
    (:then_2
      (Utilities|IsValid (Utilities|Array|Get(acopy) _outactors 2)
        (:Is%20Valid
          (Transformation|SetWorldTransform (Variables|Default|GetGargoyleSpawn3) (Transformation|GetActorTransform (Utilities|Array|Get(acopy) _outactors 2)) false false))))
    (:then_3
      (for _array_element _outactors
        (Actor|DestroyActor _array_element)))))

(fn CheckforGargoyles
  (params (Box :type Primitive%20Component%20Object%20Reference%20%28by%20ref%29))
  (return (== (Utilities|Array|Length (Collision|GetOverlappingActors Box "/Game/Assets/Blueprints/Gargoyle.Gargoyle_C" :!class /Script/Engine.PrimitiveComponent)) 0)))