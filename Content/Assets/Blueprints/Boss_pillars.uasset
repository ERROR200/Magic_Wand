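; Destructible boss pillar that flashes a light and breaks apart, both on BeginPlay and when its health runs out.
; TakeDamage subtracts either a one-off amount or a delta-time-scaled amount for constant damage.
; The shared break sequence removes the decal, flashes the light, then damages the destructible mesh and fires a radial impulse at the hit location.
; Five seconds later, the debris stops colliding.
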(event Collision|EventActorBeginOverlap
  (params (OtherActor :type Actor%20Object%20Reference)))

(event EventTick
  (params (DeltaSeconds :type Float%20%28single-precision%29)))

(event EventBeginPlay
  (bind _radialforce (Variables|Default|GetRadialForce))
  (bind _cryptlevel_asset_pillar_dm (Variables|Default|Getcryptlevel_asset_pillar_DM))
  (bind _pointlight (Variables|Default|GetPointLight))
  (Components|DestroyComponent (Variables|Default|GetDecal))
  (Rendering|Components|Light|SetIntensity _pointlight 5e+04)
  (Utilities|FlowControl|Delay 0.5)
  (Rendering|Components|Light|SetIntensity _pointlight 0.0)
  (Collision|SetCollisionObjectType _cryptlevel_asset_pillar_dm "ECC_WorldDynamic")
  (Collision|SetCollisionResponsetoAllChannels _cryptlevel_asset_pillar_dm "ECR_Block")
  (Class|DestructibleComponent|ApplyDamage _cryptlevel_asset_pillar_dm 1e+01 (stale EventTakeDamage Hit_Location) (stale EventTakeDamage Hit_Location) 0.0)
  (Transformation|SetWorldLocation _radialforce (stale EventTakeDamage Hit_Location) false false)
  (Class|RadialForceComponent|FireImpulse _radialforce)
  (Utilities|FlowControl|Delay 5.0)
  (Collision|SetCollisionObjectType _cryptlevel_asset_pillar_dm "ECC_Destructible")
  (Collision|SetCollisionResponsetoAllChannels _cryptlevel_asset_pillar_dm "ECR_Ignore"))

(event EventTakeDamage
  (params (DamageAmount :type Float%20%28single-precision%29) (Constant :type Boolean) (Effect :type Effects%20Enum :default "NewEnumerator4") (EffectTime :type Float%20%28single-precision%29) (Hit_Location :type Vector :default "0, 0, 0"))
  (bind _radialforce (Variables|Default|GetRadialForce))
  (bind _cryptlevel_asset_pillar_dm (Variables|Default|Getcryptlevel_asset_pillar_DM))
  (bind _pointlight (Variables|Default|GetPointLight))
  (if Constant
    (Variables|Default|SetHealth (- (Variables|Default|GetHealth) (* DamageAmount (Utilities|Time|GetWorldDeltaSeconds))))
    (else
      (Variables|Default|SetHealth (- (Variables|Default|GetHealth) DamageAmount))))
  (if (<= (Variables|Default|GetHealth) 0.0)
    (Components|DestroyComponent (Variables|Default|GetDecal))
    (Rendering|Components|Light|SetIntensity _pointlight 5e+04)
    (Utilities|FlowControl|Delay 0.5)
    (Rendering|Components|Light|SetIntensity _pointlight 0.0)
    (Collision|SetCollisionObjectType _cryptlevel_asset_pillar_dm "ECC_WorldDynamic")
    (Collision|SetCollisionResponsetoAllChannels _cryptlevel_asset_pillar_dm "ECR_Block")
    (Class|DestructibleComponent|ApplyDamage _cryptlevel_asset_pillar_dm 1e+01 Hit_Location Hit_Location 0.0)
    (Transformation|SetWorldLocation _radialforce Hit_Location false false)
    (Class|RadialForceComponent|FireImpulse _radialforce)
    (Utilities|FlowControl|Delay 5.0)
    (Collision|SetCollisionObjectType _cryptlevel_asset_pillar_dm "ECC_Destructible")
    (Collision|SetCollisionResponsetoAllChannels _cryptlevel_asset_pillar_dm "ECR_Ignore")))

(fn ConstructionScript)