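; Smashable carved pumpkin actor that breaks apart through a Destructible component when it takes damage.
; TakeDamage applies damage to the Destructible, scaling it by frame delta time when flagged as constant, and passes the hit location as both hit point and impulse direction.
; On first fracture only, it spawns an explosion particle and squish sound at the Sphere component, then destroys that component.
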(event OnComponentFracture(Destructible)
  (params (HitPoint :type Vector%20%28by%20ref%29 :default "0, 0, 0") (HitDirection :type Vector%20%28by%20ref%29 :default "0, 0, 0"))
  (bind _sphere (Variables|Default|GetSphere))
  (bind _returnvalue (Transformation|GetWorldLocation _sphere))
  (Utilities|FlowControl|DoOnce false
    (:Completed
      (Effects|SpawnEmitteratLocation "/Game/Assets/Particles/Necro/Skeleton_normal_Boom.Skeleton_normal_Boom" _returnvalue)
      (Audio|PlaySoundatLocation "/Game/Assets/Sounds/OtherSounds/squish_Cue.squish_Cue" _returnvalue)
      (Components|DestroyComponent _sphere))))

(event EventBeginPlay)

(event Collision|EventActorBeginOverlap
  (params (OtherActor :type Actor%20Object%20Reference)))

(event EventTick
  (params (DeltaSeconds :type Float%20%28single-precision%29)))

(event EventTakeDamage
  (params (DamageAmount :type Float%20%28single-precision%29) (Constant :type Boolean) (Effect :type Effects%20Enum :default "NewEnumerator4") (EffectTime :type Float%20%28single-precision%29) (Hit_Location :type Vector :default "0, 0, 0"))
  (if Constant
    (Variables|Default|Setdamage (* DamageAmount (Utilities|Time|GetWorldDeltaSeconds)))
    (else
      (Variables|Default|Setdamage DamageAmount)))
  (Class|DestructibleComponent|ApplyDamage (Variables|Default|GetDestructible) (Variables|Default|Getdamage) Hit_Location Hit_Location 1.0))

(fn ConstructionScript)