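; MenuFlag is a flag actor that displays tutorial instructions, with material variants for Steam VR controls.
; BeginPlay builds a dynamic material from the grab/activate tutorial instance matching the HMD and applies it to the flag mesh.
; GetNextMaterial maps MaterialIndex to the wand, shield, bag or food step, returning its material, audio and duration.
; The shield and bag steps also set player flags (CanGetShield, EatTrigger), and the shield material varies by headset.
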(event EventBeginPlay
  (switch name (Class|HeadMountedDisplayFunctionLibrary|GetHMDDeviceName)
    (:Default
      (bind _returnvalue (Rendering|Material|CreateDynamicMaterialInstance (Variables|Default|GetFlag_Test) 1 "/Game/Assets/Art/Flag/Tutorial/GrabActivate_FlagTutInst.GrabActivate_FlagTutInst" :!class /Script/Engine.PrimitiveComponent :!label _label))
      (Variables|Default|SetDynamicMat _returnvalue)
      (Rendering|Material|SetMaterial (Variables|Default|GetFlag_Test) 0 (Variables|Default|GetDynamicMat)))
    (:OculusHMD
      (goto _label))
    (:SteamVR
      (bind _returnvalue_2 (Rendering|Material|CreateDynamicMaterialInstance (Variables|Default|GetFlag_Test) 1 "/Game/Assets/Art/Flag/Tutorial/GrabActivateVive_FlagTutInst.GrabActivateVive_FlagTutInst" :!class /Script/Engine.PrimitiveComponent))
      (Variables|Default|SetDynamicMat _returnvalue_2)
      (Rendering|Material|SetMaterial (Variables|Default|GetFlag_Test) 0 (Variables|Default|GetDynamicMat)))))

(event Collision|EventActorBeginOverlap
  (params (OtherActor :type Actor%20Object%20Reference)))

(event EventTick
  (params (DeltaSeconds :type Float%20%28single-precision%29)))

(fn ConstructionScript)

(fn GetNextMaterial
  (bind _wandaudio (Variables|Default|GetWandAudio))
  (bind _shieldaudio (Variables|Default|GetShieldAudio))
  (bind _bagaudio (Variables|Default|GetBagAudio))
  (bind _playerref (Variables|Default|GetPlayerRef))
  (bind _foodaudio (Variables|Default|GetFoodAudio))
  (bind _shieldaudio_2 (Variables|Default|GetShieldAudio))
  (switch int (Variables|Default|GetMaterialIndex)
    (:0
      (return (Variables|Default|GetWandMat) _wandaudio (Variables|/Script/Engine.SoundBase|GetDuration _wandaudio)))
    (:1
      (Utilities|IsValid _playerref
        (:Is%20Valid
          (Variables|/Game/Assets/Blueprints/PersonalMCPawn.PersonalMCPawn_C|SetCanGetShield _playerref true)
          (switch name (Class|HeadMountedDisplayFunctionLibrary|GetHMDDeviceName)
            (:Default
              _)
            (:OculusHMD
              _)
            (:SteamVR
              (return (Variables|Default|GetShieldMat_Vive) _shieldaudio (Variables|/Script/Engine.SoundBase|GetDuration _shieldaudio)))))
        (:Is%20Not%20Valid
          _))
      (return (Variables|Default|GetShieldMat) _shieldaudio_2 (Variables|/Script/Engine.SoundBase|GetDuration _shieldaudio_2)))
    (:2
      (Utilities|IsValid _playerref
        (:Is%20Valid
          (Variables|/Game/Assets/Blueprints/PersonalMCPawn.PersonalMCPawn_C|SeteatTrigger _playerref true))
        (:Is%20Not%20Valid
          _))
      (return (Variables|Default|GetBagMat) _bagaudio (Variables|/Script/Engine.SoundBase|GetDuration _bagaudio)))
    (:3
      (return (Variables|Default|GetFoodMat) _foodaudio (Variables|/Script/Engine.SoundBase|GetDuration _foodaudio)))))