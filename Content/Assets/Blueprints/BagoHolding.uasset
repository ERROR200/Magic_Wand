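; VR bag of holding that hands the player a random item when a motion controller grabs it.
; Pickup spawns a random ObjectList class via a seeded stream, attaches it to the grabbing controller and records it as that controller's AttachedActor.
; Controller overlap on the pouch fires a burst effect and plays a timeline raising the dynamic material's emissive intensity, reversed on exit.
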(event OnComponentBeginOverlap(Cube1)
  (params (OverlappedComponent :type Primitive%20Component%20Object%20Reference) (OtherActor :type Actor%20Object%20Reference) (OtherComp :type Primitive%20Component%20Object%20Reference) (OtherBodyIndex :type Integer) (bFromSweep :type Boolean) (SweepResult :type Hit%20Result%20Structure%20%28by%20ref%29))
  (Utilities|Casting|CastToBP_MotionController OtherActor)
  (Components|Activation|Activate (Variables|Default|GetBag_o_holding_burst) true)
  (bind _emissive (Timeline|emis Play)
    (:Update
      (Rendering|Material|SetScalarParameterValue (Variables|Default|Getpouch%20material) "Emissive Intensity" _emissive :!class /Script/Engine.MaterialInstanceDynamic))))

(event OnComponentEndOverlap(Cube1)
  (params (OverlappedComponent :type Primitive%20Component%20Object%20Reference) (OtherActor :type Actor%20Object%20Reference) (OtherComp :type Primitive%20Component%20Object%20Reference) (OtherBodyIndex :type Integer))
  (Utilities|Casting|CastToBP_MotionController OtherActor)
  (bind _emissive (Timeline|emis Reverse)
    (:Update
      (Rendering|Material|SetScalarParameterValue (Variables|Default|Getpouch%20material) "Emissive Intensity" _emissive :!class /Script/Engine.MaterialInstanceDynamic))))

(event EventBeginPlay
  (Class|KismetMathLibrary|SeedRandomStream (Variables|Default|Getstream))
  (bind _returnvalue (Rendering|Material|CreateDynamicMaterialInstance (Variables|Default|GetCube1) 0 "/Game/Assets/Art/Pouch/Pouch_MatInst.Pouch_MatInst" :!class /Script/Engine.PrimitiveComponent))
  (Variables|Default|Setpouch%20material _returnvalue))

(event EventPickup
  (params (AttachTo :type Scene%20Component%20Object%20Reference) (hand :type EControllerHand%20Enum :default "Left"))
  (bind _object_list (Variables|Default|Getobject_list))
  (bind _returnvalue (Game|SpawnActorfromClass (Utilities|Array|Get(acopy) _object_list (Math|Random|RandomIntegerinRangefromStream 0 (- (Utilities|Array|Length _object_list) 1) (Variables|Default|Getstream))) (Transformation|GetActorTransform) "AlwaysSpawn" 0 0))
  (bind _asbp_motion_controller (Utilities|Casting|CastToBP_MotionController (Components|GetOwner AttachTo))
    (:then
      (Class|PickupActorInterface|Pickup(Message) _returnvalue AttachTo "Left")
      (Variables|/Game/VirtualRealityBP/Blueprints/BP_MotionController.BP_MotionController_C|SetAttachedActor _asbp_motion_controller _returnvalue))
    (:CastFailed
      (Development|PrintString "bag fail"))))

(fn ConstructionScript)