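; Tutorial actor that demonstrates spell gestures and grip or trigger presses using rigged hands and Oculus controller models.
; SetHandAnim and SetControllerAnim store the animation, side and visibility, then Tick replays it through delayed DoOnce gates and SelectAnimation.
; Controller button highlights use a timeline to drive emissive parameters on dynamic materials created in the construction script.
; StopAnimations clears the play flags and hides the hands after a short delay.
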(event Custom|ButtonHighlights
  (params (Anim :type TutorialAnimation%20Enum :default "NewEnumerator7") (Value :type Float%20%28single-precision%29) (Material :type Material%20Instance%20Dynamic%20Object%20Reference))
  (switch Utilities|FlowControl|Switch|SwitchonTutorialAnimation Anim
    (:NewEnumerator6
      (Variables|Default|SetParameter "GripButton Emissive Intensity")
      (bind _newtrack_0 (Timeline|Timeline_0 PlayFromStart)
        (:Update
          (Rendering|Material|SetScalarParameterValue Material (Variables|Default|GetParameter) (* _newtrack_0 Value) :!class /Script/Engine.MaterialInstanceDynamic))))
    (:NewEnumerator4
      (Variables|Default|SetParameter "Trigger Emissive Intensity")
      (Timeline|Timeline_0 PlayFromStart))))

(event Custom|SetControllerAnim
  (params (Anim :type TutorialAnimation%20Enum :default "NewEnumerator7") (Visible :type Boolean) (isLeftHand :type Boolean))
  (Variables|Default|SetcontrollerAnim Anim)
  (Variables|Default|SetvisibleController Visible)
  (Variables|Default|SetisRightHand isLeftHand)
  (Variables|Default|SetcanPlayController true))

(event Custom|AnimateControl
  (params (Anim :type TutorialAnimation%20Enum :default "NewEnumerator7") (isLeft :type Boolean) (Visible :type Boolean))
  (Utilities|FlowControl|DoOnce false :!label _label
    (:Completed
      (if isLeft
        (CallFunction|ButtonHighlights Anim 1e+01 (Variables|Default|GetDynamicMat_LeftController))
        (Utilities|FlowControl|Delay 1.0)
        (CallFunction|SelectAnimation Anim (Variables|Default|GetOculusController_Rigged_Left) 0 false Visible)
        (else
          (CallFunction|ButtonHighlights Anim 1e+01 (Variables|Default|GetDynamicMat_RightController))
          (Utilities|FlowControl|Delay 1.0)
          (CallFunction|SelectAnimation Anim (Variables|Default|GetOculusController_Rigged) 0 false Visible)))
      (Utilities|FlowControl|Delay 2.0)
      (goto _label Reset))))

(event Custom|SetHandAnim
  (params (Anim :type TutorialAnimation%20Enum :default "NewEnumerator7") (Visible :type Boolean) (isLeftHand :type Boolean))
  (Variables|Default|SethandAnim Anim)
  (Variables|Default|SetvisibleHand Visible)
  (Variables|Default|SetisLeftHand isLeftHand)
  (Variables|Default|SetcanPlayHand true))

(event Custom|StopAnimations
  (Variables|Default|SetcanPlayHand false)
  (Variables|Default|SetcanPlayController false)
  (CallFunction|ButtonHighlights "NewEnumerator7" 1.0 (Variables|Default|GetDynamicMat_LeftController))
  (CallFunction|ButtonHighlights "NewEnumerator7" 1.0 (Variables|Default|GetDynamicMat_RightController))
  (Utilities|FlowControl|Delay 1.0)
  (Rendering|SetVisibility (Variables|Default|GetHandRigged_Left) false true)
  (Rendering|SetVisibility (Variables|Default|GetHandRigged) false true))

(event Custom|AnimateHand
  (params (Anim :type TutorialAnimation%20Enum :default "NewEnumerator7") (isLeft :type Boolean) (Visible :type Boolean))
  (Utilities|FlowControl|DoOnce false :!label _label
    (:Completed
      (Utilities|FlowControl|Delay 1.0)
      (if isLeft
        (CallFunction|SelectAnimation Anim 0 (Variables|Default|GetHandRigged_Left) true Visible)
        (else
          (CallFunction|SelectAnimation Anim 0 (Variables|Default|GetHandRigged) true Visible)))
      (Utilities|FlowControl|Delay 2.0)
      (goto _label Reset))))

(event EventBeginPlay
  (Rendering|SetVisibility (Variables|Default|GetHandRigged_Left) false true)
  (Rendering|SetVisibility (Variables|Default|GetHandRigged) false true))

(event Collision|EventActorBeginOverlap
  (params (OtherActor :type Actor%20Object%20Reference)))

(event EventTick
  (params (DeltaSeconds :type Float%20%28single-precision%29))
  (if (Variables|Default|GetcanPlayHand)
    (CallFunction|AnimateHand (Variables|Default|GethandAnim) (Variables|Default|GetisLeftHand) (Variables|Default|GetvisibleHand)))
  (if (Variables|Default|GetcanPlayController)
    (CallFunction|AnimateControl (Variables|Default|GetcontrollerAnim) (Variables|Default|GetisRightHand) (Variables|Default|GetvisibleController))))

(fn ConstructionScript
  (bind _oculuscontroller_rigged_left (Variables|Default|GetOculusController_Rigged_Left))
  (bind _oculuscontroller_rigged (Variables|Default|GetOculusController_Rigged))
  (bind _returnvalue (Rendering|Material|CreateDynamicMaterialInstance _oculuscontroller_rigged_left 0 (Rendering|Material|GetMaterial _oculuscontroller_rigged_left 0) :!class /Script/Engine.PrimitiveComponent))
  (Variables|Default|SetDynamicMat_LeftController _returnvalue)
  (bind _returnvalue_2 (Rendering|Material|CreateDynamicMaterialInstance _oculuscontroller_rigged 0 (Rendering|Material|GetMaterial _oculuscontroller_rigged 0) :!class /Script/Engine.PrimitiveComponent))
  (Variables|Default|SetDynamicMat_RightController _returnvalue_2))

(fn SelectAnimation
  (params (Anim :type TutorialAnimation%20Enum :default "NewEnumerator7") (Controller :type Skeletal%20Mesh%20Component%20Object%20Reference) (Hand :type Skeletal%20Mesh%20Component%20Object%20Reference) (displayHand :type Boolean) (Visible :type Boolean))
  (if Visible
    (if displayHand
      (Rendering|SetVisibility Hand true false)
      (else
        (Rendering|SetVisibility Controller true false))))
  (switch Utilities|FlowControl|Switch|SwitchonTutorialAnimation Anim
    (:NewEnumerator6
      (Components|Animation|PlayAnimation Controller "/Game/Assets/Art/OculusController/OculusController_GripAnim.OculusController_GripAnim" false))
    (:NewEnumerator4
      (Components|Animation|PlayAnimation Controller "/Game/Assets/Art/OculusController/OculusController_TriggerAnim.OculusController_TriggerAnim" false))
    (:NewEnumerator0
      (Components|Animation|PlayAnimation Hand "/Game/Assets/Art/Hand/TutorialAnimations/TutorialHand_ArcaneBlastAnim.TutorialHand_ArcaneBlastAnim" false))
    (:NewEnumerator1
      (Components|Animation|PlayAnimation Hand "/Game/Assets/Art/Hand/TutorialAnimations/TutorialHand_FireballAnim.TutorialHand_FireballAnim" false))
    (:NewEnumerator2
      (Components|Animation|PlayAnimation Hand "/Game/Assets/Art/Hand/TutorialAnimations/TutorialHand_LightningAnim.TutorialHand_LightningAnim" false))
    (:NewEnumerator3
      (Components|Animation|PlayAnimation Hand "/Game/Assets/Art/Hand/TutorialAnimations/TutorialHand_BlizzardAnim.TutorialHand_BlizzardAnim" false))))

(fn HideAnimation)