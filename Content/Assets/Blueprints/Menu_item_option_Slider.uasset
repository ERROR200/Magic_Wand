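; VR options-menu slider for Master, Music or SFX volume, shown and collidable only while Active.
; Taking damage loads or creates the "Options" save, attaches the physics-enabled mesh to the right-hand controller and opens a Tick gate.
; Each tick writes a fixed full volume for its item type, not the slider position, and refreshes the pawn's sound settings.
; stop_slider saves, detaches the mesh and closes the gate.
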(event Custom|update_element
  (bind _active (Variables|Default|Getactive))
  (Rendering|SetVisibility (Variables|Default|Getmesh) _active false)
  (Collision|SetCollisionEnabled (Variables|Default|Getmesh) (select _active "QueryAndPhysics" "NoCollision")))

(event Custom|stop_slider
  (bind _save_data (Variables|Default|Getsave_data))
  (Physics|SetSimulatePhysics (Variables|Default|Getmesh) false)
  (SaveGame|SaveGametoSlot (Variables|Default|Getsave_data) "Options")
  (Transformation|DetachFromComponent (Variables|Default|Getmesh) "KeepWorld" "KeepWorld" "KeepWorld" true)
  (Utilities|FlowControl|Gate true) ; enters at Close
)

(event EventBeginPlay)

(event Collision|EventActorBeginOverlap
  (params (OtherActor :type Actor%20Object%20Reference)))

(event EventTick
  (params (DeltaSeconds :type Float%20%28single-precision%29))
  (bind _save_data (Variables|Default|Getsave_data))
  (Utilities|FlowControl|Gate true
    (:Exit
      (switch Utilities|FlowControl|Switch|SwitchonOptions_sound (Variables|Default|Getmenu%20item%20type)
        (:NewEnumerator0
          (Variables|/Game/Assets/Blueprints/Settings_save_data.Settings_save_data_C|Setsettings_struct _save_data (Utilities|Struct|MakeSettings 1.0 (.music_volume (Variables|/Game/Assets/Blueprints/Settings_save_data.Settings_save_data_C|Getsettings_struct _save_data)) (.sfx_volume (Variables|/Game/Assets/Blueprints/Settings_save_data.Settings_save_data_C|Getsettings_struct _save_data)) (.video_quality (Variables|/Game/Assets/Blueprints/Settings_save_data.Settings_save_data_C|Getsettings_struct _save_data)) (.video_spectator_mode (Variables|/Game/Assets/Blueprints/Settings_save_data.Settings_save_data_C|Getsettings_struct _save_data)))))
        (:NewEnumerator1
          (Variables|/Game/Assets/Blueprints/Settings_save_data.Settings_save_data_C|Setsettings_struct _save_data (Utilities|Struct|MakeSettings (.master_volume (Variables|/Game/Assets/Blueprints/Settings_save_data.Settings_save_data_C|Getsettings_struct _save_data)) 1.0 (.sfx_volume (Variables|/Game/Assets/Blueprints/Settings_save_data.Settings_save_data_C|Getsettings_struct _save_data)) (.video_quality (Variables|/Game/Assets/Blueprints/Settings_save_data.Settings_save_data_C|Getsettings_struct _save_data)) (.video_spectator_mode (Variables|/Game/Assets/Blueprints/Settings_save_data.Settings_save_data_C|Getsettings_struct _save_data)))))
        (:NewEnumerator2
          (Variables|/Game/Assets/Blueprints/Settings_save_data.Settings_save_data_C|Setsettings_struct _save_data (Utilities|Struct|MakeSettings (.master_volume (Variables|/Game/Assets/Blueprints/Settings_save_data.Settings_save_data_C|Getsettings_struct _save_data)) (.music_volume (Variables|/Game/Assets/Blueprints/Settings_save_data.Settings_save_data_C|Getsettings_struct _save_data)) 1.0 (.video_quality (Variables|/Game/Assets/Blueprints/Settings_save_data.Settings_save_data_C|Getsettings_struct _save_data)) (.video_spectator_mode (Variables|/Game/Assets/Blueprints/Settings_save_data.Settings_save_data_C|Getsettings_struct _save_data))))))
      (Default|SoundSettingsUpdate (stale EventTakeDamage _aspersonal_mcpawn)))))

(event EventTakeDamage
  (params (DamageAmount :type Float%20%28single-precision%29) (Constant :type Boolean) (Effect :type Effects%20Enum :default "NewEnumerator4") (EffectTime :type Float%20%28single-precision%29) (Hit_Location :type Vector :default "0, 0, 0"))
  (Audio|PlaySound2D "/Engine/VREditor/Sounds/UI/Camera_Shutter.Camera_Shutter")
  (Physics|SetSimulatePhysics (Variables|Default|Getmesh) true)
  (bind _returnvalue (SaveGame|DoesSaveGameExist "Options"))
  (if _returnvalue
    (bind _returnvalue_2 (SaveGame|LoadGamefromSlot "Options"))
    (bind _assettings_save_data (Utilities|Casting|CastToSettings_save_data _returnvalue_2)
      (:then
        (Variables|Default|Setsave_data _assettings_save_data))
      (:CastFailed
        (bind _returnvalue_3 (SaveGame|CreateSaveGameObject "/Game/Assets/Blueprints/Settings_save_data.Settings_save_data_C" :!label _label))
        (Variables|Default|Setsave_data _returnvalue_3)))
    (else
      (goto _label)))
  (bind _aspersonal_mcpawn (Utilities|Casting|CastToPersonalMCPawn (Game|Player|GetPlayerPawn 0)))
  (Transformation|AttachComponentToComponent (Variables|Default|Getmesh) (Variables|/Game/VirtualRealityBP/Blueprints/BP_MotionController.BP_MotionController_C|GetHandMesh (Variables|/Game/Assets/Blueprints/PersonalMCPawn.PersonalMCPawn_C|GetController_R _aspersonal_mcpawn)) "None" "KeepWorld" "KeepWorld" "KeepWorld" true)
  (Utilities|FlowControl|Gate true) ; enters at Open
)

(fn ConstructionScript
  (bind _active (Variables|Default|Getactive))
  (Rendering|SetVisibility (Variables|Default|Getmesh) _active false)
  (Collision|SetCollisionEnabled (Variables|Default|Getmesh) (select _active "QueryAndPhysics" "NoCollision")))