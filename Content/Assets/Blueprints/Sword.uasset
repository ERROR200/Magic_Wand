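; Sword actor that can be picked up, dropped and swung to damage what it touches.
; Pickup disables physics and attaches the mesh to the supplied component, while Drop re-enables physics and detaches it.
; Each tick samples the mesh's physics velocity at VelocityPoint, allowing damage only above a speed threshold.
; While that flag is set, mesh overlaps send a fixed-damage message to the other actor.
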(event OnComponentBeginOverlap(StaticMesh)
  (params (OverlappedComponent :type Primitive%20Component%20Object%20Reference) (OtherActor :type Actor%20Object%20Reference) (OtherComp :type Primitive%20Component%20Object%20Reference) (OtherBodyIndex :type Integer) (bFromSweep :type Boolean) (SweepResult :type Hit%20Result%20Structure%20%28by%20ref%29))
  (if (Variables|Default|Getcan%20damage)
    (Class|IDamage|TakeDamage(Message) OtherActor 3.0 false "NewEnumerator4" 0.2 (Transformation|GetActorLocation OtherActor))))

(event EventBeginPlay)

(event Collision|EventActorBeginOverlap
  (params (OtherActor :type Actor%20Object%20Reference)))

(event EventPickup
  (params (AttachTo :type Scene%20Component%20Object%20Reference) (hand :type EControllerHand%20Enum :default "Left"))
  (Physics|SetSimulatePhysics (Variables|Default|GetStaticMesh) false)
  (Transformation|AttachComponentToComponent (Variables|Default|GetStaticMesh) AttachTo "None" "SnapToTarget" "KeepWorld" "KeepWorld" false))

(event EventTick
  (params (DeltaSeconds :type Float%20%28single-precision%29))
  (bind _returnvalue (Class|PrimitiveComponent|GetPhysicsLinearVelocityatPoint (Variables|Default|GetStaticMesh) (Transformation|GetWorldLocation (Variables|Default|Getvelocity%20point)) "None"))
  (Variables|Default|Setcan%20damage (> (Math|Vector|VectorLength _returnvalue) 3e+02)))

(event EventDrop
  (params (hand :type EControllerHand%20Enum :default "Left"))
  (Physics|SetSimulatePhysics (Variables|Default|GetStaticMesh) true)
  (Transformation|DetachFromComponent (Variables|Default|GetStaticMesh) "KeepRelative" "KeepRelative" "KeepRelative" true))

(fn ConstructionScript)