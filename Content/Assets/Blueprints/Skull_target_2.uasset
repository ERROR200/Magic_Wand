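; A skull target actor that pops in with a poof effect, lights up and can be shot or otherwise damaged to score.
; Activation opens a damage gate and drives a timeline that animates the emissive intensity of a dynamic material created in the construction script.
; Each accepted hit fires a radial force impulse at the hit location.
; Only the first reports to LevelManager's tally, cuts the glow, then poofs and destroys the actor.
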(event Custom|activate_skulls
  (bind _radialforce (Variables|Default|GetRadialForce))
  (Utilities|FlowControl|Sequence
    (:then_0
      (Variables|Default|SetcanBeHit true)
      (Utilities|FlowControl|Gate true) ; enters at Open
    )
    (:then_1
      (bind _newtrack_0 (Timeline|Timeline_0 PlayFromStart)
        (:Update
          (Rendering|Material|SetScalarParameterValue (Variables|Default|GetBodyMaterial) "Emissive Intensity" (* _newtrack_0 1e+02) :!class /Script/Engine.MaterialInstanceDynamic))))))

(event Collision|EventActorBeginOverlap
  (params (OtherActor :type Actor%20Object%20Reference)))

(event EventTick
  (params (DeltaSeconds :type Float%20%28single-precision%29)))

(event EventBeginPlay
  (bind _skull_mesh (Variables|Default|GetSkull_Mesh))
  (Rendering|SetVisibility _skull_mesh false false)
  (Effects|SpawnEmitteratLocation "/Game/Assets/Particles/Objects/apple_poof.apple_poof" (Transformation|GetWorldLocation _skull_mesh))
  (Utilities|FlowControl|Delay 0.2)
  (Rendering|SetVisibility _skull_mesh true false)
  (CallFunction|ActivateSkulls))

(event EventTakeDamage
  (params (DamageAmount :type Float%20%28single-precision%29) (Constant :type Boolean) (Effect :type Effects%20Enum :default "NewEnumerator4") (EffectTime :type Float%20%28single-precision%29) (Hit_Location :type Vector :default "0, 0, 0"))
  (bind _radialforce (Variables|Default|GetRadialForce))
  (Utilities|FlowControl|Gate true
    (:Exit
      (Transformation|SetWorldLocation _radialforce Hit_Location false false)
      (Class|RadialForceComponent|FireImpulse _radialforce)
      (Utilities|FlowControl|DoOnce false
        (:Completed
          (bind _outactors (Actor|GetAllActorsOfClass "/Game/Assets/Blueprints/LevelManager.LevelManager_C"))
          (Utilities|IsValid (Utilities|Array|Get(acopy) _outactors)
            (:Is%20Valid
              (Default|SkullTargetTally (Utilities|Array|Get(acopy) _outactors))
              (Timeline|Timeline_1 Play
                (:Update
                  (Rendering|Material|SetScalarParameterValue (Variables|Default|GetBodyMaterial) "Emissive Intensity" 0.0 :!class /Script/Engine.MaterialInstanceDynamic))
                (:Finished
                  (Effects|SpawnEmitteratLocation "/Game/Assets/Particles/Objects/apple_poof.apple_poof" (Transformation|GetWorldLocation (Variables|Default|GetSkull_Mesh)))
                  (Utilities|FlowControl|Delay 0.2)
                  (Actor|DestroyActor))))
            (:Is%20Not%20Valid
              (Timeline|Timeline_1 Play))))))))

(fn ConstructionScript
  (bind _skull_mesh (Variables|Default|GetSkull_Mesh))
  (bind _returnvalue (Rendering|Material|CreateDynamicMaterialInstance _skull_mesh 0 (Rendering|Material|GetMaterial _skull_mesh 0) :!class /Script/Engine.PrimitiveComponent))
  (Variables|Default|SetBodyMaterial _returnvalue))