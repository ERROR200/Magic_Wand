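; Menu option button actor that changes video quality or spectator mode when it takes damage, with a half-second DoOnce cooldown.
; It loads or creates the "Options" save, then sets QualitySetting or a FlipFlop-driven spectator flag according to MenuItemType.
; It saves the settings and calls VideoSettingsUpdate on the PersonalMCPawn player pawn to refresh them.
; The FlipFlop starts at enabled regardless of the saved spectator value.
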(event Collision|EventActorBeginOverlap
  (params (OtherActor :type Actor%20Object%20Reference)))

(event EventBeginPlay)

(event EventTick
  (params (DeltaSeconds :type Float%20%28single-precision%29)))

(event EventTakeDamage
  (params (DamageAmount :type Float%20%28single-precision%29) (Constant :type Boolean) (Effect :type Effects%20Enum :default "NewEnumerator4") (EffectTime :type Float%20%28single-precision%29) (Hit_Location :type Vector :default "0, 0, 0"))
  (Utilities|FlowControl|DoOnce false :!label _label
    (:Completed
      (Utilities|FlowControl|Sequence
        (:then_0
          (bind _returnvalue (SaveGame|DoesSaveGameExist "Options"))
          (if _returnvalue
            (bind _returnvalue_2 (SaveGame|LoadGamefromSlot "Options"))
            (bind _assettings_save_data (Utilities|Casting|CastToSettings_save_data _returnvalue_2)
              (:then
                (Variables|Default|Setsave_data _assettings_save_data))
              (:CastFailed
                (bind _returnvalue_3 (SaveGame|CreateSaveGameObject "/Game/Assets/Blueprints/Settings_save_data.Settings_save_data_C" :!label _label_2))
                (Variables|Default|Setsave_data _returnvalue_3)))
            (else
              (goto _label_2)))
          (switch Utilities|FlowControl|Switch|SwitchonOptions_Video (Variables|Default|Getmenu%20item%20type)
            (:NewEnumerator0
              (Variables|/Game/Assets/Blueprints/Settings_save_data.Settings_save_data_C|Setsettings_struct (Variables|Default|Getsave_data) (Utilities|Struct|MakeSettings (.master_volume (Variables|/Game/Assets/Blueprints/Settings_save_data.Settings_save_data_C|Getsettings_struct (Variables|Default|Getsave_data))) (.music_volume (Variables|/Game/Assets/Blueprints/Settings_save_data.Settings_save_data_C|Getsettings_struct (Variables|Default|Getsave_data))) (.sfx_volume (Variables|/Game/Assets/Blueprints/Settings_save_data.Settings_save_data_C|Getsettings_struct (Variables|Default|Getsave_data))) (Variables|Default|GetQuality_setting) (.video_spectator_mode (Variables|/Game/Assets/Blueprints/Settings_save_data.Settings_save_data_C|Getsettings_struct (Variables|Default|Getsave_data))))))
            (:NewEnumerator1
              (Utilities|FlowControl|FlipFlop
                (:A
                  (Variables|/Game/Assets/Blueprints/Settings_save_data.Settings_save_data_C|Setsettings_struct (Variables|Default|Getsave_data) (Utilities|Struct|MakeSettings (.master_volume (Variables|/Game/Assets/Blueprints/Settings_save_data.Settings_save_data_C|Getsettings_struct (Variables|Default|Getsave_data))) (.music_volume (Variables|/Game/Assets/Blueprints/Settings_save_data.Settings_save_data_C|Getsettings_struct (Variables|Default|Getsave_data))) (.sfx_volume (Variables|/Game/Assets/Blueprints/Settings_save_data.Settings_save_data_C|Getsettings_struct (Variables|Default|Getsave_data))) (.video_quality (Variables|/Game/Assets/Blueprints/Settings_save_data.Settings_save_data_C|Getsettings_struct (Variables|Default|Getsave_data))) true)))
                (:B
                  (Variables|/Game/Assets/Blueprints/Settings_save_data.Settings_save_data_C|Setsettings_struct (Variables|Default|Getsave_data) (Utilities|Struct|MakeSettings (.master_volume (Variables|/Game/Assets/Blueprints/Settings_save_data.Settings_save_data_C|Getsettings_struct (Variables|Default|Getsave_data))) (.music_volume (Variables|/Game/Assets/Blueprints/Settings_save_data.Settings_save_data_C|Getsettings_struct (Variables|Default|Getsave_data))) (.sfx_volume (Variables|/Game/Assets/Blueprints/Settings_save_data.Settings_save_data_C|Getsettings_struct (Variables|Default|Getsave_data))) (.video_quality (Variables|/Game/Assets/Blueprints/Settings_save_data.Settings_save_data_C|Getsettings_struct (Variables|Default|Getsave_data))) false))))))
          (SaveGame|SaveGametoSlot (Variables|Default|Getsave_data) "Options")
          (bind _aspersonal_mcpawn (Utilities|Casting|CastToPersonalMCPawn (Game|Player|GetPlayerPawn 0)))
          (Default|VideoSettingsUpdate _aspersonal_mcpawn))
        (:then_1
          (Utilities|FlowControl|Delay 0.5)
          (goto _label Reset))))))

(fn ConstructionScript)