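; Gargoyle enemy that, while active, periodically spawns Gargoyle_Fire projectiles from its fireball spawn point.
; Health scales from a hit count at BeginPlay, and Tick drives the charge countdown for firing.
; ResetState decrements the hit count and, after enough health loss, deactivates the gargoyle and its particles and resets the charge.
; It then reports a kill to the level manager's current spawner and plays a death particle.
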(event EventBeginPlay
  (bind _healthhits (Variables|Default|GetHealthHits))
  (bind _returnvalue (* _healthhits 1e+01))
  (|CallParentFunction)
  (Variables|Default|SetHealth _returnvalue)
  (Variables|Default|SetlastWholeHealthValue _returnvalue))

(event Collision|EventActorBeginOverlap
  (params (OtherActor :type Actor%20Object%20Reference))
  (|CallParentFunction OtherActor) ; This node is disabled and will not be called.\nDrag off pins to build functionality.
)

(event EventTick
  (params (DeltaSeconds :type Float%20%28single-precision%29))
  (if (Variables|Default|GetisActive)
    (CallFunction|Projectile)
    (|CallParentFunction DeltaSeconds)
    (if (Components|Activation|IsActive (Variables|Default|GetParticleSystem))
      (Components|Activation|Activate (Variables|Default|GetParticleSystem) true))))

(event EventResetState
  (bind _deathparticle (Variables|Default|GetdeathParticle))
  (bind _levelmanagerref (Variables|Default|GetLevelManagerRef))
  (bind _spawnerholder (Variables|/Game/Assets/Blueprints/LevelManager.LevelManager_C|GetSpawnerHolder _levelmanagerref))
  (bind _currentspawnemmiter (Variables|/Game/Assets/Blueprints/LevelManager.LevelManager_C|GetCurrentSpawnEmmiter _levelmanagerref))
  (bind _output (Utilities|Array|Get(acopy) _spawnerholder _currentspawnemmiter))
  (if (Variables|Default|GetisActive)
    (Math|Integer|DecrementInt (Variables|Default|GetHealthHits)
      (:%20%20
        (if (>= (- (Variables|Default|GetlastWholeHealthValue) (Variables|Default|GetHealth)) (Variables|Default|GetHealthLostToDeativate))
          (Variables|Default|SetlastWholeHealthValue (Variables|Default|GetHealth))
          (Variables|Default|SetisActive false)
          (Components|Activation|Deactivate (Variables|Default|GetParticleSystem))
          (Variables|Default|SetchargeCounter (Variables|Default|GetchargeTime))
          (Utilities|IsValid _output
            (:Is%20Valid
              (Default|EnemyKilled _output)
              (Utilities|IsValid _deathparticle
                (:Is%20Valid
                  (Effects|SpawnEmitteratLocation _deathparticle (Transformation|GetWorldLocation (Variables|Default|GetParticleSystem)))
                  (if (== (Variables|Default|GetHealthHits) 1)
                    (Variables|Default|SetHealth 1.0)))))))))))

(fn ConstructionScript
  (|CallParentFunction))

(fn Projectile
  (bind _output_get (Variables|Default|SetchargeCounter (- (Variables|Default|GetchargeCounter) (Utilities|Time|GetWorldDeltaSeconds))))
  (if (<= _output_get 0.0)
    (Game|SpawnActorfromClass "/Game/Assets/Blueprints/Spells/Gargoyle_Fire.Gargoyle_Fire_C" (Math|Transform|MakeTransform (Transformation|GetWorldLocation (Variables|Default|GetFireball_Spawn)) "0, 0, 0" "1,1,1") "AlwaysSpawn" 0 0)
    (Variables|Default|SetchargeCounter (Variables|Default|GetchargeTime))))