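; Spectator camera actor that renders a view of the game to a shared render target while active.
; Activate and deactivate events assign or clear the scene capture's texture target and toggle an active flag.
; While active in Follow mode, Tick rotates the actor to look at the player pawn's camera.
; The construction script tags the actor with "S" plus its level area, identifying it by area.
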(event Custom|activate
  (Variables|/Script/Engine.SceneCaptureComponent2D|SetTextureTarget (Variables|Default|GetSceneCaptureComponent2D) "/Game/Assets/Spectator_camera_render.Spectator_camera_render")
  (Variables|Default|Setis%20active true))

(event Custom|deactivate
  (Variables|/Script/Engine.SceneCaptureComponent2D|SetTextureTarget (Variables|Default|GetSceneCaptureComponent2D) 0)
  (Variables|Default|Setis%20active false))

(event EventBeginPlay)

(event Collision|EventActorBeginOverlap
  (params (OtherActor :type Actor%20Object%20Reference)))

(event EventTick
  (params (DeltaSeconds :type Float%20%28single-precision%29))
  (if (Variables|Default|Getis%20active)
    (switch Utilities|FlowControl|Switch|Switchonspec_camera_mode (Variables|Default|Getcamera_mode)
      (:NewEnumerator1
        (bind _aspersonal_mcpawn (Utilities|Casting|CastToPersonalMCPawn (Game|Player|GetPlayerPawn 0)))
        (Transformation|SetActorRotation (Math|Rotator|FindLookatRotation (Transformation|GetWorldLocation (Variables|Default|GetDefaultSceneRoot)) (Transformation|GetWorldLocation (Variables|/Game/Assets/Blueprints/PersonalMCPawn.PersonalMCPawn_C|GetCamera _aspersonal_mcpawn))))))))

(fn ConstructionScript
  (Variables|Default|SetTags (Utilities|Array|MakeArray (Utilities|String|StringToName (Utilities|String|Append "S" (Utilities|String|ToString(Integer) (Variables|Default|Getlevel_area)))))))