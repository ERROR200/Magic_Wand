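; Stone shield actor that sheds physics-simulated chunks as it takes damage and bursts apart when its health runs out.
; The construction script gathers static mesh children of Scene, and BeginPlay divides health by chunk count for a break threshold.
; TakeDamage accumulates damage, frees seeded-random chunks with radial impulses, and throttles damage flagged Constant with a short delay.
; At zero health, kill_shield simulates physics on all pieces once and fires the impulse.
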(event Custom|kill_shield
  (Utilities|FlowControl|DoOnce false
    (:Completed
      (for _array_element (Variables|Default|Getshield_break_list)
        (Utilities|IsValid _array_element
          (:Is%20Valid
            (Physics|SetSimulatePhysics _array_element true))))
      (Class|RadialForceComponent|FireImpulse (Variables|Default|GetRadialForce)))))

(event EventBeginPlay
  (Class|KismetMathLibrary|SeedRandomStream (Variables|Default|Getrandom))
  (Variables|Default|Setchunk_threashold (/ (Variables|Default|GetShieldHealth) (Math|Conversions|ToFloat(Integer) (Utilities|Array|Length (Variables|Default|Getshield%20chunk%20list))))))

(event Collision|EventActorBeginOverlap
  (params (OtherActor :type Actor%20Object%20Reference)))

(event EventTakeDamage
  (params (DamageAmount :type Float%20%28single-precision%29) (Constant :type Boolean) (Effect :type Effects%20Enum :default "NewEnumerator4") (EffectTime :type Float%20%28single-precision%29) (Hit_Location :type Vector :default "0, 0, 0"))
  (bind _shield_chunk_list (Variables|Default|Getshield%20chunk%20list))
  (bind _random (Variables|Default|Getrandom))
  (bind _returnvalue (Utilities|Array|LastIndex _shield_chunk_list))
  (bind _returnvalue_2 (Math|Random|RandomIntegerinRangefromStream 0 _returnvalue _random))
  (bind _output (Utilities|Array|Get(acopy) _shield_chunk_list _returnvalue_2))
  (if Constant
    (Utilities|FlowControl|DoOnce false :!label _label
      (:Completed
        (Utilities|FlowControl|Sequence
          (:then_0
            _)
          (:then_1
            (Utilities|FlowControl|Delay 0.3)
            (goto _label Reset))))))
  (Variables|Default|SetShieldHealth (- (Variables|Default|GetShieldHealth) DamageAmount))
  (Variables|Default|Setchunk_damage (+ (Variables|Default|Getchunk_damage) DamageAmount))
  (if (>= (Variables|Default|Getchunk_damage) (Variables|Default|Getchunk_threashold))
    (if (<= (Variables|Default|GetShieldHealth) 0.0)
      (Utilities|FlowControl|DoOnce false
        (:Completed
          (for _array_element (Variables|Default|Getshield_break_list)
            (Utilities|IsValid _array_element
              (:Is%20Valid
                (Physics|SetSimulatePhysics _array_element true))))
          (Class|RadialForceComponent|FireImpulse (Variables|Default|GetRadialForce))))
      (else
        (for _index (range 0 (Math|Float|Truncate (/ DamageAmount (Variables|Default|Getchunk_threashold))))
          (Variables|Default|Setchunk_damage 0.0)
          (if (== (Utilities|Array|Length _shield_chunk_list) 0)
            (CallFunction|KillShield)
            (else
              (Utilities|IsValid _output
                (:Is%20Valid
                  (Physics|SetSimulatePhysics _output true)
                  (Class|RadialForceComponent|FireImpulse (Variables|Default|GetRadialForce))
                  (Physics|SetSimulatePhysics _output true)
                  (if (Physics|IsSimulatingPhysics _output "None")
                    (Utilities|Array|RemoveItem _shield_chunk_list _output)))))))))))

(fn ConstructionScript
  (for _array_element (Components|GetChildrenComponents (Variables|Default|GetScene) false)
    (bind _asstatic_mesh_component (Utilities|Casting|CastToStaticMeshComponent _array_element))
    (Utilities|Array|Add (Variables|Default|Getshield%20chunk%20list) _asstatic_mesh_component))
  (Variables|Default|Setshield_break_list (Variables|Default|Getshield%20chunk%20list)))