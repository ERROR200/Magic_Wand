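; Fast skeleton enemy that charges and leaps at the player, and explodes as its attack.
; With line of sight and a required effect state, a timeline ramps it to sprint speed, then after a random delay it launches once within a jump distance band.
; Losing sight triggers a player search, while another effect state cancels the charge.
; Tick runs pathfinding and feeds state to the animation Blueprint.
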(event Custom|ChargeJump
  (bind _returnvalue (Game|Player|GetPlayerPawn 0))
  (bind _self self)
  (bind _returnvalue_2 (Transformation|GetHorizontalDistanceTo _returnvalue _self))
  (if (and (<= _returnvalue_2 (Variables|Default|GetmaxJumpDist)) (>= _returnvalue_2 (Variables|Default|GetminJumpDist)))
    (Variables|Default|SetJumped true)
    (Utilities|FlowControl|Delay 0.2)
    (CallFunction|Launch)))

(event EventBeginPlay
  (|CallParentFunction)
  (bind _asfast_skeleton_anim_bp (Utilities|Casting|CastToFastSkeleton_AnimBP (Components|SkeletalMesh|GetAnimInstance (Variables|Character|GetMesh))))
  (Variables|Default|SetAnimRef _asfast_skeleton_anim_bp))

(event Collision|EventActorBeginOverlap
  (params (OtherActor :type Actor%20Object%20Reference))
  (|CallParentFunction OtherActor) ; This node is disabled and will not be called.\nDrag off pins to build functionality.
)

(event EventAttack
  (CallFunction|Explode))

(event EventTick
  (params (DeltaSeconds :type Float%20%28single-precision%29))
  (|CallParentFunction DeltaSeconds)
  (CallFunction|PathFinding)
  (Default|UpdateInfo (Variables|Default|GetAnimRef) (Variables|Default|GetEnemyState) (Variables|Default|GetLeftArmAttack)))

(event EventSpecialAbility
  (if (Variables|Default|GetHasDirectLineOfSight)
    (if (Utilities|Enum|Equal(Enum) (Variables|Default|GetCurrentEffect) "NewEnumerator4")
      (if (Variables|Default|GetCharge)
        (if (not (Variables|Default|GetJumped))
          (CallFunction|ChargeJump))
        (else
          (Utilities|FlowControl|DoOnce false :!label _label
            (:Completed
              (bind _timer (Timeline|Speedup PlayFromStart)
                (:Update
                  (Variables|Default|SetForwardSpeed (Math|Float|Lerp (Variables|Default|GetDefaultSpeed) (Variables|Default|GetSprintSpeed) _timer)))
                (:Finished
                  (Utilities|FlowControl|Delay (Math|Random|RandomFloatinRange 0.5 1.0))
                  (if (not (Variables|Default|Getdead))
                    (Variables|Default|SetCharge true)
                    (CallFunction|ChargeJump))))))))
      (else
        (Variables|Default|SetCharge false)
        (Utilities|FlowControl|Sequence
          (:then_0
            (goto _label Reset))
          (:then_1
            (Timeline|Speedup Stop)))))
    (else
      (CallFunction|SearchforPlayer))))

(fn ConstructionScript
  (|CallParentFunction))