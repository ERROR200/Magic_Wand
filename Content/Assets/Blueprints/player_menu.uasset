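; In-world player pause menu actor with two selectable objects, a StaticMesh and a Sphere.
; Opening pauses the game and plays a pause-tickable timeline that lerps both from start transforms set by initialise to their construction-time placements; closing unpauses and reverses it.
; Pickup opens the menu when closed; when open, overlap with the grabbing actor selects an option.
; The Sphere calls DeathOverride on PersonalMCPawn and closes the menu, while the StaticMesh just closes it.
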(event Custom|initialise
  (params (start_Pos :type Transform) (Sart_pos_2 :type Transform))
  (Variables|Default|Setstart_transform start_Pos)
  (Variables|Default|Setstart_transform_2 Sart_pos_2))

(event Custom|openmenu
  (params (Forward/Backward :type Boolean))
  (if Forward/Backward
    (Variables|Default|Setis%20open true)
    (Game|SetGamePaused true)
    (bind _alpha (Timeline|open Play)
      (:Update
        (Transformation|SetRelativeTransform (Variables|Default|GetStaticMesh) (Math|Transform|Lerp(Transform) (Variables|Default|Getstart_transform) (Variables|Default|GetTarget_transform) _alpha) false false)
        (Transformation|SetRelativeTransform (Variables|Default|GetSphere) (Math|Transform|Lerp(Transform) (Variables|Default|Getstart_transform_2) (Variables|Default|GetTarget_transform_2) _alpha) false false)))
    (else
      (Variables|Default|Setis%20open false)
      (Game|SetGamePaused false)
      (Timeline|open Reverse))))

(event Custom|toggle_menu
  (if (Variables|Default|Getis%20open)
    (Variables|Default|Setis%20open false)
    (Game|SetGamePaused false)
    (bind _alpha (Timeline|open Reverse)
      (:Update
        (Transformation|SetRelativeTransform (Variables|Default|GetStaticMesh) (Math|Transform|Lerp(Transform) (Variables|Default|Getstart_transform) (Variables|Default|GetTarget_transform) _alpha) false false)
        (Transformation|SetRelativeTransform (Variables|Default|GetSphere) (Math|Transform|Lerp(Transform) (Variables|Default|Getstart_transform_2) (Variables|Default|GetTarget_transform_2) _alpha) false false)))
    (else
      (Variables|Default|Setis%20open true)
      (Game|SetGamePaused true)
      (Timeline|open Play))))

(event EventBeginPlay
  (Class|ActorComponent|SetTickablewhenPaused (Variables|Default|Getopen) true)
  (Class|Actor|GetTickablewhenPaused))

(event Collision|EventActorBeginOverlap
  (params (OtherActor :type Actor%20Object%20Reference)))

(event EventPickup
  (params (AttachTo :type Scene%20Component%20Object%20Reference) (hand :type EControllerHand%20Enum :default "Left"))
  (bind _returnvalue (Components|GetOwner AttachTo))
  (if (Variables|Default|Getis%20open)
    (if (Collision|IsOverlappingActor (Variables|Default|GetSphere) _returnvalue :!class /Script/Engine.PrimitiveComponent)
      (bind _aspersonal_mcpawn (Utilities|Casting|CastToPersonalMCPawn (Game|Player|GetPlayerPawn 0)))
      (Default|DeathOverride _aspersonal_mcpawn)
      (CallFunction|Openmenu false :!label _label)
      (elif (Collision|IsOverlappingActor (Variables|Default|GetStaticMesh) _returnvalue :!class /Script/Engine.PrimitiveComponent)
        (goto _label)))
    (else
      (CallFunction|Openmenu true))))

(fn ConstructionScript
  (Variables|Default|SetTarget_transform (Transformation|GetRelativeTransform (Variables|Default|GetStaticMesh)))
  (Variables|Default|SetTarget_transform_2 (Transformation|GetRelativeTransform (Variables|Default|GetSphere))))