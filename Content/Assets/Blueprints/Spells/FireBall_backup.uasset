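; Fireball spell actor that wanders around its cast location and damages what it overlaps, with checks for inactive Gargoyles and unhittable skull targets.
; Once started, Tick lerps it toward a random stream-based offset, picking another on arrival.
; Each delay-throttled hit spawns effects, then HitScale slows and enlarges it, sets damage to one and decrements HitCount.
; When hits run low, Kill stops sound, particles and movement, then destroys it.
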(event OnComponentBeginOverlap(Sphere)
  (params (OverlappedComponent :type Primitive%20Component%20Object%20Reference) (OtherActor :type Actor%20Object%20Reference) (OtherComp :type Primitive%20Component%20Object%20Reference) (OtherBodyIndex :type Integer) (bFromSweep :type Boolean) (SweepResult :type Hit%20Result%20Structure%20%28by%20ref%29))
  (bind _returnvalue (Transformation|GetActorLocation))
  (bind _returnvalue_2 (Transformation|GetActorLocation))
  (bind _asgargoyle (Utilities|Casting|CastToGargoyle OtherActor)
    (:then
      (if (Variables|/Game/Assets/Blueprints/Gargoyle.Gargoyle_C|GetisActive _asgargoyle)
        (bind _asskull_target_2 (Utilities|Casting|CastToSkull_target_2 OtherActor :!label _label)
          (:then
            (if (Variables|/Game/Assets/Blueprints/Skull_target_2.Skull_target_2_C|GetcanBeHit _asskull_target_2)
              (if (Utilities|Enum|Equal(Enum) (Collision|GetCollisionObjectType OtherComp) "ECC_GameTraceChannel1") :!label _label_2
                (bind _aspersonal_mcpawn (Utilities|Casting|CastToPersonalMCPawn (Game|Player|GetPlayerPawn 0)))
                (if (> (Variables|Default|GetDamageAmount) 0.0)
                  (Utilities|FlowControl|Sequence
                    (:then_0
                      (Utilities|FlowControl|DoOnce false :!label _label_3
                        (:Completed
                          (Effects|SpawnEmitteratLocation "/Game/Assets/Particles/Fire/fire_damage.fire_damage" _returnvalue_2 (Math|Rotator|FindLookatRotation _returnvalue_2 (Transformation|GetWorldLocation (Variables|/Game/Assets/Blueprints/PersonalMCPawn.PersonalMCPawn_C|GetCamera _aspersonal_mcpawn))) "2.000000,2.000000,2.000000")
                          (Class|IDamage|TakeDamage(Message) OtherActor (Variables|Default|GetDamageAmount) false "NewEnumerator2" 1.0 _returnvalue)
                          (Audio|PlaySoundatLocation "/Game/Assets/Sounds/fire/fire_hit.fire_hit" _returnvalue)
                          (CallFunction|HitScale))))
                    (:then_1
                      (Utilities|FlowControl|Delay (Variables|Default|GetDelayBetweenHits))
                      (goto _label_3 Reset)))))))
          (:CastFailed
            (goto _label_2)))))
    (:CastFailed
      (goto _label))))

(event Custom|kill
  (bind _returnvalue (Transformation|GetActorLocation))
  (bind _cast_location (Variables|Default|GetCast_location))
  (bind _location_mod (Variables|Default|Getlocation_mod))
  (bind _returnvalue_2 (+ _cast_location _location_mod))
  (Utilities|Time|ClearandInvalidateTimerbyHandle (stale Custom|start _returnvalue_3))
  (Utilities|IsValid (stale Custom|flame_sound_loop _returnvalue)
    (:Is%20Valid
      (Audio|Components|Audio|Stop (stale Custom|flame_sound_loop _returnvalue)))
    (:Is%20Not%20Valid
      _))
  (Variables|Default|SetDamageAmount 0.0)
  (Components|Activation|Deactivate (Variables|Default|GetParticleSystem))
  (Utilities|FlowControl|Sequence
    (:then_0
      (Utilities|FlowControl|Gate false) ; enters at Close
    )
    (:then_1
      (Utilities|FlowControl|Delay 2.0)
      (Actor|DestroyActor))))

(event Custom|fireball%20location%20mod
  (bind _random (Variables|Default|Getrandom))
  (bind _random_bounds (Variables|Default|Getrandom_bounds))
  (bind _returnvalue (* _random_bounds -1.0))
  (Variables|Default|Setlocation_mod (Math|Vector|MakeVector (Math|Random|RandomFloatinRangefromStream _returnvalue _random_bounds _random) (Math|Random|RandomFloatinRangefromStream _returnvalue _random_bounds _random) (Math|Random|RandomFloatinRangefromStream _returnvalue _random_bounds _random))))

(event Custom|flame_sound_loop
  (bind _returnvalue (Audio|SpawnSoundAttached "/Game/Assets/Sounds/fire/fire_burn_loop_Cue.fire_burn_loop_Cue" (Variables|Default|GetSphere))))

(event Custom|up%20fireball%20bounds
  (bind _outactors (Actor|GetAllActorsOfClass "/Game/Assets/Blueprints/Spells/FireBall.FireBall_C"))
  (for _array_element _outactors
    (Utilities|IsValid _array_element
      (:Is%20Valid
        (Variables|/Game/Assets/Blueprints/Spells/FireBall.FireBall_C|Setrandom_bounds _array_element (* (Variables|/Game/Assets/Blueprints/Spells/FireBall.FireBall_C|Getrandom_bounds _array_element) 2.0))))))

(event Custom|start
  (bind _returnvalue (Transformation|GetActorLocation))
  (bind _cast_location (Variables|Default|GetCast_location))
  (bind _location_mod (Variables|Default|Getlocation_mod))
  (bind _returnvalue_2 (+ _cast_location _location_mod))
  (CallFunction|FireballLocationMod)
  (Audio|Components|Audio|Play (Variables|Default|GetFire_burn_start_cue) 0.0)
  (Utilities|FlowControl|Sequence
    (:then_0
      (Utilities|FlowControl|Gate true) ; enters at Open
    )
    (:then_1
      (Utilities|FlowControl|Delay 0.5)
      (CallFunction|FlameSoundLoop)
      (bind _returnvalue_3 (Utilities|Time|SetTimerbyEvent (delegate Custom|flame_sound_loop) 2.5 true)))))

(event EventTick
  (params (DeltaSeconds :type Float%20%28single-precision%29))
  (bind _returnvalue (Transformation|GetActorLocation))
  (bind _cast_location (Variables|Default|GetCast_location))
  (bind _location_mod (Variables|Default|Getlocation_mod))
  (bind _returnvalue_2 (+ _cast_location _location_mod))
  (Utilities|FlowControl|Gate true
    (:Exit
      (if (<= (Variables|Default|GetHitCount) 1)
        (Utilities|FlowControl|DoOnce false
          (:Completed
            (CallFunction|Kill)))
        (else
          (Utilities|FlowControl|Gate false
            (:Exit
              (Transformation|SetActorLocation (Math|Vector|Lerp(Vector) _returnvalue _returnvalue_2 (Variables|Default|GetFireball_speed)) false true)
              (if (Math|Vector|Equal(Vector) _returnvalue _returnvalue_2 3e+01)
                (Development|PrintString "change")
                (CallFunction|FireballLocationMod)))))))))

(fn ConstructionScript)

(fn HitScale
  (bind _particlesystem (Variables|Default|GetParticleSystem))
  (Variables|Default|SetFireball_speed (/ (Variables|Default|GetFireball_speed) 1.5))
  (Math|Integer|DecrementInt (Variables|Default|GetHitCount)
    (:%20%20
      (Transformation|SetActorScale3D (* (Transformation|GetActorScale3D) 1.2))
      (Variables|Default|SetDamageAmount 1.0)
      (Transformation|SetRelativeScale3D _particlesystem (+ (Variables|/Script/Engine.SceneComponent|GetRelativeScale3D _particlesystem) "0.400000,0.400000,0.400000")))))