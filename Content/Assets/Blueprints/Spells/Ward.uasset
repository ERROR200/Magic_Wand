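; Ward spell actor that, as wired, only destroys itself on KillSpell and sets its instanced mesh's random seed in the construction script.
; Disconnected, never-run graph logic would scale a plane by the VR pawn's remaining right-hand ward charge and hold the ward beyond the casting hand, facing the camera.
; That unused logic also removes the ward's box, held and mesh components once the charge drops below zero.
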(event EventBeginPlay)

(event Collision|EventActorBeginOverlap
  (params (OtherActor :type Actor%20Object%20Reference)))

(event EventKillSpell
  (params (input_actor :type Actor%20Object%20Reference))
  (Actor|DestroyActor))

(event EventTick
  (params (DeltaSeconds :type Float%20%28single-precision%29)))

(fn ConstructionScript
  (bind _random (Variables|Default|Getrandom))
  (Class|KismetMathLibrary|SeedRandomStream _random)
  (Variables|/Script/Engine.InstancedStaticMeshComponent|SetInstancingRandomSeed (Variables|Default|GetInstancedStaticMesh) (Class|KismetMathLibrary|RandomIntegerfromStream 0 _random)))