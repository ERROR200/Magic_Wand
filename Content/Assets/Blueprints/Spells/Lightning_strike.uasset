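; Lightning strike spell actor that deals one burst of area damage shortly after spawning, then destroys itself.
; BeginPlay plays the strike sound, flashes the lights and, after a brief delay, damages actors overlapping the capsule.
; Damage falls off in three horizontal-distance bands and is sent via TakeDamageMessage with a timed effect.
; A looping timer randomly moves, rotates and scales the decal from a seeded stream until it is hidden.
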(event Custom|decal_change
  (bind _random (Variables|Default|Getrandom))
  (bind _random_value (Variables|Default|GetRandom_value))
  (bind _returnvalue (* _random_value -1.0))
  (Transformation|SetWorldTransform (Variables|Default|GetDecal) (Math|Transform|MakeTransform (+ (Transformation|GetActorLocation) (Math|Vector|MakeVector (Math|Random|RandomFloatinRangefromStream _returnvalue _random_value _random) (Math|Random|RandomFloatinRangefromStream _returnvalue _random_value _random) (Math|Random|RandomFloatinRangefromStream _returnvalue _random_value _random))) (Math|Rotator|MakeRotator 0.0 9e+01 (Math|Random|RandomFloatinRangefromStream -1.8e+02 1.8e+02 _random)) (+ "0, 0, 0" (Math|Random|RandomFloatinRangefromStream 0.2 0.75 _random))) false false))

(event EventBeginPlay
  (bind _defaultsceneroot (Variables|Default|GetDefaultSceneRoot))
  (bind _returnvalue (Transformation|GetWorldLocation _defaultsceneroot))
  (bind _returnvalue_2 (Utilities|Time|SetTimerbyEvent (delegate Custom|decal_change) 0.1 true))
  (Class|KismetMathLibrary|SeedRandomStream (Variables|Default|Getrandom))
  (Audio|SpawnSoundatLocation "/Game/Assets/Sounds/Lightning_strike1_sound_Cue.Lightning_strike1_sound_Cue" (Transformation|GetActorLocation))
  (Rendering|Components|Light|SetIntensity (Variables|Default|GetPointLight) 1e+01)
  (Utilities|FlowControl|Delay 0.2)
  (for _array_element (Collision|GetOverlappingActors (Variables|Default|GetCapsule) 0 :!class /Script/Engine.PrimitiveComponent)
    (if (<= (Math|Float|Absolute(Float) (Math|Vector|VectorLength (- (Math|Vector|MakeVector (.x (Transformation|GetActorLocation _array_element)) (.y (Transformation|GetActorLocation _array_element)) (.z _returnvalue)) (Math|Vector|MakeVector (.x _returnvalue) (.y _returnvalue) (.z _returnvalue))))) 75.0)
      (Variables|Default|SetDamageAmount 3.0)
      (Class|IDamage|TakeDamage(Message) _array_element (Variables|Default|GetDamageAmount) false "NewEnumerator3" 2.0 (Transformation|GetActorLocation) :!label _label)
      (elif (<= (Math|Float|Absolute(Float) (Math|Vector|VectorLength (- (Math|Vector|MakeVector (.x (Transformation|GetActorLocation _array_element)) (.y (Transformation|GetActorLocation _array_element)) (.z _returnvalue)) (Math|Vector|MakeVector (.x _returnvalue) (.y _returnvalue) (.z _returnvalue))))) 2e+02)
        (Variables|Default|SetDamageAmount 1.5)
        (goto _label)
        (elif (<= (Math|Float|Absolute(Float) (Math|Vector|VectorLength (- (Math|Vector|MakeVector (.x (Transformation|GetActorLocation _array_element)) (.y (Transformation|GetActorLocation _array_element)) (.z _returnvalue)) (Math|Vector|MakeVector (.x _returnvalue) (.y _returnvalue) (.z _returnvalue))))) 5e+02)
          (Variables|Default|SetDamageAmount 0.5)
          (goto _label)))))
  (Rendering|Components|Light|SetIntensity (Variables|Default|GetPointLight) 0.0)
  (Utilities|FlowControl|Delay 0.9)
  (Rendering|SetVisibility (Variables|Default|GetDecal) false false)
  (Utilities|Time|ClearandInvalidateTimerbyHandle _returnvalue_2)
  (Utilities|FlowControl|Delay 3.0)
  (Actor|DestroyActor))

(fn ConstructionScript)