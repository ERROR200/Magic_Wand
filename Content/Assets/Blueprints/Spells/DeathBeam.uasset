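; DeathBeam is a short-lived beam spell actor that destroys itself on spawn if another instance already exists.
; BeginPlay plays the laser sound, activates the fire effect and opens a gate that Tick feeds.
; Each frame it traces between two arrows, ignoring the player and first wand, spawning a hit emitter and sending constant damage to the hit actor.
; DamageTime counts down during firing, then the beam effects deactivate and the actor is destroyed.
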(event EventBeginPlay
  (bind _outactors (Actor|GetAllActorsOfClass "DeathBeam_C"))
  (if (> (Utilities|Array|Length _outactors) 1)
    (Actor|DestroyActor)
    (else
      (Audio|PlaySound2D "/Game/Assets/Sounds/New_beam/lazer_cue.lazer_cue")
      (bind _outactors_2 (Actor|GetAllActorsOfClass "/Game/Assets/Blueprints/Wand.Wand_C"))
      (Components|Activation|Activate (Variables|Default|GetBeam_Fire) false)
      (Utilities|FlowControl|Gate true) ; enters at Open
    )))

(event EventTick
  (params (DeltaSeconds :type Float%20%28single-precision%29))
  (Utilities|FlowControl|Gate true
    (:Exit
      (bind _outhit (Collision|LineTraceForObjects (Transformation|GetWorldLocation (Variables|Default|GetArrow)) (Transformation|GetWorldLocation (Variables|Default|GetArrow1)) (Utilities|Array|MakeArray "ObjectTypeQuery1" "ObjectTypeQuery2" "ObjectTypeQuery7" "ObjectTypeQuery4" "ObjectTypeQuery11") false (Utilities|Array|MakeArray (Game|Player|GetPlayerPawn 0) (Utilities|Array|Get(acopy) (stale EventBeginPlay _outactors_2))) "None"))
      (Effects|SpawnEmitteratLocation "/Game/Assets/Particles/Beam/Beam_hit.Beam_hit" (.location _outhit))
      (Class|IDamage|TakeDamage(Message) (.hitactor _outhit) 6.0 true "NewEnumerator0" 0.1 (.location _outhit))
      (bind _output_get (Variables|Default|SetDamageTime (- (Variables|Default|GetDamageTime) (Utilities|Time|GetWorldDeltaSeconds))))
      (if (< _output_get 0.0)
        (Components|Activation|Deactivate (Variables|Default|GetBeam_charge))
        (Actor|DestroyActor)))))

(event EventKillSpell
  (params (input_actor :type Actor%20Object%20Reference)))

(fn ConstructionScript)