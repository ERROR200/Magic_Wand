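; Lightning spell actor that aims at world geometry and calls down a lightning strike on the targeted point.
; Each tick it line-traces between its two arrow components against WorldStatic, moving a particle marker to the hit or hiding it and zeroing the cast location.
; ActivateSpell spawns Lightning_strike there unless the location is zero; KillSpell stops the charge effect and destroys the actor.
; Camera-driven arrow rotation is disconnected, and the BeginPlay Wand lookup is unused.
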(event EventBeginPlay
  (bind _outactors (Actor|GetAllActorsOfClass "/Game/Assets/Blueprints/Wand.Wand_C"))
  (Utilities|FlowControl|Delay 1.0))

(event EventTick
  (params (DeltaSeconds :type Float%20%28single-precision%29))
  (bind _particlesystem (Variables|Default|GetParticleSystem))
  (bind _particlesystem_2 (Variables|Default|GetParticleSystem))
  (bind _aspersonal_mcpawn (Utilities|Casting|CastToPersonalMCPawn (Game|Player|GetPlayerPawn 0)))
  (bind (_outhit _returnvalue) (Collision|LineTraceForObjects (Transformation|GetWorldLocation (Variables|Default|GetArrow)) (Transformation|GetWorldLocation (Variables|Default|GetArrow1)) (Utilities|Array|MakeArray "ObjectTypeQuery1") false 0 "None"))
  (if _returnvalue
    (Components|Activation|SetActive _particlesystem_2 true false)
    (bind _output_get (Variables|Default|Setcast_location (.location _outhit)))
    (Transformation|SetWorldLocation _particlesystem _output_get false false)
    (Transformation|SetWorldRotation _particlesystem "-90.000000, 0,0.000000" false false)
    (else
      (Components|Activation|SetActive _particlesystem_2 false false)
      (Variables|Default|Setcast_location "0, 0, 0"))))

(event EventActivateSpell
  (params (input_actor :type Actor%20Object%20Reference))
  (bind _cast_location (Variables|Default|Getcast_location))
  (if (not (Math|Vector|Equal(Vector) _cast_location "0, 0, 0" 1.0))
    (Game|SpawnActorfromClass "/Game/Assets/Blueprints/Spells/Lightning_strike.Lightning_strike_C" (Math|Transform|MakeTransform _cast_location "0, 0, 0" "1,1,1") "AlwaysSpawn" 0 0)))

(event EventKillSpell
  (params (input_actor :type Actor%20Object%20Reference))
  (Components|Activation|Deactivate (Variables|Default|GetLightning_charge))
  (Actor|DestroyActor))

(fn ConstructionScript)