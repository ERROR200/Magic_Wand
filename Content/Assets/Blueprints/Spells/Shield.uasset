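; VR shield spell actor that attaches to a motion controller and breaks loose when damaged.
; A timeline fades its emissive material on spawn and plays backwards on removal before destroying it.
; Hits while held give haptics and sound, then drop it with doubled velocity, after a decal crack animation for one effect type.
; Its mesh hits send damage to the other actor, then remove the shield after a delay.
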(event OnComponentHit(StaticMesh)
  (params (HitComponent :type Primitive%20Component%20Object%20Reference) (OtherActor :type Actor%20Object%20Reference) (OtherComp :type Primitive%20Component%20Object%20Reference) (NormalImpulse :type Vector :default "0, 0, 0") (Hit :type Hit%20Result%20Structure%20%28by%20ref%29))
  (Class|IDamage|TakeDamage(Message) OtherActor 0.5 false "NewEnumerator4" 0.2 (.location Hit))
  (Utilities|FlowControl|Delay 1.0)
  (CallFunction|Remove))

(event Custom|remove
  (Audio|PlaySoundatLocation "/Game/Assets/Sounds/OtherSounds/shield_manifold_remove_cue.shield_manifold_remove_cue" (Transformation|GetWorldLocation (Variables|Default|GetStaticMesh)))
  (Components|Activation|Activate (Variables|Default|GetParticleSystem) true)
  (bind (_direction _colour_lerp) (Timeline|Timeline_0 Reverse)
    (:Update
      (Rendering|Material|SetVectorParameterValue (Variables|Default|Getdynamat) "Emmisive overide" (Math|Color|Lerp(LinearColor) :A "(R=5.254912,G=0.000000,B=10.000000,A=1.000000)" :Alpha _colour_lerp) :!class /Script/Engine.MaterialInstanceDynamic))
    (:Finished
      (switch Utilities|FlowControl|Switch|SwitchonETimelineDirection _direction
        (:Forward
          (Components|Activation|Activate (Variables|Default|GetParticleSystem) true))
        (:Backward
          (Actor|DestroyActor))))))

(event EventBeginPlay
  (Transformation|SetRelativeRotation (Variables|Default|GetDecal) (Math|Rotator|MakeRotator (Math|Random|RandomFloatinRange 0.0 3.6e+02) 0.0 0.0) false false)
  (Rendering|Material|SetVectorParameterValue (Variables|Default|Getcrack_dynamat) "colour" "(R=2.000000,G=10.000000,B=0.000000,A=0.000000)" :!class /Script/Engine.MaterialInstanceDynamic)
  (bind (_direction _colour_lerp) (Timeline|Timeline_0 Play)
    (:Update
      (Rendering|Material|SetVectorParameterValue (Variables|Default|Getdynamat) "Emmisive overide" (Math|Color|Lerp(LinearColor) :A "(R=5.254912,G=0.000000,B=10.000000,A=1.000000)" :Alpha _colour_lerp) :!class /Script/Engine.MaterialInstanceDynamic))
    (:Finished
      (switch Utilities|FlowControl|Switch|SwitchonETimelineDirection _direction
        (:Forward
          (Components|Activation|Activate (Variables|Default|GetParticleSystem) true))
        (:Backward
          (Actor|DestroyActor))))))

(event EventTakeDamage
  (params (DamageAmount :type Float%20%28single-precision%29) (Constant :type Boolean) (Effect :type Effects%20Enum :default "NewEnumerator4") (EffectTime :type Float%20%28single-precision%29) (Hit_Location :type Vector :default "0, 0, 0"))
  (bind _returnvalue (Game|GetPlayerController 0))
  (bind _staticmesh (Variables|Default|GetStaticMesh))
  (bind _staticmesh_2 (Variables|Default|GetStaticMesh))
  (bind _returnvalue_2 (Transformation|GetWorldLocation _staticmesh_2))
  (Utilities|IsValid (Actor|GetAttachParentActor)
    (:Is%20Valid
      (Class|PlayerController|PlayHapticEffect _returnvalue "/Game/VirtualRealityBP/Blueprints/MotionControllerHaptic_shock.MotionControllerHaptic_shock" (stale EventPickup hand) 1.0 false)
      (Audio|PlaySoundatLocation "/Game/Assets/Sounds/OtherSounds/shield_hit_cue1.shield_hit_cue1" _returnvalue_2 "0, 0, 0" 1.0 1.0 0.5)
      (if (Utilities|Enum|Equal(Enum) Effect "NewEnumerator2")
        (bind _newtrack_0 (Timeline|crack Play)
          (:Update
            (Rendering|Material|SetVectorParameterValue (Variables|Default|Getcrack_dynamat) "colour" (Utilities|Struct|MakeLinearColor 2.0 1e+01 0.0 _newtrack_0) :!class /Script/Engine.MaterialInstanceDynamic))
          (:Finished
            (Audio|PlaySoundatLocation "/Game/Assets/Sounds/OtherSounds/shield_hit_cue1.shield_hit_cue1" _returnvalue_2 "0, 0, 0" 1.0 2.0 0.5)
            (Class|PlayerController|PlayHapticEffect _returnvalue "/Game/VirtualRealityBP/Blueprints/MotionControllerHaptic_shock.MotionControllerHaptic_shock" (stale EventPickup hand) 1.0 false)
            (Utilities|FlowControl|DoOnce false :!label _label
              (:Completed
                (Physics|SetSimulatePhysics (Variables|Default|GetStaticMesh) true)
                (Collision|SetCollisionObjectType (Variables|Default|GetStaticMesh) "ECC_GameTraceChannel2")
                (Transformation|DetachFromActor "KeepWorld" "KeepWorld" "KeepWorld")
                (Variables|Default|SetTags (Utilities|Array|MakeArray "OLDSHIELD"))
                (bind _returnvalue_3 (Physics|GetPhysicsLinearVelocity _staticmesh "None"))
                (Physics|SetPhysicsLinearVelocity _staticmesh (* _returnvalue_3 2.0) false "None")))))
        (else
          (goto _label))))))

(event EventPickup
  (params (AttachTo :type Scene%20Component%20Object%20Reference) (hand :type EControllerHand%20Enum :default "Left"))
  (Utilities|FlowControl|DoOnce false
    (:Completed
      (Physics|SetSimulatePhysics (Variables|Default|GetStaticMesh) false)
      (Transformation|AttachComponentToComponent (VehicleSound|GetRootComponent) AttachTo "None" "SnapToTarget" "SnapToTarget" "KeepWorld" false))))

(event EventDrop
  (params (hand :type EControllerHand%20Enum :default "Left"))
  (bind _staticmesh (Variables|Default|GetStaticMesh))
  (Utilities|FlowControl|DoOnce false
    (:Completed
      (Physics|SetSimulatePhysics (Variables|Default|GetStaticMesh) true)
      (Collision|SetCollisionObjectType (Variables|Default|GetStaticMesh) "ECC_GameTraceChannel2")
      (Transformation|DetachFromActor "KeepWorld" "KeepWorld" "KeepWorld")
      (Variables|Default|SetTags (Utilities|Array|MakeArray "OLDSHIELD"))
      (bind _returnvalue (Physics|GetPhysicsLinearVelocity _staticmesh "None"))
      (Physics|SetPhysicsLinearVelocity _staticmesh (* _returnvalue 2.0) false "None"))))

(fn ConstructionScript
  (bind _returnvalue (Rendering|Material|CreateDynamicMaterialInstance (Variables|Default|GetStaticMesh) 0 "/Game/Assets/Art/Shield/Shield_Inst.Shield_Inst" :!class /Script/Engine.PrimitiveComponent))
  (Variables|Default|Setdynamat _returnvalue)
  (bind _returnvalue_2 (Rendering|Material|CreateDynamicMaterialInstance (Variables|Default|GetDecal) :!class /Script/Engine.DecalComponent))
  (Variables|Default|Setcrack_dynamat _returnvalue_2))