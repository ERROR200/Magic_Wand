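; Menu variant of the Death Beam spell that plays a laser sound and fires a beam on spawn, destroying itself if multiple DeathBeam actors exist.
; A Tick-fed gate traces between two arrows and spawns hit effects until DamageTime expires, then stops the beam particles.
; Damage and the Steve component's move to the impact point happen only once.
; KillSpell detaches the actor, stops all menu option sliders and destroys it.
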(event EventBeginPlay
  (bind _outactors (Actor|GetAllActorsOfClass "/Game/Assets/Blueprints/Spells/DeathBeam.DeathBeam_C"))
  (if (> (Utilities|Array|Length _outactors) 1)
    (Actor|DestroyActor)
    (else
      (Audio|PlaySound2D "/Game/Assets/Sounds/New_beam/lazer_cue.lazer_cue")
      (bind _outactors_2 (Actor|GetAllActorsOfClass "/Game/Assets/Blueprints/Wand.Wand_C"))
      (Components|Activation|Activate (Variables|Default|GetBeam_Fire) false)
      (Utilities|FlowControl|Gate true) ; enters at Open
    )))

(event EventTick
  (params (DeltaSeconds :type Float%20%28single-precision%29))
  (Utilities|FlowControl|Gate true :!label _label
    (:Exit
      (bind _outhit (Collision|LineTraceForObjects (Transformation|GetWorldLocation (Variables|Default|GetArrow)) (Transformation|GetWorldLocation (Variables|Default|GetArrow1)) (Utilities|Array|MakeArray "ObjectTypeQuery1" "ObjectTypeQuery2" "ObjectTypeQuery7" "ObjectTypeQuery4") false (Utilities|Array|MakeArray (Game|Player|GetPlayerPawn 0) (Utilities|Array|Get(acopy) (stale EventBeginPlay _outactors_2))) "None"))
      (Effects|SpawnEmitteratLocation "/Game/Assets/Particles/Beam/Beam_hit.Beam_hit" (.location _outhit))
      (Utilities|FlowControl|Sequence
        (:then_0
          (Utilities|FlowControl|DoOnce false
            (:Completed
              (Class|IDamage|TakeDamage(Message) (.hitactor _outhit) 6.0 true "NewEnumerator0" 0.1 (.location _outhit))
              (Transformation|SetWorldLocation (Variables|Default|Getsteve) (.impactpoint _outhit) false false))))
        (:then_1
          (bind _output_get (Variables|Default|SetDamageTime (- (Variables|Default|GetDamageTime) (Utilities|Time|GetWorldDeltaSeconds))))
          (if (< _output_get 0.0)
            (Components|Activation|Deactivate (Variables|Default|GetBeam_charge))
            (goto _label Close)))))))

(event EventKillSpell
  (params (input_actor :type Actor%20Object%20Reference))
  (Transformation|DetachFromActor "KeepWorld" "KeepWorld" "KeepWorld")
  (bind _outactors (Actor|GetAllActorsOfClass "/Game/Assets/Blueprints/Menu_item_option_Slider.Menu_item_option_Slider_C"))
  (for _array_element _outactors
    (Default|StopSlider _array_element))
  (Actor|DestroyActor))

(fn ConstructionScript)