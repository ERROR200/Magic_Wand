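; Gargoyle fire spell projectile that damages the player pawn on overlap, or is stopped by a Ward.
; BeginPlay stores a direction toward the player's camera, but the movement and lifetime countdown logic is disconnected from Tick and never runs.
; Incoming damage, scaled by frame time, drains LifeTime.
; A hit or depleted LifeTime disables damage, deactivates the particles and destroys the actor after a short delay.
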(event OnComponentBeginOverlap(Sphere)
  (params (OverlappedComponent :type Primitive%20Component%20Object%20Reference) (OtherActor :type Actor%20Object%20Reference) (OtherComp :type Primitive%20Component%20Object%20Reference) (OtherBodyIndex :type Integer) (bFromSweep :type Boolean) (SweepResult :type Hit%20Result%20Structure%20%28by%20ref%29))
  (if (Variables|Default|GetCanDamage)
    (Utilities|Casting|CastToWard OtherActor
      (:then
        _)
      (:CastFailed
        (bind _aspersonal_mcpawn (Utilities|Casting|CastToPersonalMCPawn OtherActor))
        (Default|ReceiveDamage _aspersonal_mcpawn)))
    (Variables|Default|SetCanDamage false)
    (Components|Activation|Deactivate (Variables|Default|GetParticleSystem))
    (Utilities|FlowControl|Delay 0.1)
    (Actor|DestroyActor)))

(event EventBeginPlay
  (bind _outactors (Actor|GetAllActorsOfClass "/Game/Assets/Blueprints/PersonalMCPawn.PersonalMCPawn_C"))
  (Utilities|IsValid (Utilities|Array|Get(acopy) _outactors)
    (:Is%20Valid
      (Variables|Default|SetforwardDir (Math|Vector|Normalize (- (Transformation|GetWorldLocation (Variables|/Game/Assets/Blueprints/PersonalMCPawn.PersonalMCPawn_C|GetCamera (Utilities|Array|Get(acopy) _outactors))) (Transformation|GetActorLocation)))))))

(event Collision|EventActorBeginOverlap
  (params (OtherActor :type Actor%20Object%20Reference)))

(event EventTakeDamage
  (params (DamageAmount :type Float%20%28single-precision%29) (Constant :type Boolean) (Effect :type Effects%20Enum :default "NewEnumerator4") (EffectTime :type Float%20%28single-precision%29) (Hit_Location :type Vector :default "0, 0, 0"))
  (bind _output_get (Variables|Default|SetLifeTime (- (Variables|Default|GetLifeTime) (* (Utilities|Time|GetWorldDeltaSeconds) DamageAmount))))
  (if (<= _output_get 0.0)
    (Variables|Default|SetCanDamage false)
    (Components|Activation|Deactivate (Variables|Default|GetParticleSystem))
    (Utilities|FlowControl|Delay 0.1)
    (Actor|DestroyActor)))

(event EventTick
  (params (DeltaSeconds :type Float%20%28single-precision%29)))

(fn ConstructionScript)