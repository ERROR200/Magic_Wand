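; Death shot spell projectile that damages actors its collision sphere overlaps.
; On spawn it plays a fire pulse emitter, flies for a fixed time, then stops, deactivates its particle and disables collision before destroying itself after a second delay.
; Each overlap sends a TakeDamageMessage with damage, a timed effect and the impact point, with no actor filtering and without ending the projectile.
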(event OnComponentBeginOverlap(Sphere)
  (params (OverlappedComponent :type Primitive%20Component%20Object%20Reference) (OtherActor :type Actor%20Object%20Reference) (OtherComp :type Primitive%20Component%20Object%20Reference) (OtherBodyIndex :type Integer) (bFromSweep :type Boolean) (SweepResult :type Hit%20Result%20Structure%20%28by%20ref%29))
  (Class|IDamage|TakeDamage(Message) OtherActor 3.0 false "NewEnumerator0" 0.1 (.impactpoint SweepResult)))

(event EventBeginPlay
  (bind _returnvalue (Transformation|GetActorTransform))
  (Effects|SpawnEmitteratLocation "/Game/Assets/Particles/Beam/Beam_Pulse_fire.Beam_Pulse_fire" (.location _returnvalue) (.rotation _returnvalue))
  (Utilities|FlowControl|Delay 3.0)
  (Variables|/Script/Engine.MovementComponent|SetVelocity (Variables|Default|GetProjectileMovement) "0, 0, 0")
  (Components|Activation|Deactivate (Variables|Default|Getparticle))
  (Collision|SetCollisionEnabled (Variables|Default|GetSphere) "NoCollision")
  (Utilities|FlowControl|Delay 3.0)
  (Actor|DestroyActor))

(event Collision|EventActorBeginOverlap
  (params (OtherActor :type Actor%20Object%20Reference)))

(event EventTick
  (params (DeltaSeconds :type Float%20%28single-precision%29)))

(fn ConstructionScript)