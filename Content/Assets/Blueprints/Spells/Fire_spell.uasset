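; Fire spell actor that charges up to four fireballs and supplies their aim point, likely from a wand.
; BeginPlay and a looping timer spawn fireballs at the arrow with sound and a light timeline.
; Tick line-traces between two arrows, shows an impact marker and feeds wand and cast locations to each fireball.
; Stopping the cast timer starts the fireballs; KillSpell kills them and destroys the actor inside the loop.
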(event Custom|spawn_balls
  (Utilities|FlowControl|DoN 4
    (:Exit
      (Audio|Components|Audio|Play (Variables|Default|Getsound_Cue) 0.0)
      (bind _returnvalue (Game|SpawnActorfromClass "/Game/Assets/Blueprints/Spells/FireBall.FireBall_C" (Transformation|GetWorldTransform (Variables|Default|GetArrow)) "AlwaysSpawn" 0 0))
      (Utilities|Array|Add (Variables|Default|GetFireball) _returnvalue)
      (bind _newtrack_0 (Timeline|firelight PlayFromStart)
        (:Update
          (Rendering|Components|Light|SetIntensity (Variables|Default|GetPointLight) _newtrack_0))))))

(event Custom|stop%20casting%20timer
  (Utilities|Time|ClearandInvalidateTimerbyHandle (stale EventBeginPlay _returnvalue))
  (for _array_element (Variables|Default|GetFireball)
    (Default|Start _array_element)))

(event EventBeginPlay
  (bind _returnvalue (Utilities|Time|SetTimerbyEvent (delegate Custom|spawn_balls) (Variables|Default|Getfireball%20cast%20timer) true))
  (Utilities|FlowControl|DoN 4
    (:Exit
      (Audio|Components|Audio|Play (Variables|Default|Getsound_Cue) 0.0)
      (bind _returnvalue_2 (Game|SpawnActorfromClass "/Game/Assets/Blueprints/Spells/FireBall.FireBall_C" (Transformation|GetWorldTransform (Variables|Default|GetArrow)) "AlwaysSpawn" 0 0))
      (Utilities|Array|Add (Variables|Default|GetFireball) _returnvalue_2)
      (bind _newtrack_0 (Timeline|firelight PlayFromStart)
        (:Update
          (Rendering|Components|Light|SetIntensity (Variables|Default|GetPointLight) _newtrack_0))))))

(event EventTick
  (params (DeltaSeconds :type Float%20%28single-precision%29))
  (bind _particlesystem (Variables|Default|GetParticleSystem))
  (bind _particlesystem_2 (Variables|Default|GetParticleSystem))
  (bind (_outhit _returnvalue) (Collision|LineTraceForObjects (Transformation|GetWorldLocation (Variables|Default|GetArrow)) (Transformation|GetWorldLocation (Variables|Default|GetArrow1)) (Utilities|Array|MakeArray "ObjectTypeQuery1" "ObjectTypeQuery7") false (Variables|Default|GetFireball) "None"))
  (if _returnvalue
    (Components|Activation|SetActive _particlesystem_2 true false)
    (Rendering|SetVisibility _particlesystem_2 true false)
    (Transformation|SetWorldLocation _particlesystem (.impactpoint _outhit) false false)
    (Variables|Default|Setcast_location (Math|Vector|MakeVector (.X (Math|Vector|BreakVector (.impactpoint _outhit))) (.Y (Math|Vector|BreakVector (.impactpoint _outhit))) (+ (.Z (Math|Vector|BreakVector (.impactpoint _outhit))) 1e+02)))
    (Transformation|SetWorldRotation _particlesystem (Math|Conversions|RotationFromXVector (.impactnormal _outhit)) false false)
    (else
      (Components|Activation|SetActive _particlesystem_2 false false)
      (Rendering|SetVisibility _particlesystem_2 false false)
      (Variables|Default|Setcast_location (.traceend _outhit))))
  (for _array_element (Variables|Default|GetFireball)
    (Utilities|IsValid _array_element
      (:Is%20Valid
        (Variables|/Game/Assets/Blueprints/Spells/FireBall.FireBall_C|SetWand_location _array_element (Transformation|GetActorLocation))
        (Variables|/Game/Assets/Blueprints/Spells/FireBall.FireBall_C|SetCast_location _array_element (Variables|Default|Getcast_location))))))

(event EventKillSpell
  (params (input_actor :type Actor%20Object%20Reference))
  (Components|Activation|Deactivate (Variables|Default|GetFire_charge))
  (for _array_element (Variables|Default|GetFireball)
    (Utilities|IsValid _array_element
      (:Is%20Valid
        (Default|Kill _array_element))
      (:Is%20Not%20Valid
        _))
    (Actor|DestroyActor)))

(fn ConstructionScript)