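; Fireball spell projectile that, once started, eases toward its cast location by lerping its position each Tick.
; Sphere overlaps on a custom collision channel spawn fire bursts facing the player camera and apply damage with a timed effect.
; Each damaging hit halves speed, enlarges the fireball and spends a hit, with a gate throttling hit frequency.
; When hits run low, it stops, disables damage and particles, then destroys itself after a delay.
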(event OnComponentBeginOverlap(Sphere)
  (params (OverlappedComponent :type Primitive%20Component%20Object%20Reference) (OtherActor :type Actor%20Object%20Reference) (OtherComp :type Primitive%20Component%20Object%20Reference) (OtherBodyIndex :type Integer) (bFromSweep :type Boolean) (SweepResult :type Hit%20Result%20Structure%20%28by%20ref%29))
  (bind _returnvalue (Transformation|GetActorLocation))
  (if (Utilities|Enum|Equal(Enum) (Collision|GetCollisionObjectType OtherComp) "ECC_GameTraceChannel1")
    (bind _aspersonal_mcpawn (Utilities|Casting|CastToPersonalMCPawn (Game|Player|GetPlayerPawn 0)))
    (Effects|SpawnEmitteratLocation "/Game/Assets/Particles/Fire/fire_damage.fire_damage" _returnvalue (Math|Rotator|FindLookatRotation _returnvalue (Transformation|GetWorldLocation (Variables|/Game/Assets/Blueprints/PersonalMCPawn.PersonalMCPawn_C|GetCamera _aspersonal_mcpawn))) "2.000000,2.000000,2.000000")
    (if (> (Variables|Default|GetDamageAmount) 0.0)
      (Utilities|FlowControl|Sequence
        (:then_0
          (Utilities|FlowControl|Gate false :!label _label
            (:Exit
              (Class|IDamage|TakeDamage(Message) OtherActor (Variables|Default|GetDamageAmount) false "NewEnumerator2" 1.0 (Transformation|GetActorLocation))
              (Variables|Default|SetFireball_speed (/ (Variables|Default|GetFireball_speed) 2.0))
              (Math|Integer|DecrementInt (Variables|Default|GetHitCount)
                (:%20%20
                  (Transformation|SetActorScale3D (* (Transformation|GetActorScale3D) 1.2)))))))
        (:then_1
          (goto _label Close))
        (:then_2
          (Utilities|FlowControl|Delay (Variables|Default|GetDelayBetweenHits))
          (goto _label Open))))))

(event Custom|kill
  (Variables|Default|SetDamageAmount 0.0)
  (Components|Activation|Deactivate (Variables|Default|GetParticleSystem))
  (Utilities|FlowControl|Sequence
    (:then_0
      (Utilities|FlowControl|Gate false) ; enters at Close
    )
    (:then_1
      (Utilities|FlowControl|Delay 2.0)
      (Actor|DestroyActor))))

(event Custom|start
  (Utilities|FlowControl|Gate true) ; enters at Open
)

(event EventBeginPlay)

(event Collision|EventActorBeginOverlap
  (params (OtherActor :type Actor%20Object%20Reference)))

(event EventTick
  (params (DeltaSeconds :type Float%20%28single-precision%29))
  (Utilities|FlowControl|Gate true
    (:Exit
      (if (<= (Variables|Default|GetHitCount) 1)
        (Utilities|FlowControl|DoOnce false
          (:Completed
            (CallFunction|Kill)))
        (else
          (Utilities|FlowControl|Gate false
            (:Exit
              (Transformation|SetActorLocation (Math|Vector|Lerp(Vector) (Transformation|GetActorLocation) (Variables|Default|GetCast_location) (Variables|Default|GetFireball_speed)) false false))))))))

(fn ConstructionScript)