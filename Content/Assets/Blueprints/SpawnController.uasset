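; Wave spawner that runs the enemy waves defined in WaveInfo and tells LevelManager when all are complete.
; Tick starts each wave after a delay once EnemiesLeft reaches zero, and looping timers spawn each enemy type as a timed sub-wave.
; Enemies appear at five ground-traced points picked through a seeded random stream.
; Gargoyles are instead activated at random from existing references, leaving that pool when on their last health hit.
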(event Custom|SpawnNextWave
  (Variables|Default|SetEnableSpawning false)
  (bind _wavespawnscount (CallFunction|GetWaveSpawnTotal))
  (Variables|Default|SetNumOfEnemiesToSpawn _wavespawnscount)
  (Variables|Default|SetCurrentSpawnType 0)
  (Utilities|Time|SetTimerbyFunctionName 0 "SpawnSubWave" (.TimeBetweenSpawns (Utilities|Struct|BreakNumOfEnemies (Utilities|Array|Get(acopy) (Utilities|Struct|BreakWaveEnemies (Utilities|Array|Get(acopy) (Variables|Default|GetWaveInfo) (Variables|Default|GetCurrentWave)))))) true))

(event Custom|ReloadGargoyles
  (for _index (range 0 (- (Utilities|Array|Length (Variables|Default|GetGargoyleRefs)) 1))
    (Default|ResetHealth (Utilities|Array|Get(acopy) (Variables|Default|GetGargoyleRefs) _index))))

(event Custom|SpawnSubWave
  (if (not (Variables|Default|GetisSubWaveDelayOn))
    (bind (_enemiesleftsubwave _stopspawning _subwavedelay _timebetweenspawns) (CallFunction|SpawnEnemy))
    (if (== _enemiesleftsubwave 0)
      (Utilities|Time|ClearTimerbyFunctionName 0 "SpawnSubWave")
      (Variables|Default|SetsubWaveDelayTime _subwavedelay)
      (Variables|Default|SetisSubWaveDelayOn true)
      (if _stopspawning
        (Math|Integer|IncrementInt (Variables|Default|GetCurrentWave) :!label _label
          (:%20%20
            (Variables|Default|SetEnableSpawning true)))
        (else
          (Utilities|Time|SetTimerbyFunctionName 0 "SpawnSubWave" _timebetweenspawns true)))
      (elif _stopspawning
        (Utilities|Time|ClearTimerbyFunctionName 0 "SpawnSubWave")
        (goto _label)))
    (else
      (Utilities|FlowControl|DoOnce false :!label _label_2
        (:Completed
          (Utilities|FlowControl|Delay (Variables|Default|GetsubWaveDelayTime))
          (Variables|Default|SetisSubWaveDelayOn false)
          (Utilities|Time|SetTimerbyFunctionName 0 "SpawnSubWave" (.TimeBetweenSpawns (Utilities|Struct|BreakNumOfEnemies (Utilities|Array|Get(acopy) (Utilities|Struct|BreakWaveEnemies (Utilities|Array|Get(acopy) (Variables|Default|GetWaveInfo) (Variables|Default|GetCurrentWave)))))) true)
          (goto _label_2 Reset))))))

(event Custom|RespawnEnemy
  (params (type :type AI%20Basic%20Enemy%20Class%20Reference))
  (bind _spawnlocations (Variables|Default|GetSpawnLocations))
  (bind _spawnlocations_2 (Variables|Default|GetSpawnLocations))
  (bind _myrandom (Variables|Default|GetMyRandom))
  (bind _returnvalue (Utilities|Array|Length _spawnlocations))
  (bind _returnvalue_2 (- _returnvalue 1))
  (bind _returnvalue_3 (Math|Random|RandomIntegerinRangefromStream 0 _returnvalue_2 _myrandom))
  (bind _output (Utilities|Array|Get(acopy) _spawnlocations_2 _returnvalue_3))
  (Game|SpawnActorfromClass type (Math|Transform|MakeTransform (.location _output) (.rotation _output) "1,1,1") "Undefined" 0 0))

(event Custom|EnemyKilled
  (Variables|Default|SetEnemiesLeft (- (Variables|Default|GetEnemiesLeft) 1)))

(event EventBeginPlay
  (bind _outactors (Actor|GetAllActorsOfClass "/Game/Assets/Blueprints/LevelManager.LevelManager_C"))
  (Variables|Default|SetLevelManagerRef (Utilities|Array|Get(acopy) _outactors))
  (CallFunction|AddLocations)
  (CallFunction|GroundSpawnLocations)
  (Variables|Default|SetNumberOfWaves (Utilities|Array|Length (Variables|Default|GetWaveInfo)))
  (Class|KismetMathLibrary|SeedRandomStream (Variables|Default|GetMyRandom)))

(event Collision|EventActorBeginOverlap
  (params (OtherActor :type Actor%20Object%20Reference)))

(event EventTick
  (params (DeltaSeconds :type Float%20%28single-precision%29))
  (if (and (Variables|Default|GetEnableSpawning) (== (Variables|Default|GetEnemiesLeft) 0))
    (Utilities|FlowControl|Delay (Variables|Default|GetDelayBetweenWaves))
    (Utilities|FlowControl|DoOnce false :!label _label
      (:Completed
        (if (< (Variables|Default|GetCurrentWave) (Variables|Default|GetNumberOfWaves))
          (CallFunction|SpawnNextWave)
          (else
            (Default|WavesComplete (Variables|Default|GetLevelManagerRef))
            (Variables|Default|SetEnableSpawning false)
            (Actor|Tick|SetActorTickEnabled false)
            (Components|Activation|Deactivate (Variables|Default|GetDefaultSceneRoot))))))
    (else
      (goto _label Reset))))

(fn ConstructionScript)

(fn SpawnEnemy
  (bind _spawnlocations (Variables|Default|GetSpawnLocations))
  (bind _spawnlocations_2 (Variables|Default|GetSpawnLocations))
  (bind _myrandom (Variables|Default|GetMyRandom))
  (bind _currentwave (Variables|Default|GetCurrentWave))
  (bind _waveinfo (Variables|Default|GetWaveInfo))
  (bind _currentspawntype (Variables|Default|GetCurrentSpawnType))
  (bind _returnvalue (Utilities|Array|Length _spawnlocations))
  (bind _returnvalue_2 (- _currentspawntype 1))
  (bind _output (Utilities|Array|Get(acopy) _waveinfo _currentwave))
  (bind _enemytype (Utilities|Struct|BreakWaveEnemies _output))
  (bind _returnvalue_3 (Math|Integer|Clamp(Integer) _returnvalue_2 0 99))
  (bind _returnvalue_4 (- _returnvalue 1))
  (bind _returnvalue_5 (Math|Random|RandomIntegerinRangefromStream 0 _returnvalue_4 _myrandom))
  (bind _output_2 (Utilities|Array|Get(acopy) _enemytype _returnvalue_3))
  (bind (_enemytype_2 _numberofenemies _subwavedelay _timebetweenspawns) (Utilities|Struct|BreakNumOfEnemies _output_2))
  (bind _output_3 (Utilities|Array|Get(acopy) _spawnlocations_2 _returnvalue_5))
  (bind _newparam (CallFunction|GetAISpawnClass))
  (if (and (Utilities|IsValidClass _newparam) (> (Utilities|Array|Get(acopy) (Variables|Default|GetNumOfEnemiesToSpawn) (Variables|Default|GetCurrentSpawnType)) 0))
    (if (not (== _newparam "/Game/Assets/Blueprints/Gargoyle.Gargoyle_C"))
      (Game|SpawnActorfromClass _newparam (Math|Transform|MakeTransform (.location _output_3) (.rotation _output_3) "1,1,1") "AlwaysSpawn" 0 0)
      (else
        (CallFunction|GetGargoyle)))
    (Math|Integer|IncrementInt (Variables|Default|GetEnemiesLeft)
      (:%20%20
        (bind _result (Math|Integer|DecrementInt (Utilities|Array|Get(acopy) (Variables|Default|GetNumOfEnemiesToSpawn) (Variables|Default|GetCurrentSpawnType)))
          (:%20%20
            _)))))
  (return _result (>= (Variables|Default|GetCurrentSpawnType) (Utilities|Array|Length _enemytype)) _subwavedelay _timebetweenspawns))

(fn GetWaveSpawnTotal
  (bind _waveinfo (Variables|Default|GetWaveInfo))
  (bind _currentwave (Variables|Default|GetCurrentWave))
  (bind _output (Utilities|Array|Get(acopy) _waveinfo _currentwave))
  (bind _enemytype (Utilities|Struct|BreakWaveEnemies _output))
  (for _index (range 0 (Utilities|Array|Length _enemytype))
    (Utilities|Array|Add (LocalVariables|GettempArray) (.NumberOfEnemies (Utilities|Struct|BreakNumOfEnemies (Utilities|Array|Get(acopy) _enemytype _index)))))
  (return (LocalVariables|GettempArray)))

(fn GetAISpawnClass
  (if (<= (Utilities|Array|Get(acopy) (Variables|Default|GetNumOfEnemiesToSpawn) (Variables|Default|GetCurrentSpawnType)) 0)
    (Math|Integer|IncrementInt (Variables|Default|GetCurrentSpawnType)
      (:%20%20
        _)))
  (return (.Enemytype (Utilities|Struct|BreakNumOfEnemies (Utilities|Array|Get(acopy) (Utilities|Struct|BreakWaveEnemies (Utilities|Array|Get(acopy) (Variables|Default|GetWaveInfo) (Variables|Default|GetCurrentWave))) (Variables|Default|GetCurrentSpawnType))))))

(fn AddLocations
  (bind _spawnpoint1 (Variables|Default|GetSpawnPoint1))
  (bind _spawnpoint2 (Variables|Default|GetSpawnPoint2))
  (bind _spawnpoint3 (Variables|Default|GetSpawnPoint3))
  (bind _spawnpoint4 (Variables|Default|GetSpawnPoint4))
  (bind _spawnpoint5 (Variables|Default|GetSpawnPoint5))
  (Utilities|Array|Add (Variables|Default|GetSpawnLocations) (Transformation|GetWorldTransform _spawnpoint1))
  (Rendering|ToggleVisibility _spawnpoint1 false)
  (Utilities|Array|Add (Variables|Default|GetSpawnLocations) (Transformation|GetWorldTransform _spawnpoint2))
  (Rendering|ToggleVisibility _spawnpoint2 false)
  (Utilities|Array|Add (Variables|Default|GetSpawnLocations) (Transformation|GetWorldTransform _spawnpoint3))
  (Rendering|ToggleVisibility _spawnpoint3 false)
  (Utilities|Array|Add (Variables|Default|GetSpawnLocations) (Transformation|GetWorldTransform _spawnpoint4))
  (Rendering|ToggleVisibility _spawnpoint4 false)
  (Utilities|Array|Add (Variables|Default|GetSpawnLocations) (Transformation|GetWorldTransform _spawnpoint5))
  (Rendering|ToggleVisibility _spawnpoint5 false))

(fn GroundSpawnLocations
  (for _index (range 0 (- (Utilities|Array|Length (Variables|Default|GetSpawnLocations)) 1))
    (bind (_outhit _returnvalue) (Collision|LineTraceByChannel (.location (Utilities|Array|Get(acopy) (Variables|Default|GetSpawnLocations) _index)) (- (.location (Utilities|Array|Get(acopy) (Variables|Default|GetSpawnLocations) _index)) "0, 0,10000.000000") "TraceTypeQuery1" false 0 "None"))
    (if _returnvalue
      (Utilities|Array|SetArrayElem (Variables|Default|GetSpawnLocations) _index (Math|Transform|MakeTransform (.Location (Collision|BreakHitResult _outhit)) "0, 0, 0" "1,1,1")))))

(fn GetTotalEnemyCount
  (for _array_element (Variables|Default|GetWaveInfo)
    (for _array_element_2 (Utilities|Struct|BreakWaveEnemies _array_element)
      (if (not (== (.Enemytype (Utilities|Struct|BreakNumOfEnemies _array_element_2)) "/Game/Assets/Blueprints/Gargoyle.Gargoyle_C"))
        (LocalVariables|Settally (+ (.NumberOfEnemies (Utilities|Struct|BreakNumOfEnemies _array_element_2)) (LocalVariables|Gettally))))))
  (return (+ (Utilities|Array|Length (Variables|Default|GetGargoyleRefs)) (LocalVariables|Gettally))))

(fn GetGargoyle
  (bind _gargoylerefs (Variables|Default|GetGargoyleRefs))
  (bind _myrandom (Variables|Default|GetMyRandom))
  (bind _returnvalue (Utilities|Array|Length _gargoylerefs))
  (bind _returnvalue_2 (Class|KismetMathLibrary|RandomIntegerfromStream _returnvalue _myrandom))
  (LocalVariables|SetrandomValue _returnvalue_2)
  (while (Variables|/Game/Assets/Blueprints/Gargoyle.Gargoyle_C|GetisActive (Utilities|Array|Get(acopy) _gargoylerefs (LocalVariables|GetrandomValue)))
    (LocalVariables|SetrandomValue _returnvalue_2))
  (Variables|/Game/Assets/Blueprints/Gargoyle.Gargoyle_C|SetisActive (Utilities|Array|Get(acopy) _gargoylerefs (LocalVariables|GetrandomValue)) true)
  (if (not (!= (Variables|/Game/Assets/Blueprints/Gargoyle.Gargoyle_C|GetHealthHits (Utilities|Array|Get(acopy) _gargoylerefs (LocalVariables|GetrandomValue))) 1))
    (Utilities|Array|RemoveIndex (Variables|Default|GetGargoyleRefs) (LocalVariables|GetrandomValue))))