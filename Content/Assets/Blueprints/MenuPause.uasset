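; MenuPause is an actor that pauses the game when the VR headset comes off and resumes it when worn.
; Shortly after BeginPlay, outside testing mode, it adds a VRNotifications component to its parent actor and binds both headset delegates.
; Tick prints input-focus and tracking debug text and unpauses once each time focus returns.
; A looping timer for focus-based pause checking is left unconnected.
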(event Custom|PutOnHeadset
  (Game|SetGamePaused false))

(event Custom|TakeOffHeadset
  (Game|SetGamePaused true))

(event Custom|UpdatePause
  ;[1 1 1] Pause Checking
  (Game|SetGamePaused (not (Class|OculusFunctionLibrary|HasInputFocus))))

(event EventBeginPlay
  (bind _returnvalue (Actor|GetParentActor))
  (Utilities|FlowControl|Delay 0.2)
  (if (not (Variables|Default|GetisTestingMode))
    (Utilities|IsValid _returnvalue
      (:Is%20Valid
        (bind _returnvalue_2 (AddComponent|AddVRNotificationsComponent _returnvalue))
        (EventDispatchers|BindEventtoHMDPutonHeadDelegate _returnvalue_2 (delegate Custom|PutOnHeadset))
        (EventDispatchers|BindEventtoHMDRemovedfromHeadDelegate _returnvalue_2 (delegate Custom|TakeOffHeadset))))))

(event Collision|EventActorBeginOverlap
  (params (OtherActor :type Actor%20Object%20Reference)))

(event EventTick
  (params (DeltaSeconds :type Float%20%28single-precision%29))
  (bind _returnvalue (Class|OculusFunctionLibrary|HasInputFocus))
  (Development|PrintString (Utilities|String|Append " 
 
 
 
 
 
 
 
 
 
 
 
 
 
 
 
 
Has input: " (Utilities|String|ToString(Boolean) _returnvalue) " 
Valid tracking: " (Utilities|String|ToString(Boolean) (Class|HeadMountedDisplayFunctionLibrary|HasValidTrackingPosition))) true true "(R=0.000000,G=0.660000,B=1.000000,A=1.000000)" DeltaSeconds)
  (if _returnvalue
    (Utilities|FlowControl|DoOnce false :!label _label
      (:Completed
        (Game|SetGamePaused false)))
    (else
      (goto _label Reset))))

(fn ConstructionScript)