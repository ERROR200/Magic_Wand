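; PillarEnergy is an energy pillar Blueprint that grows in height and changes opacity shortly after it spawns.
; The construction script creates a dynamic material instance on the PillarHold component and stores it as DynamicMat.
; BeginPlay zeroes the "Opacity Overide" parameter, waits briefly, then plays the Spawn timeline, whose Height and Opacity tracks drive PillarHold's Z scale and that parameter.
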(event EventBeginPlay
  (Rendering|Material|SetScalarParameterValue (Variables|Default|GetDynamicMat) "Opacity Overide" 0.0 :!class /Script/Engine.MaterialInstanceDynamic)
  (Utilities|FlowControl|Delay 1.0)
  (bind (_direction _height _opacity) (Timeline|Spawn Play)
    (:Update
      (Transformation|SetWorldScale3D (Variables|Default|GetPillarHold) (Math|Vector|MakeVector 1.0 1.0 _height))
      (Rendering|Material|SetScalarParameterValue (Variables|Default|GetDynamicMat) "Opacity Overide" _opacity :!class /Script/Engine.MaterialInstanceDynamic))))

(event Collision|EventActorBeginOverlap
  (params (OtherActor :type Actor%20Object%20Reference)))

(event EventTick
  (params (DeltaSeconds :type Float%20%28single-precision%29)))

(fn ConstructionScript
  (bind _pillarhold (Variables|Default|GetPillarHold))
  (bind _returnvalue (Rendering|Material|CreateDynamicMaterialInstance _pillarhold 0 (Rendering|Material|GetMaterial _pillarhold 0) :!class /Script/Engine.PrimitiveComponent))
  (Variables|Default|SetDynamicMat _returnvalue))