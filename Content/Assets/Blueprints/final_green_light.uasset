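; Green light actor that stays dark at level start and lights up when its glow event is triggered.
; On BeginPlay it caches the light component's intensity as GlowLevel, then sets the intensity to zero.
; The glow event restores that intensity and, if the Bats reference is valid, activates that actor's root component.
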(event Custom|glow
  (bind _bats (Variables|Default|Getbats))
  (Rendering|Components|Light|SetIntensity (Variables|Default|GetLightComponent) (Variables|Default|Getglow%20level))
  (Utilities|IsValid _bats
    (:Is%20Valid
      (Components|Activation|Activate (Variables|/Script/Engine.Actor|GetRootComponent _bats) true))))

(event EventBeginPlay
  (bind _lightcomponent (Variables|Default|GetLightComponent))
  (Variables|Default|Setglow%20level (Variables|/Script/Engine.LightComponentBase|GetIntensity _lightcomponent))
  (Rendering|Components|Light|SetIntensity _lightcomponent 0.0))

(event EventTick
  (params (DeltaSeconds :type Float%20%28single-precision%29)))

(fn ConstructionScript)