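; Score_current is a Blueprint that keeps the running score and shows it through a score widget from its Widget component.
; BeginPlay caches that widget and initializes the display.
; The update event adds multiplier-scaled points to Score and pushes score and multiplier to the widget.
; A multiplier above one is incremented and starts a five-second countdown in Tick, which resets it to one on expiry without refreshing the widget.
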(event Custom|update
  (params (Value :type Float%20%28single-precision%29) (Multiplier :type Integer))
  (bind _score_widget (Variables|Default|Getscore_widget))
  (if (> Multiplier 1)
    (bind _result (Math|Integer|IncrementInt (Variables|Default|Getmultiplier))
      (:%20%20
        (Variables|Default|SetCounter 5.0))))
  (Utilities|IsValid _score_widget
    (:Is%20Valid
      (bind _output_get (Variables|Default|SetScore (+ (* _result Value) (Variables|Default|GetScore))))
      (Default|UpdateScore _score_widget _output_get)
      (Default|SetMultiplier _score_widget (Variables|Default|Getmultiplier)))))

(event EventBeginPlay
  (bind _asscore_current_widjet (Utilities|Casting|CastToscore_current_widjet (UserInterface|GetUserWidgetObject (Variables|Default|GetWidget))))
  (Variables|Default|Setscore_widget _asscore_current_widjet)
  (CallFunction|Update 0.0 1))

(event Collision|EventActorBeginOverlap
  (params (OtherActor :type Actor%20Object%20Reference)))

(event EventTick
  (params (DeltaSeconds :type Float%20%28single-precision%29))
  (if (> (Variables|Default|GetCounter) 0.0)
    (bind _output_get (Variables|Default|SetCounter (- (Variables|Default|GetCounter) DeltaSeconds)))
    (if (<= _output_get 0.0)
      (Variables|Default|Setmultiplier 1))))

(fn ConstructionScript)