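; Axe is a spinning, flying actor that homes in on the player's camera.
; On BeginPlay it caches the first PersonalMCPawn as the player.
; Each tick it spins its Pivot in pitch and, once an aim delay runs out, lerps the root's rotation toward a point slightly offset from the camera.
; The root moves along its forward vector by a fixed step per frame without sweeping, so travel speed depends on frame rate.
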(event EventBeginPlay
  (bind _outactors (Actor|GetAllActorsOfClass "/Game/Assets/Blueprints/PersonalMCPawn.PersonalMCPawn_C"))
  (Variables|Default|SetPlayerRef (Utilities|Array|Get(acopy) _outactors)))

(event Collision|EventActorBeginOverlap
  (params (OtherActor :type Actor%20Object%20Reference)))

(event EventTick
  (params (DeltaSeconds :type Float%20%28single-precision%29))
  (bind _returnvalue (Utilities|Time|GetWorldDeltaSeconds))
  (bind _defaultsceneroot (Variables|Default|GetDefaultSceneRoot))
  (bind _defaultsceneroot_2 (Variables|Default|GetDefaultSceneRoot))
  (Transformation|AddLocalRotation (Variables|Default|GetPivot) (Math|Rotator|MakeRotator 0.0 (* DeltaSeconds (Variables|Default|GetCurrentRotateSpeed)) 0.0) false false)
  (if (<= (Variables|Default|GetAimDelay) 0.0)
    (Transformation|SetRelativeRotation _defaultsceneroot (Math|Rotator|Lerp(Rotator) (Variables|/Script/Engine.SceneComponent|GetRelativeRotation _defaultsceneroot_2) (Math|Rotator|FindLookatRotation (Transformation|GetWorldLocation _defaultsceneroot_2) (- (Transformation|GetWorldLocation (Variables|/Game/Assets/Blueprints/PersonalMCPawn.PersonalMCPawn_C|GetCamera (Variables|Default|GetPlayerRef))) (Math|Vector|MakeVector 0.0 2.0 0.0))) (* _returnvalue (Variables|Default|GetAimSpeed)) true) false false)
    (else
      (Variables|Default|SetAimDelay (- (Variables|Default|GetAimDelay) _returnvalue))))
  (Transformation|AddRelativeLocation _defaultsceneroot (* (Math|Vector|GetForwardVector (Variables|Default|GetDefaultSceneRoot)) 2.0) false false))

(fn ConstructionScript)