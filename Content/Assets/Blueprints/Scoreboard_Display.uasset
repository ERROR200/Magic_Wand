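; Scoreboard display actor that fades in a plane and then shows a score on its widget.
; The construction script creates dynamic material instances for the plane's two material slots, and BeginPlay zeroes their opacity fade.
; Scoreboard_activate plays a timeline that raises both fades, the first only to a faint level.
; When the timeline finishes, it passes the score to the Scoreboard user widget's Update.
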(event Custom|Scoreboard_activate
  (params (Score :type Integer))
  (bind _newtrack_0 (Timeline|Timeline_0 Play)
    (:Update
      (Rendering|Material|SetScalarParameterValue (Variables|Default|Getdynamat) "Opacity Fade" (Math|Float|Lerp 0.0 0.03 _newtrack_0) :!class /Script/Engine.MaterialInstanceDynamic)
      (Rendering|Material|SetScalarParameterValue (Variables|Default|Getdynamat2) "Opacity Fade" _newtrack_0 :!class /Script/Engine.MaterialInstanceDynamic))
    (:Finished
      (bind _asscoreboard (Utilities|Casting|CastToScoreboard (UserInterface|GetUserWidgetObject (Variables|Default|GetWidget))))
      (Default|Update _asscoreboard Score))))

(event EventBeginPlay
  (Rendering|Material|SetScalarParameterValue (Variables|Default|Getdynamat) "Opacity Fade" 0.0 :!class /Script/Engine.MaterialInstanceDynamic)
  (Rendering|Material|SetScalarParameterValue (Variables|Default|Getdynamat2) "Opacity Fade" 0.0 :!class /Script/Engine.MaterialInstanceDynamic))

(event Collision|EventActorBeginOverlap
  (params (OtherActor :type Actor%20Object%20Reference)))

(event EventTick
  (params (DeltaSeconds :type Float%20%28single-precision%29)))

(fn ConstructionScript
  (bind _plane (Variables|Default|GetPlane))
  (bind _returnvalue (Rendering|Material|CreateDynamicMaterialInstance _plane 0 0 :!class /Script/Engine.PrimitiveComponent))
  (Variables|Default|Setdynamat _returnvalue)
  (bind _returnvalue_2 (Rendering|Material|CreateDynamicMaterialInstance _plane 1 0 :!class /Script/Engine.PrimitiveComponent))
  (Variables|Default|Setdynamat2 _returnvalue_2))