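; Necrobeam spell actor in the Boss_AI folder that fires a continuous stream of necrobeam projectiles.
; After a short startup delay on BeginPlay, it plays fire and hold sounds while a looping timer spawns projectiles from its Arrow.
; An older sphere-trace beam with hit effects and damage is left disconnected, as is the destroy logic.
; KillSpell is empty, so nothing here stops the stream.
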(event Custom|spawn%20projectile
  (Game|SpawnActorfromClass "/Game/Assets/Blueprints/Boss_AI/Necrobeam_projectile.Necrobeam_projectile_C" (Transformation|GetWorldTransform (Variables|Default|GetArrow)) "AlwaysSpawn" 0 0))

(event EventBeginPlay
  (bind _outactors (Actor|GetAllActorsOfClass "/Game/Assets/Blueprints/Wand.Wand_C"))
  (Utilities|FlowControl|Delay 2.0)
  (Audio|Components|Audio|Play (Variables|Default|GetBeam_fire_sound) 0.0)
  (Utilities|FlowControl|Sequence
    (:then_0
      (Utilities|Time|SetTimerbyEvent (delegate Custom|spawn%20projectile) 0.1 true))
    (:then_1
      (Utilities|FlowControl|Delay 0.2)
      (Audio|Components|Audio|Play (Variables|Default|GetBeam_hold_sound) 0.0))))

(event EventTick
  (params (DeltaSeconds :type Float%20%28single-precision%29)))

(event EventKillSpell
  (params (input_actor :type Actor%20Object%20Reference)))

(fn ConstructionScript)