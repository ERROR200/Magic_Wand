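; Tutorial flag actor that shows a series of lesson images (wand, shield, bag, food) while Wilfred plays matching narration.
; On BeginPlay it plays the grab line and a float timeline.
; ChangeMaterial fades a dynamic material's Amount, swaps in the next material, unlocks player shield and eat flags, and re-calls itself after each clip when PaxTutorial is set.
; After the last clip it moves the LevelManager, enables spawning, then flies away and destroys itself.
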(event Custom|ChangeMaterial
  (bind _flag_test (Variables|Default|GetFlag_Test))
  (bind _defaultsceneroot (Variables|Default|GetDefaultSceneRoot))
  (bind _wilfredref (Variables|Default|GetWilfredRef))
  (bind _returnvalue (Transformation|GetWorldLocation _defaultsceneroot))
  (bind _newtrack_0 (Timeline|Swap Play)
    (:Update
      (Rendering|Material|SetScalarParameterValue (Variables|Default|GetDynamicMat) "Amount" _newtrack_0 :!class /Script/Engine.MaterialInstanceDynamic))
    (:Finished
      (Utilities|FlowControl|Delay 1.0)
      (if (== _newtrack_0 1.0)
        (bind (_return _audio _time) (CallFunction|GetNextMaterial))
        (Utilities|FlowControl|Sequence
          (:then_0
            (Rendering|Material|SetMaterial _flag_test 1 _return)
            (bind _returnvalue_2 (Rendering|Material|CreateDynamicMaterialInstance _flag_test 1 _return :!class /Script/Engine.PrimitiveComponent))
            (bind _output_get (Variables|Default|SetDynamicMat _returnvalue_2))
            (Rendering|Material|SetScalarParameterValue _output_get "Amount" 1.0 :!class /Script/Engine.MaterialInstanceDynamic)
            (Math|Integer|IncrementInt (Variables|Default|GetMaterialIndex)
              (:%20%20
                (Timeline|Swap Reverse))))
          (:then_1
            ;[1 1 1] Audio to play
            (Utilities|FlowControl|Delay 1.5)
            (if (Variables|Default|GetPaxTutorial)
              (Utilities|IsValid _wilfredref
                (:Is%20Valid
                  (Default|SetAudio _wilfredref _audio)
                  (if (== (Variables|Default|GetMaterialIndex) 4)
                    (Utilities|FlowControl|Delay _time)
                    (Utilities|FlowControl|Delay 0.5)
                    (bind _outactors (Actor|GetAllActorsOfClass "/Game/Assets/Blueprints/LevelManager.LevelManager_C"))
                    (Utilities|IsValid (Utilities|Array|Get(acopy) _outactors)
                      (:Is%20Valid
                        (bind _outactors_2 (Actor|GetAllActorsOfClass "/Game/Assets/Blueprints/LevelManagerPoint.LevelManagerPoint_C"))
                        (Utilities|IsValid (Utilities|Array|Get(acopy) _outactors_2)
                          (:Is%20Valid
                            (Default|MovetoLocation (Utilities|Array|Get(acopy) _outactors) 1.0 (Transformation|GetWorldTransform (Variables|/Game/Assets/Blueprints/LevelManagerPoint.LevelManagerPoint_C|GetOrb_point (Utilities|Array|Get(acopy) _outactors_2))))
                            (Utilities|FlowControl|Delay 0.5)
                            (Variables|/Game/Assets/Blueprints/SpawnController.SpawnController_C|SetEnableSpawning (Variables|Default|GetSpawnContRef) true)
                            (bind _newtrack_1 (Timeline|FlyAway Play)
                              (:Update
                                (Transformation|SetWorldLocation _defaultsceneroot (Math|Vector|MakeVector (.x _returnvalue) (.y _returnvalue) (+ (.z _returnvalue) _newtrack_1)) false false))
                              (:Finished
                                (Actor|DestroyActor)))))))
                    (else
                      (Utilities|FlowControl|Delay _time)
                      (CallFunction|ChangeMaterial))))))))))))

(event EventBeginPlay
  (bind _defaultsceneroot (Variables|Default|GetDefaultSceneRoot))
  (bind _outactors (Actor|GetAllActorsOfClass "/Game/Assets/Blueprints/Wilfred.Wilfred_C"))
  (Variables|Default|SetWilfredRef (Utilities|Array|Get(acopy) _outactors))
  (bind _outactors_2 (Actor|GetAllActorsOfClass "/Game/Assets/Blueprints/SpawnController.SpawnController_C"))
  (Variables|Default|SetSpawnContRef (Utilities|Array|Get(acopy) _outactors_2))
  (if (== (Utilities|Array|Length _outactors_2) 1)
    (bind _outactors_3 (Actor|GetAllActorsOfClass "/Game/Assets/Blueprints/PersonalMCPawn.PersonalMCPawn_C"))
    (Variables|Default|SetPlayerRef (Utilities|Array|Get(acopy) _outactors_3))
    (Utilities|FlowControl|Delay 1.5)
    (Utilities|IsValid (Variables|Default|GetWilfredRef)
      (:Is%20Valid
        (Default|SetAudio (Variables|Default|GetWilfredRef) (Variables|Default|GetGrabAudio))
        (bind _newtrack_1 (Timeline|Float Play)
          (:Update
            (Transformation|SetRelativeLocation _defaultsceneroot (+ (* (Math|Vector|GetRightVector _defaultsceneroot) (.x _newtrack_1)) (+ (Math|Vector|MakeVector 0.0 0.0 (.z _newtrack_1)) (Transformation|GetWorldLocation _defaultsceneroot))) false false)))))))

(event Collision|EventActorBeginOverlap
  (params (OtherActor :type Actor%20Object%20Reference)))

(event EventTick
  (params (DeltaSeconds :type Float%20%28single-precision%29)))

(fn ConstructionScript
  (bind _flag_test (Variables|Default|GetFlag_Test))
  (bind _returnvalue (Rendering|Material|CreateDynamicMaterialInstance _flag_test 1 (Rendering|Material|GetMaterial _flag_test 1) :!class /Script/Engine.PrimitiveComponent))
  (Variables|Default|SetDynamicMat _returnvalue))

(fn GetNextMaterial
  (bind _wandaudio (Variables|Default|GetWandAudio))
  (bind _shieldaudio (Variables|Default|GetShieldAudio))
  (bind _bagaudio (Variables|Default|GetBagAudio))
  (bind _playerref (Variables|Default|GetPlayerRef))
  (bind _foodaudio (Variables|Default|GetFoodAudio))
  (switch int (Variables|Default|GetMaterialIndex)
    (:0
      (return (Variables|Default|GetWandMat) _wandaudio (Variables|/Script/Engine.SoundBase|GetDuration _wandaudio)))
    (:1
      (Utilities|IsValid _playerref
        (:Is%20Valid
          (Variables|/Game/Assets/Blueprints/PersonalMCPawn.PersonalMCPawn_C|SetCanGetShield _playerref true))
        (:Is%20Not%20Valid
          _))
      (return (Variables|Default|GetShieldMat) _shieldaudio (Variables|/Script/Engine.SoundBase|GetDuration _shieldaudio)))
    (:2
      (Utilities|IsValid _playerref
        (:Is%20Valid
          (Variables|/Game/Assets/Blueprints/PersonalMCPawn.PersonalMCPawn_C|SeteatTrigger _playerref true))
        (:Is%20Not%20Valid
          _))
      (return (Variables|Default|GetBagMat) _bagaudio (Variables|/Script/Engine.SoundBase|GetDuration _bagaudio)))
    (:3
      (return (Variables|Default|GetFoodMat) _foodaudio (Variables|/Script/Engine.SoundBase|GetDuration _foodaudio)))))