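; VR wand actor that the player picks up and drops by hand, gating spellcasting through CanCast.
; Pickup attaches the mesh and notifies PersonalMCPawn; dropping enables physics, detaches it and destroys all Spell-tagged actors.
; A gated delay after dropping, or a mesh hit while neither held nor holstered, triggers a glow-material despawn and pawn-driven respawn.
; Timelines drive spawn scaling plus colour and flash changes on a dynamic material.
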(event OnComponentHit(StaticMesh)
  (params (HitComponent :type Primitive%20Component%20Object%20Reference) (OtherActor :type Actor%20Object%20Reference) (OtherComp :type Primitive%20Component%20Object%20Reference) (NormalImpulse :type Vector :default "0, 0, 0") (Hit :type Hit%20Result%20Structure%20%28by%20ref%29))
  (bind _staticmesh (Variables|Default|GetStaticMesh))
  (if (not (or (Variables|Default|Getis%20held) (Variables|Default|GetisHolstered)))
    (Utilities|FlowControl|DoOnce false
      (:Completed
        (bind _returnvalue (Rendering|Material|CreateDynamicMaterialInstance "/Game/Assets/Art/Wand/Wand_Glow.Wand_Glow" :!class /Script/Engine.KismetMaterialLibrary))
        (Rendering|Material|SetMaterial _staticmesh 0 _returnvalue)
        (Effects|SpawnEmitteratLocation "/Game/Assets/Particles/wand_despawn.wand_despawn" (Transformation|GetWorldLocation _staticmesh) (Transformation|GetWorldRotation _staticmesh))
        (bind (_direction _alpha _emissive) (Timeline|Timeline_0 Play)
          (:Update
            (Rendering|Material|SetScalarParameterValue _returnvalue "Alpha" _alpha :!class /Script/Engine.MaterialInstanceDynamic)
            (Rendering|Material|SetScalarParameterValue _returnvalue "Emissive" _emissive :!class /Script/Engine.MaterialInstanceDynamic))
          (:Finished
            (bind _aspersonal_mcpawn (Utilities|Casting|CastToPersonalMCPawn (Game|Player|GetPlayerPawn 0)))
            (Default|RespawnWand _aspersonal_mcpawn)))))))

(event Custom|DestorySelf
  (bind _staticmesh (Variables|Default|GetStaticMesh))
  (if (not (or (Variables|Default|Getis%20held) (Variables|Default|GetisHolstered)))
    (Utilities|FlowControl|DoOnce false
      (:Completed
        (bind _returnvalue (Rendering|Material|CreateDynamicMaterialInstance "/Game/Assets/Art/Wand/Wand_Glow.Wand_Glow" :!class /Script/Engine.KismetMaterialLibrary))
        (Rendering|Material|SetMaterial _staticmesh 0 _returnvalue)
        (Effects|SpawnEmitteratLocation "/Game/Assets/Particles/wand_despawn.wand_despawn" (Transformation|GetWorldLocation _staticmesh) (Transformation|GetWorldRotation _staticmesh))
        (bind (_direction _alpha _emissive) (Timeline|Timeline_0 Play)
          (:Update
            (Rendering|Material|SetScalarParameterValue _returnvalue "Alpha" _alpha :!class /Script/Engine.MaterialInstanceDynamic)
            (Rendering|Material|SetScalarParameterValue _returnvalue "Emissive" _emissive :!class /Script/Engine.MaterialInstanceDynamic))
          (:Finished
            (bind _aspersonal_mcpawn (Utilities|Casting|CastToPersonalMCPawn (Game|Player|GetPlayerPawn 0)))
            (Default|RespawnWand _aspersonal_mcpawn)))))))

(event Custom|ChangeColour
  (params (Colour :type Linear%20Color%20Structure) (Flash :type Boolean))
  (bind _bodymaterial (Variables|Default|GetBodyMaterial))
  (bind _returnvalue (Rendering|Material|GetVectorParameterValue (Variables|Default|GetBodyMaterial) "Emissive Colour" :!class /Script/Engine.MaterialInstanceDynamic))
  (Utilities|FlowControl|Sequence
    (:then_0
      (bind _newtrack_0 (Timeline|ColourChange PlayFromStart)
        (:Update
          (Rendering|Material|SetVectorParameterValue _bodymaterial "Emissive Colour" (Math|Color|Lerp(LinearColor) _returnvalue Colour _newtrack_0) :!class /Script/Engine.MaterialInstanceDynamic))))
    (:then_1
      (if Flash
        (bind _newtrack_0_2 (Timeline|Flash PlayFromStart)
          (:Update
            (Rendering|Material|SetScalarParameterValue _bodymaterial "Emissive Intensity" _newtrack_0_2 :!class /Script/Engine.MaterialInstanceDynamic)
            (Rendering|Material|SetScalarParameterValue _bodymaterial "Secondary Emissive Strength" (Math|Float|MapRangeClamped _newtrack_0_2 2.5 1e+02 0.1 0.5) :!class /Script/Engine.MaterialInstanceDynamic)))))))

(event Custom|ReturnToNormal
  (bind _bodymaterial (Variables|Default|GetBodyMaterial))
  (bind _returnvalue (Rendering|Material|GetVectorParameterValue (Variables|Default|GetBodyMaterial) "Emissive Colour" :!class /Script/Engine.MaterialInstanceDynamic))
  (Utilities|FlowControl|Sequence
    (:then_0
      (bind _newtrack_0 (Timeline|Flash ReverseFromEnd)
        (:Update
          (Rendering|Material|SetScalarParameterValue _bodymaterial "Emissive Intensity" _newtrack_0 :!class /Script/Engine.MaterialInstanceDynamic)
          (Rendering|Material|SetScalarParameterValue _bodymaterial "Secondary Emissive Strength" (Math|Float|MapRangeClamped _newtrack_0 2.5 1e+02 0.1 0.5) :!class /Script/Engine.MaterialInstanceDynamic))))
    (:then_1
      (bind _newtrack_0_2 (Timeline|Timeline_2 PlayFromStart)
        (:Update
          (Rendering|Material|SetVectorParameterValue (Variables|Default|GetBodyMaterial) "Emissive Colour" (Math|Color|Lerp(LinearColor) _returnvalue (Variables|Default|GetOriginalColour) _newtrack_0_2) :!class /Script/Engine.MaterialInstanceDynamic))))))

(event EventBeginPlay
  (bind _bodymaterial (Variables|Default|GetBodyMaterial))
  (bind _aspersonal_mcpawn (Utilities|Casting|CastToPersonalMCPawn (Game|Player|GetPlayerPawn 0)))
  (Rendering|Material|SetVectorParameterValue _bodymaterial "Emissive Colour" (Variables|Default|GetOriginalColour) :!class /Script/Engine.MaterialInstanceDynamic)
  (Rendering|Material|SetScalarParameterValue _bodymaterial "Secondary Emissive Strength" 0.1 :!class /Script/Engine.MaterialInstanceDynamic)
  (Rendering|Material|SetScalarParameterValue _bodymaterial "Emissive Intensity" 2.5 :!class /Script/Engine.MaterialInstanceDynamic)
  (bind _size (Timeline|Timeline_1 PlayFromStart)
    (:Update
      (Transformation|SetActorScale3D (Math|Conversions|ToVector(Float) _size)))))

(event EventPickup
  (params (AttachTo :type Scene%20Component%20Object%20Reference) (hand :type EControllerHand%20Enum :default "Left"))
  (Utilities|FlowControl|DoOnce false
    (:Completed
      (Utilities|FlowControl|Sequence
        (:then_0
          (Variables|Default|Setused%20hand hand)
          (Variables|Default|SetisHolstered false)
          (Variables|Default|Setis%20held true)
          (Variables|Default|Setcan%20cast true)
          (Physics|SetSimulatePhysics (Variables|Default|GetStaticMesh) false)
          (Transformation|AttachComponentToComponent (Variables|Default|GetStaticMesh) AttachTo "None" "SnapToTarget" "SnapToTarget" "KeepWorld" false)
          (Utilities|FlowControl|Gate false) ; enters at Close
        )
        (:then_1
          (Utilities|FlowControl|DoOnce false
            (:Completed
              (Default|DetachWand (stale EventBeginPlay _aspersonal_mcpawn)))))))))

(event EventDrop
  (params (hand :type EControllerHand%20Enum :default "Left"))
  (if (Utilities|Enum|Equal(Enum) hand (Variables|Default|Getused%20hand))
    (Utilities|FlowControl|Sequence
      (:then_0
        (Physics|SetSimulatePhysics (Variables|Default|GetStaticMesh) true)
        (Utilities|FlowControl|Sequence
          (:then_0
            (Variables|Default|Setis%20held false)
            (Transformation|DetachFromActor "KeepWorld" "KeepWorld" "KeepWorld")
            (bind _outactors (Actor|GetAllActorswithTag "Spell"))
            (for _array_element _outactors
              (Actor|DestroyActor _array_element))
            (Variables|Default|Setcan%20cast false))
          (:then_1
            (goto _label Open))
          (:then_2
            (Utilities|FlowControl|Delay 3.0)
            (Utilities|FlowControl|Gate false :!label _label
              (:Exit
                (CallFunction|DestorySelf))))))
      (:then_1
        (Utilities|FlowControl|DoOnce false) ; enters at Reset
      ))))

(fn ConstructionScript
  (bind _staticmesh (Variables|Default|GetStaticMesh))
  (bind _returnvalue (Rendering|Material|CreateDynamicMaterialInstance _staticmesh 0 (Rendering|Material|GetMaterial _staticmesh 0) :!class /Script/Engine.PrimitiveComponent))
  (bind _output_get (Variables|Default|SetBodyMaterial _returnvalue))
  (bind _returnvalue_2 (Rendering|Material|GetVectorParameterValue _output_get "Emissive Colour" :!class /Script/Engine.MaterialInstanceDynamic))
  (Variables|Default|SetOriginalColour _returnvalue_2))