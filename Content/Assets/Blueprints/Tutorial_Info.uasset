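; Tutorial director that runs spoken lessons through the LevelManager's audio, moving it between talking position and start location.
; A DialogueAudio table links clips to completion and help branches, with Tick counting down to help prompts and PlayNextClip letting other code advance.
; Each clip's action or animation triggers gameplay like wand, skulls, apples, spells, hand demos and the level ending.
; A looping timer maps clip amplitude to emissive glow.
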(event Custom|ResetSkullSpawns
  (bind _levelmanagerref (Variables|Default|GetLevelManagerRef))
  (bind _levelmanagerref_2 (Variables|Default|GetLevelManagerRef))
  (Variables|Default|SetisInTalkingPos false)
  (Utilities|FlowControl|DoOnce false) ; enters at Reset
)

(event Custom|StopTutorial
  (params (level :type Integer))
  (bind _levelmanagerref (Variables|Default|GetLevelManagerRef))
  (bind _audio (Variables|/Game/Assets/Blueprints/LevelManager.LevelManager_C|GetAudio _levelmanagerref))
  ;[1 1 1] Skip tutorial
  (if (Audio|Components|Audio|IsPlaying _audio)
    (Audio|Components|Audio|Stop _audio))
  (if (Variables|Default|GetBeginningTutorialDone)
    _
    (else
      (Variables|Default|SetCurrent_Index (+ (* level 4) 12))))
  (Variables|Default|SetBeginningTutorialDone true)
  (Variables|Default|SetTutorialActive false)
  (Default|RespawnWand (Variables|/Game/Assets/Blueprints/LevelManager.LevelManager_C|GetPlayerRef (Variables|Default|GetLevelManagerRef))))

(event Custom|PlayNextClip
  (params (NextIndex :type Integer))
  ;[1 1 1] Next Tutorial
  (if (Variables|Default|GetTutorialActive)
    (if (not (and (== NextIndex 0) (Variables|Default|GetBeginningTutorialDone)))
      (if (Utilities|IsValid (.Audio (Utilities|Struct|BreakTutorialData (Utilities|Array|Get(acopy) (Variables|Default|GetDialogue_Audio) (Variables|Default|GetCurrent_Index)))))
        (switch int NextIndex
          (:-1
            (Variables|Default|SetCurrent_Index (.HelpRequiredIndex (Utilities|Struct|BreakTutorialData (Utilities|Array|Get(acopy) (Variables|Default|GetDialogue_Audio) (Variables|Default|GetCurrent_Index))))))
          (:0
            (Variables|Default|SetCurrent_Index (.CompletedTaskIndex (Utilities|Struct|BreakTutorialData (Utilities|Array|Get(acopy) (Variables|Default|GetDialogue_Audio) (Variables|Default|GetCurrent_Index)))) :!label _label))
          (:1
            (goto _label)))
        (CallFunction|PlayAudio)))))

(event Custom|ResetTutorial
  ;[1 1 1] Reset tutorial
  (Variables|Default|SetTutorialActive true)
  (Variables|Default|SetCurrent_Index 0))

(event Custom|PlayAudio
  (bind _dialogue_audio (Variables|Default|GetDialogue_Audio))
  (bind _levelmanagerref (Variables|Default|GetLevelManagerRef))
  (bind _current_index (Variables|Default|GetCurrent_Index))
  (bind _levelmanagerref_2 (Variables|Default|GetLevelManagerRef))
  (bind _levelmanagerref_3 (Variables|Default|GetLevelManagerRef))
  (bind _levelmanagerref_4 (Variables|Default|GetLevelManagerRef))
  (bind _dialogue_audio_2 (Variables|Default|GetDialogue_Audio))
  (bind _current_index_2 (Variables|Default|GetCurrent_Index))
  (bind _output (Utilities|Array|Get(acopy) _dialogue_audio_2 _current_index_2))
  (bind _output_2 (Utilities|Array|Get(acopy) _dialogue_audio _current_index))
  (bind _playerref (Variables|/Game/Assets/Blueprints/LevelManager.LevelManager_C|GetPlayerRef _levelmanagerref))
  (bind _audio (Variables|/Game/Assets/Blueprints/LevelManager.LevelManager_C|GetAudio _levelmanagerref_3))
  (bind _audio_2 (Variables|/Game/Assets/Blueprints/LevelManager.LevelManager_C|GetAudio _levelmanagerref_4))
  (bind (_audio_3 _hasplayed _delaytimeforhelp _completedtaskindex _helprequiredindex _waitaction _handanimation _animation) (Utilities|Struct|BreakTutorialData _output_2))
  (bind (_audio_4 _hasplayed_2 _delaytimeforhelp_2 _completedtaskindex_2 _helprequiredindex_2 _waitaction_2 _handanimation_2 _animation_2) (Utilities|Struct|BreakTutorialData _output))
  (bind _returnvalue (Utilities|IsValid _audio_3))
  (bind _returnvalue_2 (select _returnvalue _audio_3 0))
  (Utilities|IsValid _audio_3
    (:Is%20Valid
      (Utilities|IsValid _audio_2
        (:Is%20Valid
          (if (not (Audio|Components|Audio|IsPlaying _audio_2))
            (if (not _hasplayed)
              (Variables|Default|SetDelayTimeForHelp _delaytimeforhelp)
              (Utilities|Array|SetArrayElem (Variables|Default|GetDialogue_Audio) (Variables|Default|GetCurrent_Index) (Utilities|Struct|MakeTutorialData _returnvalue_2 true _delaytimeforhelp _completedtaskindex _helprequiredindex _waitaction _handanimation _animation))
              (if _returnvalue
                (Audio|Components|Audio|SetSound _audio _returnvalue_2)
                (CallFunction|SpeachVis)
                (Audio|Components|Audio|Play _audio 0.0))
              (Utilities|FlowControl|Sequence
                (:then_0
                  (if (not (Variables|Default|GetisInTalkingPos))
                    (if (Utilities|Enum|NotEqual(Enum) _waitaction_2 "NewEnumerator5")
                      (bind _return (Default|GetNewSkullLoc (Variables|/Game/Assets/Blueprints/LevelManager.LevelManager_C|GetPlayerRef _levelmanagerref_2) true))
                      (Default|MovetoLocation _levelmanagerref_2 1.0 _return))))
                (:then_1
                  (switch Utilities|FlowControl|Switch|SwitchonTutorialActions _waitaction_2
                    (:NewEnumerator3
                      (if (== (Variables|Default|GetDelayTimeForHelp) -1.0)
                        _
                        (else
                          (bind _return_2 (Default|GetNewSkullLoc _playerref true))))
                      (Default|MovetoLocation _levelmanagerref 1.0 _return_2)
                      (CallFunction|ResetSkullSpawns))
                    (:NewEnumerator4
                      (CallFunction|ResetPortal))
                    (:NewEnumerator7
                      (Default|SpawnWand _playerref))
                    (:NewEnumerator8
                      (Variables|/Game/Assets/Blueprints/PersonalMCPawn.PersonalMCPawn_C|SeteatTrigger _playerref true))
                    (:NewEnumerator9
                      ;[1 1 1] End Level
                      (Utilities|FlowControl|Delay 5.0)
                      (bind _outactors (Actor|GetAllActorsOfClass "/Game/Assets/Blueprints/final_green_light.final_green_light_C"))
                      (for _array_element _outactors
                        (Default|Glow _array_element))
                      (Utilities|FlowControl|Delay 1.0)
                      (bind _outactors_2 (Actor|GetAllActorsOfClass "/Game/Assets/Blueprints/CryptEntryBP.CryptEntryBP_C"))
                      (Utilities|IsValid (Utilities|Array|Get(acopy) _outactors_2)
                        (:Is%20Valid
                          (Components|Animation|PlayAnimation (Variables|/Script/Engine.SkeletalMeshActor|GetSkeletalMeshComponent (Utilities|Array|Get(acopy) _outactors_2)) "/Game/Assets/Art/Crypt/Animation/cryptentrance_animation.cryptentrance_animation" false)
                          (Utilities|FlowControl|Delay 7.0)
                          (Default|DeathOverride (Variables|/Game/Assets/Blueprints/LevelManager.LevelManager_C|GetPlayerRef (Variables|Default|GetLevelManagerRef))))))))
                (:then_2
                  (CallFunction|CheckExtraActions)
                  (Utilities|FlowControl|Delay 4.0)
                  (CallFunction|HandAnimation)
                  (if (and (Utilities|Enum|NotEqual(Enum) _animation_2 "NewEnumerator7") (Utilities|Enum|NotEqual(Enum) _animation_2 "NewEnumerator0"))
                    (Utilities|FlowControl|Delay 8.0)
                    (Default|StopAnimations (Variables|Default|GetAnimHandsRef))))))))))))

(event Custom|CheckExtraActions
  (bind _applethrowcount (Variables|Default|GetAppleThrowCount))
  (bind _levelmanagerref (Variables|Default|GetLevelManagerRef))
  (bind _dialogue_audio (Variables|Default|GetDialogue_Audio))
  (bind _levelmanagerref_2 (Variables|Default|GetLevelManagerRef))
  (bind _delaytimeforhelp (Variables|Default|GetDelayTimeForHelp))
  (bind _current_index (Variables|Default|GetCurrent_Index))
  (bind _returnvalue (<= _delaytimeforhelp 4.0))
  (bind _output (Utilities|Array|Get(acopy) _dialogue_audio _current_index))
  (bind (_audio _hasplayed _delaytimeforhelp_2 _completedtaskindex _helprequiredindex _waitaction _handanimation _animation) (Utilities|Struct|BreakTutorialData _output))
  (if (Utilities|Enum|NotEqual(Enum) _waitaction "NewEnumerator0")
    (switch Utilities|FlowControl|Switch|SwitchonTutorialActions _waitaction
      (:NewEnumerator1
        (if _returnvalue
          (Utilities|FlowControl|DoOnce false
            (:Completed
              (CallFunction|ThrowApple "0,40.000000, 0")))))
      (:NewEnumerator2
        (if _returnvalue
          (Utilities|FlowControl|DoOnce false :!label _label
            (:Completed
              (CallFunction|ThrowApple (Math|Vector|MakeVector 1e+01 (Math|Random|RandomFloatinRange -4e+01 4e+01) (Math|Random|RandomFloatinRange -1e+01 4e+01)))
              (Math|Integer|IncrementInt _applethrowcount
                (:%20%20
                  (Utilities|FlowControl|Delay 0.05)
                  (if (< _applethrowcount 10)
                    (goto _label Reset))))))))
      (:NewEnumerator3
        (Utilities|FlowControl|DoOnce false
          (:Completed
            (Utilities|FlowControl|Sequence
              (:then_0
                (if (Variables|Default|GetBeginningTutorialDone)
                  (Default|SpawnTargetSkulls _levelmanagerref_2)
                  (else
                    (Default|StartEndRound _levelmanagerref_2)))
                (Default|MovetoLocation _levelmanagerref_2 1.0 (Variables|/Game/Assets/Blueprints/LevelManager.LevelManager_C|GetInitalStartLoc _levelmanagerref_2)))
              (:then_1
                (goto _label_2 Reset))))))
      (:NewEnumerator4
        (if (<= (Variables|Default|GetDelayTimeForHelp) 7.0)
          (Utilities|FlowControl|DoOnce false :!label _label_2
            (:Completed
              (bind _return (Default|GetNewSkullLoc (Variables|/Game/Assets/Blueprints/LevelManager.LevelManager_C|GetPlayerRef _levelmanagerref) false))
              (Default|MovetoLocation _levelmanagerref 0.5 _return)
              (Variables|Default|SetisInTalkingPos true)))))
      (:NewEnumerator5
        (if (not (Audio|Components|Audio|IsPlaying (Variables|/Game/Assets/Blueprints/LevelManager.LevelManager_C|GetAudio (Variables|Default|GetLevelManagerRef))))
          (Variables|Default|SetTutorialActive false)
          (Variables|Default|SetBeginningTutorialDone true))))))

(event Custom|StopTimerCountdown
  (Variables|Default|SetDelayTimeForHelp -1.0)
  (Default|StopAnimations (Variables|Default|GetAnimHandsRef)))

(event Custom|speach%20vis
  (bind _dialogue_audio (Variables|Default|GetDialogue_Audio))
  (bind _levelmanagerref (Variables|Default|GetLevelManagerRef))
  (bind _current_index (Variables|Default|GetCurrent_Index))
  (bind _output (Utilities|Array|Get(acopy) _dialogue_audio _current_index))
  (bind _emissivematerial (Variables|/Game/Assets/Blueprints/LevelManager.LevelManager_C|GetEmissiveMaterial _levelmanagerref))
  ;[1 1 1] Audio Recognition
  (bind _returnvalue (Utilities|Time|SetTimerbyEvent (delegate Custom|speach%20vis) 0.05 true))
  (Utilities|IsValid (.audio _output)
    (:Is%20Valid
      (bind _output_get (Variables|Default|Setsound_vis_playtime (+ (Variables|Default|Getsound_vis_playtime) 0.05)))
      (if (>= _output_get (Variables|/Script/Engine.SoundBase|GetDuration (.audio _output)))
        (Utilities|Time|ClearandInvalidateTimerbyHandle _returnvalue)
        (Variables|Default|Setsound_vis_playtime 0.0)
        (Rendering|Material|SetScalarParameterValue _emissivematerial "Emissive Intensity" 1e+02 :!class /Script/Engine.MaterialInstanceDynamic)
        (else
          (bind _outamplitudes (Class|SoundVisualizationStatics|GetAmplitude (.audio _output) 0 _output_get 0.1 1))
          (Variables|Default|SetsoundAmplitude (Utilities|Array|Get(acopy) _outamplitudes))
          (Rendering|Material|SetScalarParameterValue _emissivematerial "Emissive Intensity" (Math|Float|MapRangeClamped (Utilities|Array|Get(acopy) _outamplitudes) 1e+01 1e+02 1e+02 5e+02) :!class /Script/Engine.MaterialInstanceDynamic))))))

(event Custom|HandAnimation
  (bind _levelmanagerref (Variables|Default|GetLevelManagerRef))
  (bind _dialogue_audio (Variables|Default|GetDialogue_Audio))
  (bind _levelmanagerref_2 (Variables|Default|GetLevelManagerRef))
  (bind _animhandsref (Variables|Default|GetAnimHandsRef))
  (bind _current_index (Variables|Default|GetCurrent_Index))
  (bind _output (Utilities|Array|Get(acopy) _dialogue_audio _current_index))
  (bind (_audio _hasplayed _delaytimeforhelp _completedtaskindex _helprequiredindex _waitaction _handanimation _animation) (Utilities|Struct|BreakTutorialData _output))
  ;[1 1 1] Hand Animations
  (switch Utilities|FlowControl|Switch|SwitchonTutorialAnimation _animation
    (:NewEnumerator0
      _)
    (:NewEnumerator1
      (Default|GivePlayerSpells _levelmanagerref 1))
    (:NewEnumerator2
      (Default|GivePlayerSpells _levelmanagerref 2))
    (:NewEnumerator3
      (Default|GivePlayerSpells _levelmanagerref 3)))
  (Variables|Default|SetisInTalkingPos false)
  (Utilities|FlowControl|Delay 2.0)
  (Default|SetHandAnim _animhandsref _animation true false)
  (Default|SetControllerAnim _animhandsref "NewEnumerator4" true false)
  (Utilities|FlowControl|Delay 3.0)
  (Default|MovetoLocation _levelmanagerref_2 1.0 (Variables|/Game/Assets/Blueprints/LevelManager.LevelManager_C|GetInitalStartLoc _levelmanagerref_2)))

(event Custom|ResetPortal
  (bind _levelmanagerref (Variables|Default|GetLevelManagerRef))
  (Utilities|FlowControl|DoOnce false) ; enters at Reset
)

(event EventBeginPlay
  (bind _outactors (Actor|GetAllActorsOfClass "/Game/Assets/Blueprints/LevelManager.LevelManager_C"))
  (bind _output_get (Variables|Default|SetLevelManagerRef (Utilities|Array|Get(acopy) _outactors)))
  (bind _aspersonal_mcpawn (Utilities|Casting|CastToPersonalMCPawn (Game|Player|GetPlayerPawn 0))
    (:then
      (Utilities|FlowControl|Delay 1.0)
      (bind _return (Default|GetNewSkullLoc _aspersonal_mcpawn true))
      (Default|MovetoLocation _output_get 0.2 _return)
      (Variables|Default|SetisInTalkingPos true))
    (:CastFailed
      _))
  (CallFunction|SetUpAudioLengths)
  (bind _outactors_2 (Actor|GetAllActorsOfClass "/Game/Assets/Blueprints/Tutorial_Hands.Tutorial_Hands_C"))
  (Variables|Default|SetAnimHandsRef (Utilities|Array|Get(acopy) _outactors_2))
  (Utilities|FlowControl|Delay 2.0)
  (Variables|Default|SetTutorialActive true)
  (CallFunction|PlayAudio))

(event Collision|EventActorBeginOverlap
  (params (OtherActor :type Actor%20Object%20Reference)))

(event EventTick
  (params (DeltaSeconds :type Float%20%28single-precision%29))
  (if (Variables|Default|GetTutorialActive)
    (if (.hasPlayed (Utilities|Struct|BreakTutorialData (Utilities|Array|Get(acopy) (Variables|Default|GetDialogue_Audio) (Variables|Default|GetCurrent_Index))))
      (CallFunction|CheckExtraActions)
      (if (not (<= (Variables|Default|GetDelayTimeForHelp) -1.0))
        (if (<= (Variables|Default|GetDelayTimeForHelp) 0.0)
          (bind _output_get (Variables|Default|SetCurrent_Index (.HelpRequiredIndex (Utilities|Struct|BreakTutorialData (Utilities|Array|Get(acopy) (Variables|Default|GetDialogue_Audio) (Variables|Default|GetCurrent_Index))))))
          (if (!= _output_get 0)
            _
            (else
              (Variables|Default|SetCurrent_Index (.CompletedTaskIndex (Utilities|Struct|BreakTutorialData (Utilities|Array|Get(acopy) (Variables|Default|GetDialogue_Audio) (Variables|Default|GetCurrent_Index)))))))
          (Utilities|FlowControl|Delay 2.0)
          (CallFunction|PlayAudio)
          (else
            (Variables|Default|SetDelayTimeForHelp (- (Variables|Default|GetDelayTimeForHelp) (Utilities|Time|GetWorldDeltaSeconds))))))
      (else
        (CallFunction|PlayAudio)))))

(fn ConstructionScript)

(fn ThrowApple
  (params (Offset :type Vector))
  (bind _levelmanagerref (Variables|Default|GetLevelManagerRef))
  (bind _returnvalue (Transformation|GetActorForwardVector _levelmanagerref))
  (bind _returnvalue_2 (Transformation|GetActorRightVector _levelmanagerref))
  (bind _returnvalue_3 (Transformation|GetActorUpVector _levelmanagerref))
  (bind _returnvalue_4 (Transformation|GetActorLocation _levelmanagerref))
  (bind _returnvalue_5 (* _returnvalue (.x Offset)))
  (bind _returnvalue_6 (* _returnvalue_3 (.z Offset)))
  (bind _returnvalue_7 (* _returnvalue_2 (.y Offset)))
  (bind _returnvalue_8 (+ _returnvalue_5 _returnvalue_7 _returnvalue_6 _returnvalue_4))
  (Effects|SpawnEmitteratLocation "/Game/Assets/Particles/Objects/apple_poof.apple_poof" _returnvalue_8)
  (bind _returnvalue_9 (Game|SpawnActorfromClass "/Game/Assets/Blueprints/Objects/Apple_Heal_object.Apple_Heal_object_C" (Math|Transform|MakeTransform _returnvalue_8 "0, 0, 0" "1,1,1") "Undefined" 0 0))
  (Default|FlyatPlayer _returnvalue_9 1e+03))

(fn SetUpAudioLengths
  (bind _dialogue_audio (Variables|Default|GetDialogue_Audio))
  (for _index (range 0 (- (Utilities|Array|Length _dialogue_audio) 1))
    (if (!= (.DelayTimeForHelp (Utilities|Struct|BreakTutorialData (Utilities|Array|Get(acopy) _dialogue_audio _index))) -1.0)
      (Utilities|Array|SetArrayElem (Variables|Default|GetDialogue_Audio) _index (Utilities|Struct|MakeTutorialData (select (Utilities|IsValid (.Audio (Utilities|Struct|BreakTutorialData (Utilities|Array|Get(acopy) _dialogue_audio _index)))) (.Audio (Utilities|Struct|BreakTutorialData (Utilities|Array|Get(acopy) _dialogue_audio _index))) 0) (.hasPlayed (Utilities|Struct|BreakTutorialData (Utilities|Array|Get(acopy) _dialogue_audio _index))) (+ (Variables|/Script/Engine.SoundBase|GetDuration (.Audio (Utilities|Struct|BreakTutorialData (Utilities|Array|Get(acopy) _dialogue_audio _index)))) (.DelayTimeForHelp (Utilities|Struct|BreakTutorialData (Utilities|Array|Get(acopy) _dialogue_audio _index)))) (.CompletedTaskIndex (Utilities|Struct|BreakTutorialData (Utilities|Array|Get(acopy) _dialogue_audio _index))) (.HelpRequiredIndex (Utilities|Struct|BreakTutorialData (Utilities|Array|Get(acopy) _dialogue_audio _index))) (.WaitAction (Utilities|Struct|BreakTutorialData (Utilities|Array|Get(acopy) _dialogue_audio _index))) (.HandAnimation (Utilities|Struct|BreakTutorialData (Utilities|Array|Get(acopy) _dialogue_audio _index))) (.Animation (Utilities|Struct|BreakTutorialData (Utilities|Array|Get(acopy) _dialogue_audio _index))))))))