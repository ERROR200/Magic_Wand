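; Speedy skeleton enemy that accelerates while it has line of sight to the player, then makes a charged jump.
; StatusEffect searches for the player without sight; otherwise a Speedup timeline ramps speed through UpdateSpeed.
; When the timeline finishes, a short random delay sets Charge and calls ChargeJump.
; ChargeJump calls Launch after a brief pause if the player is within the horizontal jump range, with Jumped blocking repeats from StatusEffect.
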(event Custom|ChargeJump
  (bind _returnvalue (Game|Player|GetPlayerPawn 0))
  (bind _self self)
  (bind _returnvalue_2 (Transformation|GetHorizontalDistanceTo _returnvalue _self))
  (if (and (<= _returnvalue_2 (Variables|Default|GetmaxJumpDist)) (>= _returnvalue_2 (Variables|Default|GetminJumpDist)))
    (Variables|Default|SetJumped true)
    (Utilities|FlowControl|Delay 0.2)
    (CallFunction|Launch)))

(event EventBeginPlay
  (|CallParentFunction) ; This node is disabled and will not be called.\nDrag off pins to build functionality.
)

(event Collision|EventActorBeginOverlap
  (params (OtherActor :type Actor%20Object%20Reference))
  (|CallParentFunction OtherActor) ; This node is disabled and will not be called.\nDrag off pins to build functionality.
)

(event EventStatusEffect
  (if (Variables|Default|GetHasDirectLineOfSight)
    (if (Variables|Default|GetCharge)
      (if (not (Variables|Default|GetJumped))
        (CallFunction|ChargeJump))
      (else
        (bind _timer (Timeline|Speedup Play)
          (:Update
            (CallFunction|UpdateSpeed (Math|Float|Lerp 1.8 7.8 _timer)))
          (:Finished
            (Utilities|FlowControl|Delay (Math|Random|RandomFloatinRange 0.5 1.0))
            (Variables|Default|SetCharge true)
            (CallFunction|ChargeJump)))))
    (else
      (CallFunction|SearchforPlayer))))

(event EventTick
  (params (DeltaSeconds :type Float%20%28single-precision%29))
  (|CallParentFunction DeltaSeconds) ; This node is disabled and will not be called.\nDrag off pins to build functionality.
)

(fn ConstructionScript)