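; Wilfred is a talking wizard skull that voices scripted lines and random combat banter, and reports motion-controller grabs to its parent LevelManager.
; SetAudio starts each line and a timer that samples sound wave amplitude to pulse the skull's emissive material.
; SetExpression blends four facial morph targets on a timeline, with MultiGates stepping through preset expression sequences.
; Hit counters and a Tick countdown trigger seeded-random combat remarks when he is not talking.
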(event OnComponentBeginOverlap(WizardSkull_Rigged)
  (params (OverlappedComponent :type Primitive%20Component%20Object%20Reference) (OtherActor :type Actor%20Object%20Reference) (OtherComp :type Primitive%20Component%20Object%20Reference) (OtherBodyIndex :type Integer) (bFromSweep :type Boolean) (SweepResult :type Hit%20Result%20Structure%20%28by%20ref%29))
  (bind _levelmanagerref (Variables|Default|GetLevelManagerRef))
  (Utilities|IsValid _levelmanagerref
    (:Is%20Valid
      (bind _asbp_motion_controller (Utilities|Casting|CastToBP_MotionController OtherActor))
      (Variables|/Game/Assets/Blueprints/LevelManager.LevelManager_C|SetHandGrabRef _levelmanagerref _asbp_motion_controller))))

(event OnComponentEndOverlap(WizardSkull_Rigged)
  (params (OverlappedComponent :type Primitive%20Component%20Object%20Reference) (OtherActor :type Actor%20Object%20Reference) (OtherComp :type Primitive%20Component%20Object%20Reference) (OtherBodyIndex :type Integer))
  (bind _levelmanagerref (Variables|Default|GetLevelManagerRef))
  (Utilities|IsValid _levelmanagerref
    (:Is%20Valid
      (Variables|/Game/Assets/Blueprints/LevelManager.LevelManager_C|SetHandGrabRef _levelmanagerref 0))))

(event Custom|TutorialEnd
  (CallFunction|SetAudio "/Game/Assets/Sounds/DemoTutorial/DemoTutorial_06_Cue.DemoTutorial_06_Cue" "/Game/Assets/Sounds/DemoTutorial/DemoTutorial_06.DemoTutorial_06")
  (Utilities|FlowControl|Delay (+ (Variables|/Script/Engine.SoundBase|GetDuration (Variables|Default|GetActiveAudio)) 3.0))
  (Default|DeathOverride (Variables|/Game/Assets/Blueprints/LevelManager.LevelManager_C|GetPlayerRef (Variables|Default|GetLevelManagerRef))))

(event Custom|End_Lines
  (CallFunction|SetAudio "/Game/Assets/Sounds/Boss_Lines/BossBattle_19_Cue.BossBattle_19_Cue" "/Game/Assets/Sounds/Boss_Lines/BossBattle_19.BossBattle_19"))

(event Custom|SetAudio
  (params (Audio :type Sound%20Cue%20Object%20Reference) (AudioWaveRef :type Sound%20Wave%20Object%20Reference))
  (bind _output_get (Variables|Default|SetActiveAudio Audio))
  (Variables|Default|SetActiveSoundWave AudioWaveRef)
  (Audio|Components|Audio|SetSound (Variables|Default|GetAudio) _output_get)
  (Audio|Components|Audio|Play (Variables|Default|GetAudio) 0.0)
  (CallFunction|SpeechVis)
  (Variables|Default|SetisTalking true)
  (Variables|Default|SetcommentTimer 0.0))

(event Custom|SetExpression
  (params (Expression :type Facial%20Expression%20Structure))
  (bind (_happy_value _angry_value _sad_value _shocked_value) (Utilities|Struct|BreakFacialExpression Expression))
  (bind (_happy_value_2 _angry_value_2 _sad_value_2 _shocked_value_2 _time_delay _blend_time _reset_on_line_finished _reset_time) (Utilities|Struct|BreakFacialExpression Expression))
  (Variables|Default|SetResetExpression _reset_on_line_finished)
  (Variables|Default|SetFacialExpressionResetTime _reset_time)
  (Utilities|FlowControl|Delay _time_delay)
  (Components|Timeline|SetPlayRate (Variables|Default|GetChangeExpression) _blend_time)
  (bind _time (Timeline|ChangeExpression PlayFromStart)
    (:Update
      (CallFunction|SetHappyExpression (Math|Float|Lerp (.happy_value (Variables|Default|GetOldExpression)) _happy_value _time))
      (CallFunction|SetSadExpression (Math|Float|Lerp (.sad_value (Variables|Default|GetOldExpression)) _sad_value _time))
      (CallFunction|SetShockedExpression (Math|Float|Lerp (.shocked_value (Variables|Default|GetOldExpression)) _shocked_value _time))
      (CallFunction|SetMadExpression (Math|Float|Lerp (.angry_value (Variables|Default|GetOldExpression)) _angry_value _time)))
    (:Finished
      (Variables|Default|SetOldExpression Expression))))

(event Custom|Speech%20Vis
  (bind _emissivematerial (Variables|Default|GetEmissiveMaterial))
  (bind _activeaudio (Variables|Default|GetActiveAudio))
  ;[1 1 1] Audio Recognition
  (bind _returnvalue (Utilities|Time|SetTimerbyEvent (delegate Custom|Speech%20Vis) 0.05 true))
  (Utilities|IsValid _activeaudio
    (:Is%20Valid
      (bind _output_get (Variables|Default|Setsound_vis_playtime (+ (Variables|Default|Getsound_vis_playtime) 0.05)))
      (if (>= _output_get (Variables|/Script/Engine.SoundBase|GetDuration _activeaudio))
        (Utilities|Time|ClearandInvalidateTimerbyHandle _returnvalue)
        (Variables|Default|Setsound_vis_playtime 0.5)
        (Variables|Default|SetsoundAmplitude 0.0)
        (Rendering|Material|SetScalarParameterValue _emissivematerial "Emissive Intensity" 1e+02 :!class /Script/Engine.MaterialInstanceDynamic)
        (Variables|Default|SetisTalking false)
        (Audio|Components|Audio|SetVolumeMultiplier (Variables|Default|GetAudio) (Variables|Default|GetvolumeMultiplier) :!class /Script/Engine.AudioComponent)
        (if (Variables|Default|GetResetExpression)
          (Variables|Default|SetResetExpression false)
          (CallFunction|SetExpression (Utilities|Struct|MakeFacialExpression 0.0 0.0 0.0 0.0 0.0 (Variables|Default|GetFacialExpressionResetTime) false 1.0)))
        (else
          (bind _outamplitudes (Class|SoundVisualizationStatics|GetAmplitude (Variables|Default|GetActiveSoundWave) 0 _output_get 0.1 1))
          (Variables|Default|SetsoundAmplitude (Utilities|Array|Get(acopy) _outamplitudes))
          (Rendering|Material|SetScalarParameterValue _emissivematerial "Emissive Intensity" (Math|Float|MapRangeClamped (Utilities|Array|Get(acopy) _outamplitudes) 1e+01 1e+02 1e+02 5e+02) :!class /Script/Engine.MaterialInstanceDynamic))))))

(event Custom|BossExpressions
  (Utilities|FlowControl|MultiGate false false -1
    (:Out%200
      (CallFunction|SetExpression (Utilities|Struct|MakeFacialExpression 0.0 1.0 0.0 1.0 0.0 1.0 false 1.0)))
    (:Out%201
      (CallFunction|SetExpression (Utilities|Struct|MakeFacialExpression 0.5 -0.75 0.0 0.0 0.0 1.0 false 1.0)))
    (:Out%202
      (CallFunction|SetExpression (Utilities|Struct|MakeFacialExpression 0.0 0.0 0.8 1.0 0.0 1.0 false 1.0)))
    (:Out%203
      (CallFunction|SetExpression (Utilities|Struct|MakeFacialExpression 0.0 1.0 0.75 0.0 0.0 1.0 false 1.0)))
    (:Out%204
      (CallFunction|SetExpression (Utilities|Struct|MakeFacialExpression 0.0 1.0 0.0 0.35 0.0 1.0 false 1.0)))
    (:Out%205
      (CallFunction|SetExpression (Utilities|Struct|MakeFacialExpression 0.0 1.0 0.0 1.0 0.0 1.0 false 1.0)))
    (:Out%206
      (CallFunction|SetExpression (Utilities|Struct|MakeFacialExpression 1.0 1.0 0.0 0.25 0.0 1.0 false 1.0)))
    (:Out%207
      (CallFunction|SetExpression (Utilities|Struct|MakeFacialExpression 0.0 0.0 0.0 0.9 0.0 1.0 false 1.0)))
    (:Out%208
      (CallFunction|SetExpression (Utilities|Struct|MakeFacialExpression 0.5 0.5 0.0 -0.2 0.0 1.0 false 1.0)))
    (:Out%209
      (CallFunction|SetExpression (Utilities|Struct|MakeFacialExpression 0.0 1.0 0.0 0.25 0.0 1.0 false 1.0)))
    (:Out%2010
      (CallFunction|SetExpression (Utilities|Struct|MakeFacialExpression 0.0 0.25 0.25 0.1 0.0 1.0 false 1.0)))
    (:Out%2011
      (CallFunction|SetExpression (Utilities|Struct|MakeFacialExpression 0.0 1.0 0.0 0.0 0.0 1.0 false 1.0)))
    (:Out%2012
      (CallFunction|SetExpression (Utilities|Struct|MakeFacialExpression -0.9 0.1 -0.1 1.0 0.0 1.0 false 1.0)))
    (:Out%2013
      (CallFunction|SetExpression (Utilities|Struct|MakeFacialExpression -0.25 1.0 0.0 1.0 0.0 1.0 false 1.0)))))

(event Custom|SwapExpression
  (Utilities|FlowControl|MultiGate false false -1
    (:Out%200
      (CallFunction|SetExpression (Utilities|Struct|MakeFacialExpression 0.0 0.0 0.0 1.0 0.0 1.0 false 1.0)))
    (:Out%201
      (CallFunction|SetExpression (Utilities|Struct|MakeFacialExpression 0.3 0.25 0.0 -0.5 0.0 1.0 false 1.0)))
    (:Out%202
      (CallFunction|SetExpression (Utilities|Struct|MakeFacialExpression 1.0 0.0 0.35 0.25 0.0 1.0 false 1.0)))
    (:Out%203
      (CallFunction|SetExpression (Utilities|Struct|MakeFacialExpression 0.0 0.0 0.0 0.8 0.0 1.0 false 1.0)))
    (:Out%204
      (CallFunction|SetExpression (Utilities|Struct|MakeFacialExpression 1.0 0.0 0.0 -0.3 0.0 1.0 false 1.0)))
    (:Out%205
      (CallFunction|SetExpression (Utilities|Struct|MakeFacialExpression 1.0 0.0 0.0 0.5 0.0 1.0 false 1.0)))
    (:Out%206
      (CallFunction|SetExpression (Utilities|Struct|MakeFacialExpression 0.4 0.0 0.0 0.0 0.0 1.0 false 1.0)))
    (:Out%207
      (CallFunction|SetExpression (Utilities|Struct|MakeFacialExpression 0.0 0.0 0.0 0.0 0.0 1.0 false 1.0)))
    (:Out%208
      (CallFunction|SetExpression (Utilities|Struct|MakeFacialExpression 1.0 -0.3 0.5 0.4 0.0 1.0 false 1.0)))
    (:Out%209
      (CallFunction|SetExpression (Utilities|Struct|MakeFacialExpression 1.0 0.5 0.25 0.0 0.0 1.0 false 1.0)))
    (:Out%2010
      (CallFunction|SetExpression (Utilities|Struct|MakeFacialExpression 0.0 0.0 0.0 0.8 0.0 1.0 false 1.0)))
    (:Out%2011
      (CallFunction|SetExpression (Utilities|Struct|MakeFacialExpression 1.0 0.0 0.0 0.8 0.0 1.0 false 1.0)))
    (:Out%2012
      (CallFunction|SetExpression (Utilities|Struct|MakeFacialExpression 1.0 0.0 0.0 0.5 0.0 1.0 false 1.0)))
    (:Out%2013
      (CallFunction|SetExpression (Utilities|Struct|MakeFacialExpression 0.5 0.5 -0.5 -0.25 0.0 1.0 false 1.0)))
    (:Out%2014
      (CallFunction|SetExpression (Utilities|Struct|MakeFacialExpression 0.0 0.8 0.0 0.0 0.0 1.0 false 1.0)))
    (:Out%2015
      (CallFunction|SetExpression (Utilities|Struct|MakeFacialExpression 0.5 0.0 0.75 0.5 0.0 1.0 false 1.0)))
    (:Out%2016
      (CallFunction|SetExpression (Utilities|Struct|MakeFacialExpression 0.5 0.0 0.0 1.0 0.0 1.0 false 1.0)))
    (:Out%2017
      (CallFunction|SetExpression (Utilities|Struct|MakeFacialExpression 0.0 0.0 0.5 0.5 0.0 1.0 false 1.0)))
    (:Out%2018
      (CallFunction|SetExpression (Utilities|Struct|MakeFacialExpression 1.0 0.0 0.5 0.0 0.0 1.0 false 1.0)))
    (:Out%2019
      (CallFunction|SetExpression (Utilities|Struct|MakeFacialExpression 1.0 0.0 0.0 0.25 0.0 1.0 false 1.0)))
    (:Out%2020
      (CallFunction|SetExpression (Utilities|Struct|MakeFacialExpression 0.6 0.75 0.25 0.4 0.0 1.0 false 1.0)))
    (:Out%2021
      (CallFunction|SetExpression (Utilities|Struct|MakeFacialExpression 1.0 0.0 0.0 0.2 0.0 1.0 false 1.0)))))

(event EventBeginPlay
  (Class|KismetMathLibrary|SeedRandomStream (Variables|Default|GetRandom))
  (bind _aslevel_manager (Utilities|Casting|CastToLevelManager (Actor|GetParentActor))
    (:then
      (Variables|Default|SetLevelManagerRef _aslevel_manager)
      (Rendering|Material|SetScalarParameterValue (Variables|Default|GetEmissiveMaterial) "Emissive Intensity" 1e+02 :!class /Script/Engine.MaterialInstanceDynamic)
      (if (Utilities|Enum|Equal(Enum) (stale _returnvalue) "EndScene_Level") :!label _label
        (Audio|Components|Audio|SetVolumeMultiplier (Variables|Default|GetAudio) 1e+01 :!class /Script/Engine.AudioComponent))
      (Variables|Default|SetvolumeMultiplier (Variables|/Script/Engine.AudioComponent|GetVolumeMultiplier (Variables|Default|GetAudio))))
    (:CastFailed
      (bind _returnvalue (Game|GetCurrentLevelName true))
      (if (Utilities|Enum|Equal(Enum) _returnvalue "Crypt_level")
        (Audio|Components|Audio|SetVolumeMultiplier (Variables|Default|GetAudio) 8.0 :!class /Script/Engine.AudioComponent)
        (else
          (goto _label))))))

(event Collision|EventActorBeginOverlap
  (params (OtherActor :type Actor%20Object%20Reference)))

(event EventPickup
  (params (AttachTo :type Scene%20Component%20Object%20Reference) (hand :type EControllerHand%20Enum :default "Left"))
  (bind _levelmanagerref (Variables|Default|GetLevelManagerRef))
  (Utilities|IsValid _levelmanagerref
    (:Is%20Valid
      (Default|SkullGrabbed _levelmanagerref))))

(event EventTick
  (params (DeltaSeconds :type Float%20%28single-precision%29))
  (if (> (Variables|Default|GetcommentTimer) 0.0)
    (Variables|Default|SetcommentTimer (- (Variables|Default|GetcommentTimer) DeltaSeconds))
    (else
      (CallFunction|GetRandomConversation))))

(fn ConstructionScript
  (bind _wizardskull_rigged (Variables|Default|GetWizardSkull_Rigged))
  (bind _returnvalue (Rendering|Material|CreateDynamicMaterialInstance _wizardskull_rigged 0 (Rendering|Material|GetMaterial _wizardskull_rigged 0) :!class /Script/Engine.PrimitiveComponent))
  (Variables|Default|SetEmissiveMaterial _returnvalue))

(fn SetHappyExpression
  (params (Value :type Float%20%28single-precision%29))
  (Components|SkeletalMesh|SetMorphTarget (Variables|Default|GetWizardSkull_Rigged) "WizardSkull_Happy" Value true))

(fn SetShockedExpression
  (params (Value :type Float%20%28single-precision%29))
  (Components|SkeletalMesh|SetMorphTarget (Variables|Default|GetWizardSkull_Rigged) "WizardSkull_Shocked" Value true))

(fn SetSadExpression
  (params (Value :type Float%20%28single-precision%29))
  (Components|SkeletalMesh|SetMorphTarget (Variables|Default|GetWizardSkull_Rigged) "WizardSkull_Sad" Value true))

(fn SetMadExpression
  (params (Value :type Float%20%28single-precision%29))
  (Components|SkeletalMesh|SetMorphTarget (Variables|Default|GetWizardSkull_Rigged) "WizardSkull_Frown" Value true))

(fn GetEnemyHitReation
  (bind _enemyhitreactions_audioref (Variables|Default|GetEnemyHitReactions_audioRef))
  (bind _random (Variables|Default|GetRandom))
  (bind _returnvalue (Utilities|Array|Length _enemyhitreactions_audioref))
  (bind _returnvalue_2 (Math|Random|RandomIntegerinRangefromStream 0 _returnvalue _random))
  (Math|Integer|IncrementInt (Variables|Default|GetenemyHitCounter)
    (:%20%20
      (if (>= (Variables|Default|GetenemyHitCounter) (Variables|Default|GetenemyMaxCounter))
        (if (Variables|Default|GetisInCombat)
          (if (not (Variables|Default|GetisTalking))
            (Audio|Components|Audio|SetVolumeMultiplier (Variables|Default|GetAudio) (Variables|Default|GetcasualVolumeMultiplier) :!class /Script/Engine.AudioComponent)
            (CallFunction|SetAudio (Utilities|Array|Get(acopy) (Variables|Default|GetEnemyHitReactions) _returnvalue_2) (Utilities|Array|Get(acopy) _enemyhitreactions_audioref _returnvalue_2))
            (Variables|Default|SetenemyHitCounter 0)
            (else
              (Variables|Default|SetenemyHitCounter (- (Variables|Default|GetenemyHitCounter) (Math|Random|RandomIntegerinRangefromStream 3 7 _random)) :!label _label)))
          (else
            (goto _label)))))))

(fn GetPlayerHitReation
  (bind _random (Variables|Default|GetRandom))
  (bind _playerhitreactions_audioref (Variables|Default|GetPlayerHitReactions_audioRef))
  (bind _returnvalue (Utilities|Array|Length _playerhitreactions_audioref))
  (bind _returnvalue_2 (Math|Random|RandomIntegerinRangefromStream 0 _returnvalue _random))
  (Math|Integer|IncrementInt (Variables|Default|GetplayerHitCounter)
    (:%20%20
      (if (>= (Variables|Default|GetplayerHitCounter) (Variables|Default|GetplayerMaxCounter))
        (if (Variables|Default|GetisInCombat)
          (if (not (Variables|Default|GetisTalking))
            (Audio|Components|Audio|SetVolumeMultiplier (Variables|Default|GetAudio) (Variables|Default|GetcasualVolumeMultiplier) :!class /Script/Engine.AudioComponent)
            (CallFunction|SetAudio (Utilities|Array|Get(acopy) (Variables|Default|GetPlayerHitReactions) _returnvalue_2) (Utilities|Array|Get(acopy) _playerhitreactions_audioref _returnvalue_2))
            (Variables|Default|SetplayerHitCounter 0)
            (else
              (Variables|Default|SetplayerHitCounter (- (Variables|Default|GetplayerHitCounter) 1) :!label _label)))
          (else
            (goto _label)))))))

(fn GetRandomConversation
  (bind _randomconversation_audioref (Variables|Default|GetRandomConversation_audioRef))
  (bind _random (Variables|Default|GetRandom))
  (bind _returnvalue (Utilities|Array|Length _randomconversation_audioref))
  (bind _returnvalue_2 (Math|Random|RandomIntegerinRangefromStream 0 _returnvalue _random))
  (if (and (Variables|Default|GetisInCombat) (not (Variables|Default|GetisTalking)))
    (Audio|Components|Audio|SetVolumeMultiplier (Variables|Default|GetAudio) (Variables|Default|GetcasualVolumeMultiplier) :!class /Script/Engine.AudioComponent)
    (CallFunction|SetAudio (Utilities|Array|Get(acopy) (Variables|Default|GetRandomConversation) _returnvalue_2) (Utilities|Array|Get(acopy) _randomconversation_audioref _returnvalue_2)))
  (Variables|Default|SetcommentTimer (Variables|Default|GetcommentWaitTime)))