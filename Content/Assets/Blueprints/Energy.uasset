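; Energy orb actor that shows its point value on a widget and flies to a collector to award energy.
; On BeginPlay it targets the first LevelManager, falling back to Wilfred, then after a short delay a timeline lerps it toward the target's live position.
; On arrival it calls EnergyAdded or Wilfred's AddEnergy with points and multiplier, then hides and destroys itself.
; Tick turns the widget toward the player pawn.
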(event EventBeginPlay
  (bind _asenergy_widget (Utilities|Casting|CastToenergy_widget (UserInterface|GetUserWidgetObject (Variables|Default|GetWidget))))
  (Variables|Default|Setenergy%20widget _asenergy_widget)
  (bind _outactors (Actor|GetAllActorsOfClass "/Game/Assets/Blueprints/LevelManager.LevelManager_C"))
  (Utilities|IsValid (Utilities|Array|Get(acopy) _outactors)
    (:Is%20Valid
      (Variables|Default|SetTarget (Utilities|Array|Get(acopy) _outactors))
      (Variables|Default|Setstart_location (Transformation|GetActorLocation) :!label _label))
    (:Is%20Not%20Valid
      (bind _outactors_2 (Actor|GetAllActorsOfClass "/Game/Assets/Blueprints/Wilfred.Wilfred_C"))
      (Utilities|IsValid (Utilities|Array|Get(acopy) _outactors_2)
        (:Is%20Valid
          (Variables|Default|SetTarget (Utilities|Array|Get(acopy) _outactors_2))
          (goto _label))
        (:Is%20Not%20Valid
          _))))
  (Default|UpdateScore (Variables|Default|Getenergy%20widget) (Variables|Default|Getpoints))
  (Utilities|FlowControl|Delay 1.0)
  (bind _lerpline (Timeline|Timeline_0 Play)
    (:Update
      (Utilities|IsValid (Variables|Default|GetTarget)
        (:Is%20Valid
          (Transformation|SetActorLocation (Math|Vector|Lerp(Vector) (Variables|Default|Getstart_location) (Transformation|GetActorLocation (Variables|Default|GetTarget)) _lerpline) false false))))
    (:Finished
      (Utilities|IsValid (Utilities|Array|Get(acopy) _outactors)
        (:Is%20Valid
          (Default|EnergyAdded (Utilities|Array|Get(acopy) _outactors)))
        (:Is%20Not%20Valid
          (Utilities|IsValid (Utilities|Array|Get(acopy) _outactors_2)
            (:Is%20Valid
              (Default|AddEnergy (Utilities|Array|Get(acopy) _outactors_2) (Variables|Default|Getpoints) (Variables|Default|Getmultiplier)))
            (:Is%20Not%20Valid
              _))))
      (Components|Activation|Deactivate (Variables|Default|GetEnergy_point))
      (Development|SetHiddeninGame (Variables|Default|GetWidget) true false)
      (Utilities|FlowControl|Delay 1.0)
      (Actor|DestroyActor))))

(event EventTick
  (params (DeltaSeconds :type Float%20%28single-precision%29))
  (bind _widget (Variables|Default|GetWidget))
  (Transformation|SetWorldRotation _widget (Math|Rotator|FindLookatRotation (Transformation|GetWorldLocation _widget) (Transformation|GetActorLocation (Game|Player|GetPlayerPawn 0))) false false))

(fn ConstructionScript)