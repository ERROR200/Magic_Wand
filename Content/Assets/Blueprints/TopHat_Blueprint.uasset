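; Top hat actor that gets knocked off and sent flying the first time it takes damage.
; On TakeDamage, a DoOnce gate enables physics simulation on the static mesh, then waits a brief delay before applying an impulse.
; The impulse points away from the hit location through the scene component's position, with a strong upward boost added.
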(event EventBeginPlay)

(event Collision|EventActorBeginOverlap
  (params (OtherActor :type Actor%20Object%20Reference)))

(event EventTick
  (params (DeltaSeconds :type Float%20%28single-precision%29)))

(event EventTakeDamage
  (params (DamageAmount :type Float%20%28single-precision%29) (Constant :type Boolean) (Effect :type Effects%20Enum :default "NewEnumerator4") (EffectTime :type Float%20%28single-precision%29) (Hit_Location :type Vector :default "0, 0, 0"))
  (bind _scene (Variables|Default|GetScene))
  (bind _returnvalue (Transformation|GetWorldLocation _scene))
  (bind _returnvalue_2 (Math|Rotator|FindLookatRotation Hit_Location _returnvalue))
  (bind _returnvalue_3 (Math|Vector|GetForwardVector _returnvalue_2))
  (bind _returnvalue_4 (* _returnvalue_3 1e+04))
  (Utilities|FlowControl|DoOnce false
    (:Completed
      (Physics|SetSimulatePhysics (Variables|Debug|GetStaticMeshComponent) true)
      (Utilities|FlowControl|Delay 0.05)
      (Physics|AddImpulse (Variables|Debug|GetStaticMeshComponent) (Math|Vector|MakeVector (.x _returnvalue_4) (.y _returnvalue_4) (+ (.z _returnvalue_4) 3e+04)) "None" false))))

(fn ConstructionScript)