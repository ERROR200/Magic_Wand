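; Heal_object is a VR motion-controller pickup, apparently an edible apple, that scales in via a timeline on spawn.
; Pickup disables physics and snaps it to the controller, while Drop restores physics and boosts its velocity for throwing.
; Chomp and Change activate the AppleEat effect, with Change also swapping to the eaten mesh.
; Despite its name, any component hit sends a damage message to the other actor and starts a timed self-destruct.
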(event OnComponentHit(StaticMeshComponent)
  (params (HitComponent :type Primitive%20Component%20Object%20Reference) (OtherActor :type Actor%20Object%20Reference) (OtherComp :type Primitive%20Component%20Object%20Reference) (NormalImpulse :type Vector :default "0, 0, 0") (Hit :type Hit%20Result%20Structure%20%28by%20ref%29))
  (Actor|SetLifeSpan 1e+01)
  (Class|IDamage|TakeDamage(Message) OtherActor 0.5 false "NewEnumerator4" 0.2 (.location Hit)))

(event EventBeginPlay
  (bind _size (Timeline|Timeline_0 Play)
    (:Update
      (Transformation|SetActorScale3D (Math|Conversions|ToVector(Float) _size)))))

(event Collision|EventActorBeginOverlap
  (params (OtherActor :type Actor%20Object%20Reference)))

(event EventChange
  (Components|StaticMesh|SetStaticMesh (Variables|Debug|GetStaticMeshComponent) (Variables|Default|GetEatenMesh))
  (Components|Activation|Activate (Variables|Default|GetApple_eat) false))

(event EventChomp
  (Components|Activation|Activate (Variables|Default|GetApple_eat) true))

(event EventTick
  (params (DeltaSeconds :type Float%20%28single-precision%29)))

(event EventPickup
  (params (AttachTo :type Scene%20Component%20Object%20Reference) (hand :type EControllerHand%20Enum :default "Left"))
  (Physics|SetSimulatePhysics (Variables|Debug|GetStaticMeshComponent) false)
  (Transformation|AttachComponentToComponent (VehicleSound|GetRootComponent) AttachTo "None" "SnapToTarget" "SnapToTarget" "KeepWorld" false))

(event EventDrop
  (params (hand :type EControllerHand%20Enum :default "Left"))
  (bind _staticmeshcomponent (Variables|Debug|GetStaticMeshComponent))
  (Physics|SetSimulatePhysics (Variables|Debug|GetStaticMeshComponent) true)
  (Transformation|DetachFromActor "KeepWorld" "KeepWorld" "KeepWorld")
  (bind _returnvalue (Physics|GetPhysicsLinearVelocity _staticmeshcomponent "None"))
  (Physics|SetPhysicsLinearVelocity _staticmeshcomponent (* _returnvalue 1.5) false "None"))

(fn ConstructionScript)