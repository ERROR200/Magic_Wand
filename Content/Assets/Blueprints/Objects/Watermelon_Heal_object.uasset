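; VR watermelon object that motion controllers can pick up as a "HEALING"-tagged item, and that can also be launched at the player.
; Pickup disables physics and attaches it to the hand; FlyAtPlayer clears CanEat, then after a short delay launches it toward the player's camera.
; On overlap, a non-edible melon damages the player pawn once.
; That hit, or any edible overlap, starts a despawn timer and sends damage to non-Shield actors.
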(event OnComponentBeginOverlap(StaticMeshComponent)
  (params (OverlappedComponent :type Primitive%20Component%20Object%20Reference) (OtherActor :type Actor%20Object%20Reference) (OtherComp :type Primitive%20Component%20Object%20Reference) (OtherBodyIndex :type Integer) (bFromSweep :type Boolean) (SweepResult :type Hit%20Result%20Structure%20%28by%20ref%29))
  (if (Variables|Default|GetcanEat)
    _
    (else
      (bind _aspersonal_mcpawn (Utilities|Casting|CastToPersonalMCPawn OtherActor))
      (Utilities|FlowControl|DoOnce false
        (:Completed
          (Default|ReceiveDamage _aspersonal_mcpawn)))))
  (Actor|SetLifeSpan 1e+01)
  (Utilities|Casting|CastToShield OtherActor
    (:CastFailed
      (Class|IDamage|TakeDamage(Message) OtherActor 0.5 false "NewEnumerator4" 0.2 (Transformation|GetActorLocation OtherActor)))))

(event Custom|FlyAtPlayer
  (params (ThrowSpeed :type Float%20%28single-precision%29))
  (Variables|Default|SetcanEat false)
  (Utilities|FlowControl|Delay 0.2)
  (Physics|SetSimulatePhysics (Variables|Default|GetStaticMeshComponent) true)
  (bind _aspersonal_mcpawn (Utilities|Casting|CastToPersonalMCPawn (Game|Player|GetPlayerPawn 0)))
  (Physics|SetPhysicsLinearVelocity (Variables|Default|GetStaticMeshComponent) (* (Math|Vector|Normalize (- (Transformation|GetWorldLocation (Variables|/Game/Assets/Blueprints/PersonalMCPawn.PersonalMCPawn_C|GetCamera _aspersonal_mcpawn)) (Transformation|GetActorLocation))) ThrowSpeed) false "None"))

(event EventBeginPlay
  (|CallParentFunction))

(event Collision|EventActorBeginOverlap
  (params (OtherActor :type Actor%20Object%20Reference)))

(event EventTick
  (params (DeltaSeconds :type Float%20%28single-precision%29)))

(event EventPickup
  (params (AttachTo :type Scene%20Component%20Object%20Reference) (hand :type EControllerHand%20Enum :default "Left"))
  (Variables|/Script/Engine.ActorComponent|SetComponentTags (Variables|Default|GetStaticMeshComponent) (Utilities|Array|MakeArray "HEALING"))
  (Physics|SetSimulatePhysics (Variables|Default|GetStaticMeshComponent) false)
  (Transformation|AttachComponentToComponent (VehicleSound|GetRootComponent) AttachTo "None" "SnapToTarget" "SnapToTarget" "KeepWorld" false))

(fn ConstructionScript)