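; Paper is a VR grabbable physics object that ties into the tutorial sequence.
; It finds a Tutorial_Info actor on BeginPlay and polls it on Tick, allowing grabbing once the tutorial is active, or immediately if none exists.
; Pickup from BP_MotionController disables physics, snaps it to the hand and plays a tutorial clip on the first grab only.
; Drop detaches it and re-enables physics.
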(event OnComponentHit(StaticMeshComponent)
  (params (HitComponent :type Primitive%20Component%20Object%20Reference) (OtherActor :type Actor%20Object%20Reference) (OtherComp :type Primitive%20Component%20Object%20Reference) (NormalImpulse :type Vector :default "0, 0, 0") (Hit :type Hit%20Result%20Structure%20%28by%20ref%29)))

(event EventBeginPlay
  (bind _outactors (Actor|GetAllActorsOfClass "/Game/Assets/Blueprints/Tutorial_Info.Tutorial_Info_C"))
  (Utilities|IsValid (Utilities|Array|Get(acopy) _outactors)
    (:Is%20Valid
      (Variables|Default|SettutorialInfoRef (Utilities|Array|Get(acopy) _outactors)))
    (:Is%20Not%20Valid
      (Variables|Default|SetcanGrab true))))

(event Collision|EventActorBeginOverlap
  (params (OtherActor :type Actor%20Object%20Reference)))

(event EventTick
  (params (DeltaSeconds :type Float%20%28single-precision%29))
  (bind _tutorialinforef (Variables|Default|GettutorialInfoRef))
  (if (not (Variables|Default|GetcanGrab))
    (Utilities|IsValid _tutorialinforef
      (:Is%20Valid
        (if (Variables|/Game/Assets/Blueprints/Tutorial_Info.Tutorial_Info_C|GetTutorialActive _tutorialinforef)
          (Variables|Default|SetcanGrab true))))))

(event EventPickup
  (params (AttachTo :type Scene%20Component%20Object%20Reference) (hand :type EControllerHand%20Enum :default "Left"))
  (bind _tutorialinforef (Variables|Default|GettutorialInfoRef))
  (if (Variables|Default|GetcanGrab)
    (Physics|SetSimulatePhysics (Variables|Debug|GetStaticMeshComponent) false)
    (Transformation|AttachComponentToComponent (VehicleSound|GetRootComponent) AttachTo "None" "SnapToTarget" "SnapToTarget" "KeepWorld" false)
    (Utilities|FlowControl|DoOnce false
      (:Completed
        (Utilities|IsValid _tutorialinforef
          (:Is%20Valid
            (Default|PlayNextClip _tutorialinforef)))))))

(event EventDrop
  (params (hand :type EControllerHand%20Enum :default "Left"))
  (bind _staticmeshcomponent (Variables|Debug|GetStaticMeshComponent))
  (Physics|SetSimulatePhysics (Variables|Debug|GetStaticMeshComponent) true)
  (Transformation|DetachFromActor "KeepWorld" "KeepWorld" "KeepWorld")
  (bind _returnvalue (Physics|GetPhysicsLinearVelocity _staticmeshcomponent "None"))
  (Physics|SetPhysicsLinearVelocity _staticmeshcomponent _returnvalue false "None"))

(fn ConstructionScript)