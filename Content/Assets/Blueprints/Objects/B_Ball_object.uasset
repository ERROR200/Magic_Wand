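; B_Ball_object is a throwable physics ball that BP_MotionController can pick up and that damages what it hits.
; Pickup turns off physics and snaps the ball to the given component, while Drop re-enables physics, detaches it and doubles its linear velocity to boost the throw.
; Every mesh hit sends a damage message to the other actor and resets a short lifespan, so the ball expires after its last impact.
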(event OnComponentHit(StaticMeshComponent)
  (params (HitComponent :type Primitive%20Component%20Object%20Reference) (OtherActor :type Actor%20Object%20Reference) (OtherComp :type Primitive%20Component%20Object%20Reference) (NormalImpulse :type Vector :default "0, 0, 0") (Hit :type Hit%20Result%20Structure%20%28by%20ref%29))
  (Actor|SetLifeSpan 1e+01)
  (Class|IDamage|TakeDamage(Message) OtherActor 2.0 false "NewEnumerator4" 0.0))

(event EventBeginPlay)

(event Collision|EventActorBeginOverlap
  (params (OtherActor :type Actor%20Object%20Reference)))

(event EventTick
  (params (DeltaSeconds :type Float%20%28single-precision%29)))

(event EventPickup
  (params (AttachTo :type Scene%20Component%20Object%20Reference))
  (Physics|SetSimulatePhysics (Variables|Debug|GetStaticMeshComponent) false)
  (Transformation|AttachComponentToComponent (VehicleSound|GetRootComponent) AttachTo "None" "SnapToTarget" "KeepWorld" "KeepWorld" false))

(event EventDrop
  (bind _staticmeshcomponent (Variables|Debug|GetStaticMeshComponent))
  (Physics|SetSimulatePhysics (Variables|Debug|GetStaticMeshComponent) true)
  (Transformation|DetachFromActor "KeepWorld" "KeepWorld" "KeepWorld")
  (bind _returnvalue (Physics|GetPhysicsLinearVelocity _staticmeshcomponent "None"))
  (Physics|SetPhysicsLinearVelocity _staticmeshcomponent (* _returnvalue 2.0) false "None"))

(fn ConstructionScript)