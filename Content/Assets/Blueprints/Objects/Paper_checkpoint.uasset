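; Grabbable VR paper checkpoint that sends the player to its configured Level when picked up with a motion controller.
; It is grabbable at start only if no Tutorial_Info actor exists; otherwise an unlock event reveals it and enables grabbing.
; A one-time pickup attaches it and animates its dynamic material's Amount through a timeline, then calls ChangeLevel on PersonalMCPawn.
; Drop, or the timeline finishing, detaches it and enables physics.
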(event OnComponentHit(StaticMeshComponent)
  (params (HitComponent :type Primitive%20Component%20Object%20Reference) (OtherActor :type Actor%20Object%20Reference) (OtherComp :type Primitive%20Component%20Object%20Reference) (NormalImpulse :type Vector :default "0, 0, 0") (Hit :type Hit%20Result%20Structure%20%28by%20ref%29)))

(event Custom|unlock
  (Development|SetHiddeninGame (Variables|Debug|GetStaticMeshComponent) false true)
  (Variables|Default|SetcanGrab true))

(event EventBeginPlay
  (bind _outactors (Actor|GetAllActorsOfClass "/Game/Assets/Blueprints/Tutorial_Info.Tutorial_Info_C"))
  (Utilities|IsValid (Utilities|Array|Get(acopy) _outactors)
    (:Is%20Valid
      (Variables|Default|SettutorialInfoRef (Utilities|Array|Get(acopy) _outactors)))
    (:Is%20Not%20Valid
      (Variables|Default|SetcanGrab true))))

(event Collision|EventActorBeginOverlap
  (params (OtherActor :type Actor%20Object%20Reference)))

(event EventPickup
  (params (AttachTo :type Scene%20Component%20Object%20Reference) (hand :type EControllerHand%20Enum :default "Left"))
  (if (Variables|Default|GetcanGrab)
    (Utilities|FlowControl|DoOnce false
      (:Completed
        (Transformation|AttachComponentToComponent (VehicleSound|GetRootComponent) AttachTo "None" "SnapToTarget" "SnapToTarget" "KeepWorld" false)
        (bind _newtrack_0 (Timeline|Timeline_0 Play)
          (:Update
            (Rendering|Material|SetScalarParameterValue (Variables|Default|Getdynamat) "Amount" _newtrack_0 :!class /Script/Engine.MaterialInstanceDynamic))
          (:Finished
            (bind _aspersonal_mcpawn (Utilities|Casting|CastToPersonalMCPawn (Game|Player|GetPlayerPawn 0)))
            (Default|ChangeLevel _aspersonal_mcpawn (Variables|Default|GetLevel))
            (Physics|SetSimulatePhysics (Variables|Debug|GetStaticMeshComponent) true)
            (Transformation|DetachFromActor "KeepWorld" "KeepWorld" "KeepWorld")))))))

(event EventDrop
  (params (hand :type EControllerHand%20Enum :default "Left"))
  (Physics|SetSimulatePhysics (Variables|Debug|GetStaticMeshComponent) true)
  (Transformation|DetachFromActor "KeepWorld" "KeepWorld" "KeepWorld"))

(fn ConstructionScript
  (bind _returnvalue (Rendering|Material|CreateDynamicMaterialInstance (Variables|Debug|GetStaticMeshComponent) 0 (Variables|Default|GetMat) :!class /Script/Engine.PrimitiveComponent))
  (Variables|Default|Setdynamat _returnvalue))