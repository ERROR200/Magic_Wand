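; Banana pickup actor, named as a heal object, that can be carried, thrown and swapped to a rigged peel.
; The peel starts hidden without collision until Change swaps it in for the static mesh and activates AppleEat.
; Pickup stops physics and snaps the root to the given component.
; Drop restores physics on both meshes, detaches, and boosts the static mesh's velocity; no healing logic lives here.
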(event EventBeginPlay
  (bind _bananapeel_rigged (Variables|Default|GetBananaPeel_Rigged))
  (Rendering|SetVisibility _bananapeel_rigged false false)
  (Collision|SetCollisionEnabled _bananapeel_rigged "NoCollision")
  (|CallParentFunction))

(event Collision|EventActorBeginOverlap
  (params (OtherActor :type Actor%20Object%20Reference)))

(event EventTick
  (params (DeltaSeconds :type Float%20%28single-precision%29)))

(event EventDrop
  (params (hand :type EControllerHand%20Enum :default "Left"))
  (bind _staticmeshcomponent (Variables|Default|GetStaticMeshComponent))
  (Physics|SetSimulatePhysics (Variables|Default|GetStaticMeshComponent) true)
  (Transformation|DetachFromActor "KeepWorld" "KeepWorld" "KeepWorld")
  (bind _returnvalue (Physics|GetPhysicsLinearVelocity _staticmeshcomponent "None"))
  (Physics|SetPhysicsLinearVelocity _staticmeshcomponent (* _returnvalue 1.5) false "None"))

(event EventChange
  (bind _bananapeel_rigged (Variables|Default|GetBananaPeel_Rigged))
  (bind _staticmeshcomponent (Variables|Default|GetStaticMeshComponent))
  (Rendering|SetVisibility _staticmeshcomponent false false)
  (Collision|SetCollisionEnabled _staticmeshcomponent "NoCollision")
  (Rendering|SetVisibility _bananapeel_rigged true false)
  (Collision|SetCollisionEnabled _bananapeel_rigged "QueryAndPhysics")
  (Components|Activation|Activate (Variables|Default|GetApple_eat) false))

(event EventPickup
  (params (AttachTo :type Scene%20Component%20Object%20Reference) (hand :type EControllerHand%20Enum :default "Left"))
  (Physics|SetSimulatePhysics (Variables|Default|GetStaticMeshComponent) false)
  (Transformation|AttachComponentToComponent (VehicleSound|GetRootComponent) AttachTo "None" "SnapToTarget" "SnapToTarget" "KeepWorld" false))

(fn ConstructionScript)